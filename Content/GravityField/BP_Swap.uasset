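; BP_Swap is a gravity field actor that supplies a gravity direction taken from its own rotation.
; GetGravityDirection packs the actor's roll, pitch and yaw directly into the X, Y and Z of the returned vector.
; The first time BP_MainCharacter overlaps its Box, it plays a sound at the world origin and nudges the root's local rotation, which alters that vector.
; A DoOnce with no reset limits this to one trigger.
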(event OnComponentBeginOverlap(Box)
  (params (OverlappedComponent :type Primitive%20Component%20Object%20Reference) (OtherActor :type Actor%20Object%20Reference) (OtherComp :type Primitive%20Component%20Object%20Reference) (OtherBodyIndex :type Integer) (bFromSweep :type Boolean) (SweepResult :type Hit%20Result%20Structure%20%28by%20ref%29))
  (Utilities|Casting|CastToBP_MainCharacter OtherActor)
  (Utilities|FlowControl|DoOnce false
    (:Completed
      (Audio|PlaySoundatLocation 0 "0, 0, 0" "0, 0, 0" 1.0 1.0 0.0 0 0 0 0)
      (Transformation|AddLocalRotation (Variables|Default|GetDefaultSceneRoot) "0.000000,1.000000,0.000000" false false))))

(event EventBeginPlay
  (|CallParentFunction) ; This node is disabled and will not be called.\nDrag off pins to build functionality.
)

(event Collision|EventActorBeginOverlap
  (params (OtherActor :type Actor%20Object%20Reference))
  (|CallParentFunction OtherActor) ; This node is disabled and will not be called.\nDrag off pins to build functionality.
)

(event EventTick
  (params (DeltaSeconds :type Float%20%28single-precision%29))
  (|CallParentFunction DeltaSeconds) ; This node is disabled and will not be called.\nDrag off pins to build functionality.
)

(fn ConstructionScript
  (|CallParentFunction))

(fn GetGravityDirection
  (params (Actor :type Actor%20Object%20Reference))
  (bind _returnvalue (Transformation|GetActorRotation))
  (bind (_roll _pitch _yaw) (Math|Rotator|BreakRotator _returnvalue))
  (|CallParentFunction Actor)
  (bind _output_get (LocalVariables|SetGravityDir (Math|Vector|MakeVector _roll _pitch _yaw)))
  (return _output_get))