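; Gravity box with an arrow checkpoint that supplies a gravity direction and can be activated by the player.
; GetGravityDirection overrides the parent, returning the actor's raw rotation angles as the vector rather than a computed unit direction.
; Overlapping the box shows a widget and enables input; leaving reverses both.
; The first Interact from BP_MainCharacter lights the arrow materials, calls a sound playback and rotates the root.
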(event OnComponentBeginOverlap(Box)
  (params (OverlappedComponent :type Primitive%20Component%20Object%20Reference) (OtherActor :type Actor%20Object%20Reference) (OtherComp :type Primitive%20Component%20Object%20Reference) (OtherBodyIndex :type Integer) (bFromSweep :type Boolean) (SweepResult :type Hit%20Result%20Structure%20%28by%20ref%29))
  ;[1 1 1] Widget
  (Rendering|SetVisibility (Variables|Default|GetWidget) true false)
  (Input|EnableInput (Game|GetPlayerController 0)))

(event OnComponentEndOverlap(Box)
  (params (OverlappedComponent :type Primitive%20Component%20Object%20Reference) (OtherActor :type Actor%20Object%20Reference) (OtherComp :type Primitive%20Component%20Object%20Reference) (OtherBodyIndex :type Integer))
  ;[1 1 1] Widget
  (Rendering|SetVisibility (Variables|Default|GetWidget) false false)
  (Input|DisableInput (Game|GetPlayerController 0)))

(event EventBeginPlay
  (|CallParentFunction) ; This node is disabled and will not be called.\nDrag off pins to build functionality.
)

(event Collision|EventActorBeginOverlap
  (params (OtherActor :type Actor%20Object%20Reference))
  (|CallParentFunction OtherActor) ; This node is disabled and will not be called.\nDrag off pins to build functionality.
)

(event EventTick
  (params (DeltaSeconds :type Float%20%28single-precision%29))
  (|CallParentFunction DeltaSeconds) ; This node is disabled and will not be called.\nDrag off pins to build functionality.
)

(event EventInteract
  (params (Character :type BP%20Main%20Character%20Object%20Reference))
  (Utilities|Casting|CastToBP_MainCharacter Character)
  (if true
    (Utilities|FlowControl|DoOnce false
      (:Completed
        (Rendering|Material|SetMaterial (Variables|Default|GetArrowCheckpoint) 3 "/Game/Materials/WowLight.WowLight")
        (Rendering|Material|SetMaterial (Variables|Default|GetArrowCheckpoint) 4 "/Game/Materials/WowLight.WowLight")
        (Rendering|Material|SetMaterial (Variables|Default|GetArrowCheckpoint) 5 "/Game/Materials/WowLight.WowLight")
        (Audio|PlaySoundatLocation 0 "0, 0, 0" "0, 0, 0" 1.0 1.0 0.0 0 0 0 0)
        (Transformation|AddLocalRotation (Variables|Default|GetDefaultSceneRoot) "359.000000,0.000000,0.000000" false false)))))

(fn ConstructionScript
  (|CallParentFunction))

(fn GetGravityDirection
  (params (Actor :type Actor%20Object%20Reference))
  (bind _returnvalue (Transformation|GetActorRotation))
  (bind (_roll _pitch _yaw) (Math|Rotator|BreakRotator _returnvalue))
  (|CallParentFunction Actor)
  (bind _output_get (LocalVariables|SetGravityDir (Math|Vector|MakeVector _roll _pitch _yaw)))
  (return _output_get))