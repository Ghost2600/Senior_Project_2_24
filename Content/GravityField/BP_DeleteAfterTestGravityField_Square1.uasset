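; Test gravity field, named for later deletion, that rotates its own root when the main character enters or leaves its box.
; Entry runs once per BP_GravityField_Square whose GravityBoxNumber is 0, while exit runs directly.
; Both play a sound and use a FlipFlop to alternate small local rotations with debug prints.
; The GetGravityDirection override returns the actor's raw rotation angles as the gravity vector, so those rotations alter it.
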(event OnComponentBeginOverlap(Box)
  (params (OverlappedComponent :type Primitive%20Component%20Object%20Reference) (OtherActor :type Actor%20Object%20Reference) (OtherComp :type Primitive%20Component%20Object%20Reference) (OtherBodyIndex :type Integer) (bFromSweep :type Boolean) (SweepResult :type Hit%20Result%20Structure%20%28by%20ref%29))
  (bind _outactors (Actor|GetAllActorsOfClass "/Game/GravityField/BP_GravityField_Square.BP_GravityField_Square_C"))
  (bind _array_element (Utilities|Array|ForEachLoopwithBreak _outactors)
    (:LoopBody
      (if (== (Variables|/Game/GravityField/BP_GravityField_Square.BP_GravityField_Square_C|GetGravityBoxNumber _array_element) 0)
        (Utilities|Casting|CastToBP_MainCharacter OtherActor)
        (Audio|PlaySoundatLocation 0 "0, 0, 0" "0, 0, 0" 1.0 1.0 0.0 0 0 0 0)
        (Utilities|FlowControl|FlipFlop
          (:A
            (Transformation|AddLocalRotation (Variables|Default|GetDefaultSceneRoot) "0, 0, 0" false false)
            (Development|PrintString "Return"))
          (:B
            (Transformation|AddLocalRotation (Variables|Default|GetDefaultSceneRoot) "0.000000,-1.000000,0.000000" false false)
            (Development|PrintString "Arrow Move")))))))

(event OnComponentEndOverlap(Box)
  (params (OverlappedComponent :type Primitive%20Component%20Object%20Reference) (OtherActor :type Actor%20Object%20Reference) (OtherComp :type Primitive%20Component%20Object%20Reference) (OtherBodyIndex :type Integer))
  (Utilities|Casting|CastToBP_MainCharacter OtherActor)
  (Audio|PlaySoundatLocation 0 "0, 0, 0" "0, 0, 0" 1.0 1.0 0.0 0 0 0 0)
  (Utilities|FlowControl|FlipFlop
    (:A
      (Transformation|AddLocalRotation (Variables|Default|GetDefaultSceneRoot) "-1.000000,0.000000,0.000000" false false)
      (Development|PrintString "Exit"))
    (:B
      (Transformation|AddLocalRotation (Variables|Default|GetDefaultSceneRoot) "1.000000,1.000000,0.000000" false false)
      (Development|PrintString "Exit2"))))

(event EventBeginPlay
  (|CallParentFunction) ; This node is disabled and will not be called.\nDrag off pins to build functionality.
)

(event Collision|EventActorBeginOverlap
  (params (OtherActor :type Actor%20Object%20Reference))
  (|CallParentFunction OtherActor) ; This node is disabled and will not be called.\nDrag off pins to build functionality.
)

(event EventTick
  (params (DeltaSeconds :type Float%20%28single-precision%29))
  (|CallParentFunction DeltaSeconds) ; This node is disabled and will not be called.\nDrag off pins to build functionality.
)

(fn ConstructionScript
  (|CallParentFunction))

(fn GetGravityDirection
  (params (Actor :type Actor%20Object%20Reference))
  (bind _returnvalue (Transformation|GetActorRotation))
  (bind (_roll _pitch _yaw) (Math|Rotator|BreakRotator _returnvalue))
  (|CallParentFunction Actor)
  (bind _output_get (LocalVariables|SetGravityDir (Math|Vector|MakeVector _roll _pitch _yaw)))
  (Development|PrintText (Utilities|Text|ToText(String) _output_get) true true "(R=1.000000,G=0.968079,B=0.032310,A=1.000000)" 5.0)
  (return _output_get))