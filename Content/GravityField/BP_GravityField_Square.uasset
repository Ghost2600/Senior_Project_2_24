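; BP_GravityField_Square is a gravity field Blueprint that supplies a gravity direction for a given actor.
; It overrides GetGravityDirection, calling the parent and then returning the unit vector from the field's location to the actor, pointing away from the field.
; Despite the Square name, the math is purely radial, with no box-face logic.
; The direction is printed as debug text, and the event graph and construction script add no behavior.
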(event EventBeginPlay
  (|CallParentFunction) ; This node is disabled and will not be called.\nDrag off pins to build functionality.
)

(event Collision|EventActorBeginOverlap
  (params (OtherActor :type Actor%20Object%20Reference))
  (|CallParentFunction OtherActor) ; This node is disabled and will not be called.\nDrag off pins to build functionality.
)

(event EventTick
  (params (DeltaSeconds :type Float%20%28single-precision%29))
  (|CallParentFunction DeltaSeconds) ; This node is disabled and will not be called.\nDrag off pins to build functionality.
)

(fn ConstructionScript
  (|CallParentFunction))

(fn GetGravityDirection
  (params (Actor :type Actor%20Object%20Reference))
  (bind _returnvalue (Transformation|GetActorLocation))
  (bind _returnvalue_2 (Transformation|GetActorLocation Actor))
  (bind _returnvalue_3 (Math|Vector|GetUnitDirection(Vector) _returnvalue _returnvalue_2))
  (|CallParentFunction Actor)
  (Development|PrintText (Utilities|Text|ToText(String) _returnvalue_3) true true "(R=1.000000,G=0.968079,B=0.032310,A=1.000000)" 5.0)
  (return _returnvalue_3))