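; BP_DevonGreen is an organic environment Blueprint in DreamscapeTower that plays a collision sound when hit.
; Hit spawns the sound attached to the struck component, with a DoOnce and short delay throttling repeats.
; Volume is meant to follow impulse strength, but its normalization range has zero width, so it does not scale.
; Sphere overlap events are empty, and leftover grass-footstep and skeletal-animation nodes never run.
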(event OnComponentEndOverlap(Collision_Sphere)
  (params (OverlappedComponent :type Primitive%20Component%20Object%20Reference) (OtherActor :type Actor%20Object%20Reference) (OtherComp :type Primitive%20Component%20Object%20Reference) (OtherBodyIndex :type Integer))
  ;[1 1 1] delete
)

(event OnComponentBeginOverlap(Collision_Sphere)
  (params (OverlappedComponent :type Primitive%20Component%20Object%20Reference) (OtherActor :type Actor%20Object%20Reference) (OtherComp :type Primitive%20Component%20Object%20Reference) (OtherBodyIndex :type Integer) (bFromSweep :type Boolean) (SweepResult :type Hit%20Result%20Structure%20%28by%20ref%29))
  ;[1 1 1] delete
)

(event Collision|EventHit
  (params (MyComp :type Primitive%20Component%20Object%20Reference) (Other :type Actor%20Object%20Reference) (OtherComp :type Primitive%20Component%20Object%20Reference) (bSelfMoved :type Boolean) (HitLocation :type Vector :default "0, 0, 0") (HitNormal :type Vector :default "0, 0, 0") (NormalImpulse :type Vector :default "0, 0, 0") (Hit :type Hit%20Result%20Structure%20%28by%20ref%29))
  (Utilities|FlowControl|DoOnce false :!label _label
    (:Completed
      (bind _returnvalue (Audio|SpawnSoundAttached (Variables|Default|GetCollision%20Sound) MyComp "None" "0, 0, 0" "0, 0, 0" "KeepRelativeOffset" false 1.0 1.0 0.0 0 0))
      (Audio|Components|Audio|SetVolumeMultiplier _returnvalue (Math|Float|NormalizetoRange (Math|Vector|VectorLength NormalImpulse) 0.0 0.0) :!class /Script/Engine.AudioComponent)
      (Utilities|FlowControl|Delay 0.2)
      (goto _label Reset))))

(fn ConstructionScript)