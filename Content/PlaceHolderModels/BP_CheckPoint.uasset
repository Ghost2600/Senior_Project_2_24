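; BP_CheckPoint is a checkpoint actor that reacts when BP_MainCharacter overlaps its Box.
; The first overlap only, via DoOnce, plays a sound, adds a WBP_Checkpoint widget to the viewport and sets the Cube's material.
; Every qualifying overlap also writes LastCheckpoint on the BP_TestMode game mode, but assigns None, as the self reference is left unused.
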(event OnComponentBeginOverlap(Box)
  (params (OverlappedComponent :type Primitive%20Component%20Object%20Reference) (OtherActor :type Actor%20Object%20Reference) (OtherComp :type Primitive%20Component%20Object%20Reference) (OtherBodyIndex :type Integer) (bFromSweep :type Boolean) (SweepResult :type Hit%20Result%20Structure%20%28by%20ref%29))
  (if (Utilities|ClassIsChildOf (Utilities|GetClass OtherActor) "/Game/MainCharacter/BP_MainCharacter.BP_MainCharacter_C")
    (Utilities|FlowControl|Sequence
      (:then_0
        (Utilities|FlowControl|DoOnce false
          (:Completed
            (Audio|PlaySoundatLocation 0 (Transformation|GetWorldLocation (Variables|Default|GetDefaultSceneRoot)) "0, 0, 0" 0.2 1.0 0.0 0 0 0 0)
            (bind _returnvalue (UserInterface|CreateWidget "/Game/Widget/WBP_Checkpoint.WBP_Checkpoint_C"))
            (UserInterface|Viewport|AddtoViewport _returnvalue 0)
            (Rendering|Material|SetMaterial (Variables|Default|GetCube) 0 0))))
      (:then_1
        (Utilities|Casting|CastToBP_MainCharacter OtherActor)
        (bind _asbp_test_mode (Utilities|Casting|CastToBP_TestMode (Game|GetGameMode)))
        (Variables|/Game/MainCharacter/BP_TestMode.BP_TestMode_C|Setlast%20Checkpoint _asbp_test_mode 0)))))

(fn ConstructionScript)