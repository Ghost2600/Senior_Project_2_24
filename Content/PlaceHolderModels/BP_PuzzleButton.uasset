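; BP_PuzzleButton is an interactable puzzle button that opens a BP_PuzzleDoor with a matching value.
; Overlapping its Box shows a widget and enables player input on the button; leaving reverses both.
; Interact searches all puzzle doors for a DoorValue equal to ButtonValue, then turns the mesh green and calls OpenDoor with the interacting character.
; A DoOnce inside the loop limits this to the first match, one time only.
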(event OnComponentBeginOverlap(Box)
  (params (OverlappedComponent :type Primitive%20Component%20Object%20Reference) (OtherActor :type Actor%20Object%20Reference) (OtherComp :type Primitive%20Component%20Object%20Reference) (OtherBodyIndex :type Integer) (bFromSweep :type Boolean) (SweepResult :type Hit%20Result%20Structure%20%28by%20ref%29))
  ;[1 1 1] Widget
  (Rendering|SetVisibility (Variables|Default|GetWidget) true false)
  (Input|EnableInput (Game|GetPlayerController 0)))

(event OnComponentEndOverlap(Box)
  (params (OverlappedComponent :type Primitive%20Component%20Object%20Reference) (OtherActor :type Actor%20Object%20Reference) (OtherComp :type Primitive%20Component%20Object%20Reference) (OtherBodyIndex :type Integer))
  ;[1 1 1] Widget
  (Rendering|SetVisibility (Variables|Default|GetWidget) false false)
  (Input|DisableInput (Game|GetPlayerController 0)))

(event EventInteract
  (params (Character :type BP%20Main%20Character%20Object%20Reference))
  (bind _outactors (Actor|GetAllActorsOfClass "/Game/PlaceHolderModels/BP_PuzzleDoor.BP_PuzzleDoor_C"))
  (bind _array_element (Utilities|Array|ForEachLoopwithBreak _outactors)
    (:LoopBody
      (if (== (Variables|/Game/PlaceHolderModels/BP_PuzzleDoor.BP_PuzzleDoor_C|GetDoorValue _array_element) (Variables|Default|GetButtonValue))
        (Utilities|FlowControl|DoOnce false
          (:Completed
            (Rendering|Material|SetMaterial (Variables|Default|GetStaticMesh) 0 "/Game/Materials/M_Green.M_Green")
            (Default|OpenDoor _array_element Character)))))))

(fn ConstructionScript)