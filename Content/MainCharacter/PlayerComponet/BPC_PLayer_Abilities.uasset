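; Player ability component that gives the main character Push and Lift force powers, triggered by Enhanced Input actions or the F and R keys.
; Each power, when off cooldown, spawns a Niagara cast effect, capsule-traces forward for WorldDynamic objects and sends a push or lift message to the hit actor.
; Delay-based cooldowns update readiness flags on the WB_AbilityCooldowns widget created at BeginPlay and spawn a recharge effect when finished.
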(event Input|EnhancedActionEvents|EnhancedInputActionIA_Push
  (params (ActionValue :type Boolean) (ElapsedSeconds :type Float%20%28double-precision%29) (TriggeredSeconds :type Float%20%28double-precision%29) (InputAction :type Input%20Action%20Object%20Reference :default "/Game/ThirdPerson/Input/Actions/IA_Push.IA_Push"))
  (bind _maincharacter (Variables|Default|GetMainCharacter))
  ;[1 1 1 1 45] Push Force
  (CallFunction|PushFunction)
  (Variables|Default|SetPushOnCooldown true)
  (Variables|/Game/Widget/WB_AbilityCooldowns.WB_AbilityCooldowns_C|SetPushReady? (Variables|Default|GetAbilityCooldown) false)
  (Utilities|FlowControl|Delay (Variables|Default|GetPushCooldown))
  (Variables|Default|SetPushOnCooldown false)
  (Niagara|SpawnSystematLocation "/Game/VFX/Placeholder/NS_PushRecharge.NS_PushRecharge" (Transformation|GetActorLocation _maincharacter) (Transformation|GetActorRotation _maincharacter))
  (Variables|/Game/Widget/WB_AbilityCooldowns.WB_AbilityCooldowns_C|SetPushReady? (Variables|Default|GetAbilityCooldown) true))

(event Input|EnhancedActionEvents|EnhancedInputActionIA_Lift
  (params (ActionValue :type Boolean) (ElapsedSeconds :type Float%20%28double-precision%29) (TriggeredSeconds :type Float%20%28double-precision%29) (InputAction :type Input%20Action%20Object%20Reference :default "/Game/ThirdPerson/Input/Actions/IA_Lift.IA_Lift"))
  (bind _maincharacter (Variables|Default|GetMainCharacter))
  ;[1 1 1 1 45] Lift Force
  (CallFunction|LiftFunction)
  (Variables|Default|SetLiftOnCooldown true)
  (Variables|/Game/Widget/WB_AbilityCooldowns.WB_AbilityCooldowns_C|SetLiftReady? (Variables|Default|GetAbilityCooldown) false)
  (Utilities|FlowControl|Delay (Variables|Default|GetLiftCooldown))
  (Variables|Default|SetLiftOnCooldown false)
  (Niagara|SpawnSystematLocation "/Game/VFX/Placeholder/NS_LiftRecharge.NS_LiftRecharge" (Transformation|GetActorLocation _maincharacter) (Transformation|GetActorRotation _maincharacter))
  (Variables|/Game/Widget/WB_AbilityCooldowns.WB_AbilityCooldowns_C|SetLiftReady? (Variables|Default|GetAbilityCooldown) true))

(event EventBeginPlay
  (bind _debug (Variables|Default|GetDebug))
  (bind _asbp_main_character (Utilities|Casting|CastToBP_MainCharacter (Game|Player|GetPlayerPawn 0))
    (:then
      (Variables|Default|SetMainCharacter _asbp_main_character)
      (bind _returnvalue (UserInterface|CreateWidget "/Game/Widget/WB_AbilityCooldowns.WB_AbilityCooldowns_C" (Game|GetPlayerController 0)))
      (bind _output_get (Variables|Default|SetAbilityCooldown _returnvalue))
      (UserInterface|Viewport|AddtoViewport _output_get 0))
    (:CastFailed
      (Development|PrintString "ERROR[BPC_Player_Abilities]: Start Can't cast maincharacter" _debug _debug "(R=1.000000,G=0.023616,B=0.000000,A=1.000000)" 1.5e+02))))

(event Input|KeyboardEvents|R
  (params (Key :type Key%20Structure :default "None"))
  (bind _maincharacter (Variables|Default|GetMainCharacter))
  ;[1 1 1 1 45] Lift Force
  (:Pressed
    (CallFunction|LiftFunction)
    (Variables|Default|SetLiftOnCooldown true)
    (Variables|/Game/Widget/WB_AbilityCooldowns.WB_AbilityCooldowns_C|SetLiftReady? (Variables|Default|GetAbilityCooldown) false)
    (Utilities|FlowControl|Delay (Variables|Default|GetLiftCooldown))
    (Variables|Default|SetLiftOnCooldown false)
    (Niagara|SpawnSystematLocation "/Game/VFX/Placeholder/NS_LiftRecharge.NS_LiftRecharge" (Transformation|GetActorLocation _maincharacter) (Transformation|GetActorRotation _maincharacter))
    (Variables|/Game/Widget/WB_AbilityCooldowns.WB_AbilityCooldowns_C|SetLiftReady? (Variables|Default|GetAbilityCooldown) true)))

(event Input|KeyboardEvents|F
  (params (Key :type Key%20Structure :default "None"))
  (bind _maincharacter (Variables|Default|GetMainCharacter))
  ;[1 1 1 1 45] Push Force
  (:Pressed
    (CallFunction|PushFunction)
    (Variables|Default|SetPushOnCooldown true)
    (Variables|/Game/Widget/WB_AbilityCooldowns.WB_AbilityCooldowns_C|SetPushReady? (Variables|Default|GetAbilityCooldown) false)
    (Utilities|FlowControl|Delay (Variables|Default|GetPushCooldown))
    (Variables|Default|SetPushOnCooldown false)
    (Niagara|SpawnSystematLocation "/Game/VFX/Placeholder/NS_PushRecharge.NS_PushRecharge" (Transformation|GetActorLocation _maincharacter) (Transformation|GetActorRotation _maincharacter))
    (Variables|/Game/Widget/WB_AbilityCooldowns.WB_AbilityCooldowns_C|SetPushReady? (Variables|Default|GetAbilityCooldown) true)))

(fn PushFunction
  (bind _maincharacter (Variables|Default|GetMainCharacter))
  (bind _maincharacter_2 (Variables|Default|GetMainCharacter))
  (bind _returnvalue (Transformation|GetActorLocation _maincharacter_2))
  (if (not (Variables|Default|GetPushOnCooldown))
    (Niagara|SpawnSystematLocation "/Game/VFX/Placeholder/NS_PushCast.NS_PushCast" (Transformation|GetActorLocation _maincharacter) (Transformation|GetActorRotation _maincharacter) "10.000000,10.000000,10.000000")
    (bind (_outhit _returnvalue_2) (Class|KismetSystemLibrary|CapsuleTraceSingleforObjects _returnvalue (+ _returnvalue (* (Transformation|GetActorForwardVector (Variables|Default|GetMainCharacter)) 2e+03)) 96.0 42.0 (Utilities|Array|MakeArray "ObjectTypeQuery2") false 0 "ForDuration" true))
    (if _returnvalue_2
      (Class|BPIPush|Push(Message) (.HitActor (Collision|BreakHitResult _outhit)) (Transformation|GetActorLocation (Variables|Default|GetMainCharacter)) 1e+03))))

(fn LiftFunction
  (bind _maincharacter (Variables|Default|GetMainCharacter))
  (bind _maincharacter_2 (Variables|Default|GetMainCharacter))
  (bind _returnvalue (Transformation|GetActorLocation _maincharacter_2))
  (if (not (Variables|Default|GetLiftOnCooldown))
    (Niagara|SpawnSystematLocation "/Game/VFX/Placeholder/NS_LiftCast.NS_LiftCast" (Transformation|GetActorLocation _maincharacter) (Transformation|GetActorRotation _maincharacter) "10.000000,10.000000,10.000000")
    (bind (_outhit _returnvalue_2) (Class|KismetSystemLibrary|CapsuleTraceSingleforObjects _returnvalue (+ _returnvalue (* (Transformation|GetActorForwardVector (Variables|Default|GetMainCharacter)) 2e+03)) 96.0 42.0 (Utilities|Array|MakeArray "ObjectTypeQuery2") false 0 "ForDuration" true))
    (if _returnvalue_2
      (Class|BPILiftForce|Lift(Message) (.HitActor (Collision|BreakHitResult _outhit)) 1e+03 "0, 0, 0"))))