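; Player health component that links the main character to health UI updates and handles death and stun.
; On BeginPlay it caches the character and binds handlers to inherited health, death and stun events; health changes update the main widget.
; Death opens a death screen, pauses, focuses its menu button, ignores look input and resets character rotation.
; Stun only prints; death animation, input disabling and HUD removal are unconnected.
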(event Custom|UpdateHealthUI_Event
  (params (Current%20Health :type Float%20%28double-precision%29) (Max%20Health :type Float%20%28double-precision%29))
  (Default|UpdateHealth (Variables|/Game/MainCharacter/BP_MainCharacter.BP_MainCharacter_C|GetMainWidget (Variables|Default|GetMainCharacter)) Current%20Health))

(event Custom|Event%20Stun
  (bind _debug (Variables|Default|GetDebug))
  (Development|PrintString "Stun" _debug _debug))

(event Custom|Event%20Death
  (bind _returnvalue (Game|GetPlayerController 0))
  (bind _debug (Variables|Default|GetDebug))
  (Development|PrintString "Death" _debug _debug)
  (Utilities|FlowControl|Delay 1.0)
  (bind _returnvalue_2 (UserInterface|CreateWidget "/Game/Widget/DeathUI.DeathUI_C" _returnvalue))
  (UserInterface|Viewport|AddtoViewport _returnvalue_2 0)
  (Game|SetGamePaused true)
  (Input|SetInputModeGameandUI _returnvalue _returnvalue_2 "DoNotLock" true false)
  (Utilities|FlowControl|Delay 0.2)
  (Widget|SetKeyboardFocus (Variables|/Game/Widget/DeathUI.DeathUI_C|GetMainMenuButton _returnvalue_2))
  (Input|SetIgnoreLookInput (Game|GetPlayerController 0) true)
  (Transformation|SetActorRotation (Variables|Default|GetMainCharacter))
  (Variables|/Script/Engine.PlayerController|SetbShowMouseCursor (Game|GetPlayerController 0) false))

(event EventBeginPlay
  (bind _debug (Variables|Default|GetDebug))
  (|CallParentFunction)
  (bind _asbp_main_character (Utilities|Casting|CastToBP_MainCharacter (Game|Player|GetPlayerPawn 0))
    (:then
      (Variables|Default|SetMainCharacter _asbp_main_character)
      (EventDispatchers|AssignUpdateHealthUI (delegate Custom|UpdateHealthUI_Event))
      (EventDispatchers|BindEventtoDeath (delegate Custom|Event%20Death))
      (EventDispatchers|BindEventtoStun (delegate Custom|Event%20Stun)))
    (:CastFailed
      (Development|PrintString "ERROR[BPC_Player_Health]: Start Can't cast maincharacter" _debug _debug "(R=1.000000,G=0.023616,B=0.000000,A=1.000000)" 1.5e+02))))

(event EventTick
  (params (DeltaSeconds :type Float%20%28single-precision%29))
  (|CallParentFunction DeltaSeconds) ; This node is disabled and will not be called.\nDrag off pins to build functionality.
)