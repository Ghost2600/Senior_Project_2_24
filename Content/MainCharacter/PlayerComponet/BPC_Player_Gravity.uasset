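; Player gravity component that points the main character's movement gravity along the gravity field it is in.
; Overlap begin stores the BP_GravityField, applies its direction and notifies the character; overlap end falls back to another overlapping field or none, without resetting direction.
; SetGravityDirection reapplies gravity, with the current field overriding any BP_GravInterface actor.
; That actor comes from SetGravityZone, marked possibly unused, the only path restoring default gravity.
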(event Custom|Custom%20ActorBeginOverlap
  (params (Other%20Actor :type Actor%20Object%20Reference))
  (bind _asbp_gravity_field (Utilities|Casting|CastToBP_GravityField Other%20Actor))
  (bind _output_get (Variables|Private|SetCurrentGravityField _asbp_gravity_field))
  (bind _gravitydirection (Default|GetGravityDirection _output_get (Variables|Private|GetMainCharacter)))
  (Class|CharacterMovementComponent|SetGravityDirection (Variables|Default|GetCharacterMovement) _gravitydirection)
  (Default|OnGravityMovementChange (Variables|Private|GetMainCharacter)))

(event Custom|SetGravityZone
  (params (GravityActor :type Actor%20Object%20Reference))
  ;[1 1 1] Might Not Ever Be Called
  (Utilities|IsValid GravityActor
    (:Is%20Valid
      (if (Utilities|DoesObjectImplementInterface GravityActor "/Game/Blueprints/BP_GravInterface.BP_GravInterface_C")
        (Variables|Private|SetGravityActor GravityActor)
        (Variables|Private|SetIn%20Gravity true)
        (else
          (Variables|Private|SetGravityActor 0 :!label _label)
          (Variables|Private|SetIn%20Gravity false)
          (Class|CharacterMovementComponent|SetGravityDirection (Variables|Default|GetCharacterMovement) (Variables|Public|GetDefaultGravity)))))
    (:Is%20Not%20Valid
      (goto _label))))

(event Custom|Custom%20-%20ActorEndOverlap
  (params (Other%20Actor :type Actor%20Object%20Reference))
  (bind _maincharacter (Variables|Private|GetMainCharacter))
  (bind _overlappingactors (Collision|GetOverlappingActors _maincharacter "/Game/GravityField/BP_GravityField.BP_GravityField_C" :!class /Script/Engine.Actor))
  (if (Utilities|ClassIsChildOf (Utilities|GetClass Other%20Actor) "/Game/GravityField/BP_GravityField.BP_GravityField_C")
    (if (> (Utilities|Array|Length _overlappingactors) 0)
      (bind _asbp_gravity_field (Utilities|Casting|CastToBP_GravityField (Utilities|Array|Get(acopy) _overlappingactors))
        (:then
          (Variables|Private|SetCurrentGravityField _asbp_gravity_field))
        (:CastFailed
          (Variables|Private|SetCurrentGravityField 0)))
      (else
        (Variables|Private|SetCurrentGravityField 0)))
    (else
      (Variables|Private|SetCurrentGravityField 0))))

(event EventBeginPlay
  (bind _debug (Variables|Public|GetDebug))
  (bind _asbp_main_character (Utilities|Casting|CastToBP_MainCharacter (Game|Player|GetPlayerPawn 0))
    (:then
      (bind _output_get (Variables|Private|SetMainCharacter _asbp_main_character))
      (Variables|Default|SetCharacterMovement (Variables|/Script/Engine.Character|GetCharacterMovement _output_get)))
    (:CastFailed
      (Development|PrintString "ERROR[BPC_Player_Gravity]: Start Can't cast maincharacter" _debug _debug "(R=1.000000,G=0.023616,B=0.000000,A=1.000000)" 1.5e+02))))

(fn SetGravityDirection
  (if (Variables|Private|GetIn%20Gravity)
    (Utilities|IsValid (Variables|Private|GetGravityActor)
      (:Is%20Valid
        (bind _direction (Class|BPGravInterface|GetGravityDirection(Message) (Variables|Private|GetGravityActor)))
        (Class|CharacterMovementComponent|SetGravityDirection (Variables|Default|GetCharacterMovement) _direction))))
  (bind _currentgravityfield (Variables|Private|GetCurrentGravityField)
    (:then
      (bind _gravitydirection (Default|GetGravityDirection _currentgravityfield (Variables|Private|GetMainCharacter)))
      (Class|CharacterMovementComponent|SetGravityDirection (Variables|Default|GetCharacterMovement) _gravitydirection))
    (:else)))