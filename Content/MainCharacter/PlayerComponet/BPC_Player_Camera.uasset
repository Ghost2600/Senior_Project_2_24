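; Player camera component that drives BP_MainCharacter's boom camera and enemy lock-on.
; UpdateCamera applies look input with clamped pitch and realigns the detached camera root to a gravity up vector derived from CameraOrienter.
; SetCamera switches combat and normal arm lengths, via hotkeys or lock-on.
; LockOn retargets the closest combat-manager enemy on a repeating timer, ignores look input and changes movement rotation; LockOff reverts this, and UpdateLockedCamera is an empty stub.
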(event Custom|Lock%20On
  (bind _debug (Variables|Default|GetDebug))
  (bind _maincharacter (Variables|MainCharacterInfo|GetMainCharacter))
  (bind _charactermovement (Variables|/Script/Engine.Character|GetCharacterMovement _maincharacter))
  ;[1 1 1] Lock On
  (GeneralCamera|SetCamera true)
  (CallFunction|UpdateTarget)
  (Utilities|Time|SetTimerbyEvent (delegate Custom|Update%20Target) 0.1 false true)
  (Utilities|IsValid (Variables|/Game/MainCharacter/BP_MainCharacter.BP_MainCharacter_C|GetTargetActor (Variables|MainCharacterInfo|GetMainCharacter))
    (:Is%20Valid
      (bind _output_get (Variables|/Game/MainCharacter/BP_MainCharacter.BP_MainCharacter_C|SetLockOnEnganged? (Variables|MainCharacterInfo|GetMainCharacter) true))
      (Input|SetIgnoreLookInput (Game|GetPlayerController 0) _output_get)
      (Variables|/Game/MainCharacter/BP_MainCharacter.BP_MainCharacter_C|SetShouldRotate _maincharacter true)
      (Variables|/Script/Engine.CharacterMovementComponent|SetbOrientRotationToMovement _charactermovement false)
      (Variables|/Script/Engine.CharacterMovementComponent|SetbUseControllerDesiredRotation _charactermovement true)
      (Variables|/Game/MainCharacter/BP_MainCharacter.BP_MainCharacter_C|SetBreakLockOnReference (Variables|MainCharacterInfo|GetMainCharacter) ""))
    (:Is%20Not%20Valid
      (Development|PrintString "Warning[BPC_Player_Camera]: Non-valid target actor" _debug _debug "(R=1.000000,G=0.930940,B=0.000000,A=1.000000)"))))

(event Custom|Update%20Target
  ;[1 1 1] Lock On
  (if (Variables|Default|GetIsCombatCamera)
    (bind _target (LockOn|GetClosestEnemy))
    (Variables|/Game/MainCharacter/BP_MainCharacter.BP_MainCharacter_C|SetTargetActor (Variables|MainCharacterInfo|GetMainCharacter) _target)
    (Utilities|Time|SetTimerbyEvent (delegate Custom|Update%20Target) 0.1 false true)))

(event Custom|Lock%20Off
  (bind _maincharacter (Variables|MainCharacterInfo|GetMainCharacter))
  (bind _charactermovement (Variables|/Script/Engine.Character|GetCharacterMovement _maincharacter))
  ;[1 1 1] Lock_Off
  (Variables|/Game/MainCharacter/BP_MainCharacter.BP_MainCharacter_C|SetTargetActor (Variables|MainCharacterInfo|GetMainCharacter) 0)
  (Variables|/Game/MainCharacter/BP_MainCharacter.BP_MainCharacter_C|SetLockOnEnganged? (Variables|MainCharacterInfo|GetMainCharacter) false)
  (Variables|/Game/MainCharacter/BP_MainCharacter.BP_MainCharacter_C|SetShouldRotate _maincharacter false)
  (Variables|/Script/Engine.CharacterMovementComponent|SetbOrientRotationToMovement _charactermovement true)
  (Variables|/Script/Engine.CharacterMovementComponent|SetbUseControllerDesiredRotation _charactermovement false)
  (Input|ResetIgnoreLookInput (Game|GetPlayerController 0))
  (GeneralCamera|SetCamera false))

(event EventBeginPlay
  (bind _debug (Variables|Default|GetDebug))
  (bind _asbp_main_character (Utilities|Casting|CastToBP_MainCharacter (Game|Player|GetPlayerPawn 0))
    (:then
      (bind _output_get (Variables|MainCharacterInfo|SetMainCharacter _asbp_main_character))
      (Variables|Default|SetCameraBoom (Variables|/Game/MainCharacter/BP_MainCharacter.BP_MainCharacter_C|GetCameraBoom _output_get))
      (Variables|Default|SetCameraOrienter (Variables|/Game/MainCharacter/BP_MainCharacter.BP_MainCharacter_C|GetCamera%20Orienter (Variables|MainCharacterInfo|GetMainCharacter)))
      (Variables|Default|SetCameraRoot (Variables|/Game/MainCharacter/BP_MainCharacter.BP_MainCharacter_C|GetCamera%20Root (Variables|MainCharacterInfo|GetMainCharacter))))
    (:CastFailed
      (Development|PrintString "ERROR[BPC_Player_Camera]: Start Can't cast maincharacter" _debug _debug "(R=1.000000,G=0.023616,B=0.000000,A=1.000000)" 1.5e+02))))

(event Input|KeyboardEvents|1
  (params (Key :type Key%20Structure :default "None"))
  ;[0 0.4286 1 1 65] Camera Code
  ;;[1 1 1 1 45] Combat Camera
  (:Pressed
    (GeneralCamera|SetCamera true)))

(event Input|KeyboardEvents|3
  (params (Key :type Key%20Structure :default "None"))
  ;[0 0.4286 1 1 65] Camera Code
  ;;[1 1 1 1 45] Normal Camera
  (:Pressed
    (GeneralCamera|SetCamera false)))

(event Input|MouseEvents|MouseWheelDown
  (params (Key :type Key%20Structure :default "None"))
  ;[0 0.4286 1 1 65] Camera Code
  ;;[1 1 1 1 45] Normal Camera
  (:Pressed
    (GeneralCamera|SetCamera false)))

(fn SetCamera
  (params (IsCombatCamera :type Boolean))
  (bind _output_get (Variables|Default|SetIsCombatCamera IsCombatCamera))
  (if _output_get
    (Variables|/Script/Engine.SpringArmComponent|SetTargetArmLength (Variables|Default|GetCameraBoom) (Variables|Default|GetCombatCameraArmLength))
    (else
      (Variables|/Script/Engine.SpringArmComponent|SetTargetArmLength (Variables|Default|GetCameraBoom) (Variables|Default|GetNormalCameraArmLength)))))

(fn GetCameraState
  (return (Variables|Default|GetIsCombatCamera)))

(fn UpdateCamera
  (params (Get%20IA_Look%20X :type Float%20%28double-precision%29) (Get%20IA_Look%20Y :type Float%20%28double-precision%29))
  (bind _cameraboom (Variables|Default|GetCameraBoom))
  (bind _relativerotation (Variables|/Script/Engine.SceneComponent|GetRelativeRotation _cameraboom))
  ;[1 1 1] Allows camera to flip with Gravity
  (Transformation|SetRelativeRotation (Variables|Default|GetCameraBoom) (Math|Rotator|MakeRotator 0.0 (Math|Float|Clamp(Float) (+ (.pitch _relativerotation) (* Get%20IA_Look%20Y (Variables|Default|GetSensitivityVertical) -1.0)) -4e+01 4e+01) (+ (.yaw _relativerotation) (* Get%20IA_Look%20X (Variables|Default|GetSensitivityHorzontal)))) false false)
  ;[1 1 1] Gravity Rotation for Detached Camera
  (Transformation|SetWorldLocationAndRotation (Variables|Default|GetCameraRoot) (Transformation|GetActorLocation (Variables|MainCharacterInfo|GetMainCharacter)) (Math|Rotator|MakeRotfromZX (Math|Vector|GetUnitDirection(Vector) (Transformation|GetWorldLocation (Variables|Default|GetCameraOrienter)) (Transformation|GetActorLocation (Variables|MainCharacterInfo|GetMainCharacter))) (Math|Vector|GetForwardVector (Variables|Default|GetCameraRoot))) false false))

(fn GetClosestEnemy
  (LocalVariables|SetDistance 1e+06)
  (for (_array_element _array_index) (Variables|/Game/Blueprints/AI/CombatManager/NewCombatManager.NewCombatManager_C|GetEnemies (Variables|/Game/MainCharacter/BP_MainCharacter.BP_MainCharacter_C|GetActiveCombatManager (Variables|MainCharacterInfo|GetMainCharacter)))
    (if (== _array_index 0)
      (LocalVariables|SetTargetActor _array_element))
    (Utilities|IsValid (LocalVariables|GetTargetActor)
      (:Is%20Valid
        (if (<= (Math|Vector|Distance(Vector) (Transformation|GetActorLocation _array_element) (Transformation|GetActorLocation (Variables|MainCharacterInfo|GetMainCharacter))) (LocalVariables|GetDistance))
          (LocalVariables|SetDistance (Math|Vector|Distance(Vector) (Transformation|GetActorLocation _array_element) (Transformation|GetActorLocation (Variables|MainCharacterInfo|GetMainCharacter))))
          (LocalVariables|SetTargetActor _array_element)))))
  (return (LocalVariables|GetTargetActor)))

(fn UpdateLockedCamera
  (params (IA_Look%20X :type Float%20%28double-precision%29) (IA_Look%20Y :type Float%20%28double-precision%29)))