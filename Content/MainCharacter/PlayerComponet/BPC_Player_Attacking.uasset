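; Player combat component that runs light and heavy sword attack combos on BP_MainCharacter.
; Each attack shows the sword, attaches Niagara mesh and ribbon trails, plays a montage selected by combo count, and updates the attack widget.
; An IsAttacking flag with a getter and setter gates attacks, while Tick feeds the mesh trail its location and rotation.
; HitStop freezes the character through custom time dilation until a timer restores it to reduced speed.
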(event Custom|Light%20Attack
  (bind _maincharacter (Variables|Player|GetMainCharacter))
  (bind _swordtraillocation (Variables|/Game/MainCharacter/BP_MainCharacter.BP_MainCharacter_C|GetSwordTrailLocation _maincharacter))
  (bind _asbp_main_character (Utilities|Casting|CastToBP_MainCharacter (Game|GetPlayerCharacter 0)))
  ;[1 1 1] New Light Attack Combo
  (Rendering|SetVisibility (Variables|/Game/MainCharacter/BP_MainCharacter.BP_MainCharacter_C|GetSword _asbp_main_character) true false)
  (if (not (Variables|Private|GetIsAttacking))
    (Variables|Private|SetIsAttacking true)
    (bind _returnvalue (Niagara|SpawnSystemAttached "/Game/VFX/NA_MeshSwordTrail.NA_MeshSwordTrail" _swordtraillocation "None" "0, 0, 0" "0, 0, 0" "SnapToTarget" true))
    (Variables|Default|SetMeshSwordTrail _returnvalue)
    (bind _returnvalue_2 (Niagara|SpawnSystemAttached "/Game/VFX/NA_SwordRibbon.NA_SwordRibbon" _swordtraillocation "None" "0, 0, 0" "0, 0, 0" "SnapToTarget" true))
    (Variables|Default|SetRibbonSwordTrail _returnvalue_2)
    (Animation|Montage|PlayMontage (Variables|/Script/Engine.Character|GetMesh (Variables|Player|GetMainCharacter)) (Utilities|Select :Index (Variables|Private|GetLight%20Attack%20Count) :Option%200 "/Game/CharacterModel/Folderforretarget/Anims/RigLight1Short.RigLight1Short" :Option%201 "/Game/CharacterModel/Folderforretarget/Anims/RigLight2Short.RigLight2Short" :Option%202 "/Game/CharacterModel/Folderforretarget/Anims/RigLight1Short.RigLight1Short")
      (:then
        (Utilities|IsValid (Variables|/Game/MainCharacter/BP_MainCharacter.BP_MainCharacter_C|GetAttackWidgetRef (Variables|Player|GetMainCharacter))
          (:Is%20Valid
            (Variables|/Game/Widget/CombatWidget.CombatWidget_C|SetAttackIndex (Variables|/Game/MainCharacter/BP_MainCharacter.BP_MainCharacter_C|GetAttackWidgetRef (Variables|Player|GetMainCharacter)) (Variables|Private|GetLight%20Attack%20Count))
            (bind _result (Math|Integer|IncrementInt (Variables|Private|GetLight%20Attack%20Count))
              (:%20%20
                (switch int _result
                  (:0
                    (Variables|Private|SetLightComboProgress 1))
                  (:1
                    (if (== (Variables|Private|GetLightComboProgress) 1)
                      (Variables|Private|SetLightComboProgress 2)))
                  (:2
                    (if (== (Variables|Private|GetLightComboProgress) 2)
                      (Variables|/Game/MainCharacter/BP_MainCharacter.BP_MainCharacter_C|SetAttackWidgetRef (Variables|Player|GetMainCharacter) 0)
                      (bind _output_get (Variables|Private|SetLightComboProgress 3))
                      (Variables|/Game/Widget/CombatWidget.CombatWidget_C|SetAttackIndex (Variables|/Game/MainCharacter/BP_MainCharacter.BP_MainCharacter_C|GetAttackWidgetRef (Variables|Player|GetMainCharacter)) _output_get)))))))))
      (:OnCompleted
        (Variables|Private|SetLight%20Attack%20Count 0 :!label _label)
        (Utilities|FlowControl|Sequence
          (:then_0
            (Utilities|FlowControl|Delay 3.0)
            (Rendering|SetVisibility (Variables|/Game/MainCharacter/BP_MainCharacter.BP_MainCharacter_C|GetSword _asbp_main_character) false false))))
      (:OnInterrupted
        (Utilities|FlowControl|RetriggerableDelay 1.0)
        (Variables|Private|SetIsAttacking false)
        (goto _label)))))

(event Custom|Heavy%20Attack
  (bind _maincharacter (Variables|Player|GetMainCharacter))
  (bind _swordtraillocation (Variables|/Game/MainCharacter/BP_MainCharacter.BP_MainCharacter_C|GetSwordTrailLocation _maincharacter))
  (bind _asbp_main_character (Utilities|Casting|CastToBP_MainCharacter (Game|GetPlayerCharacter 0)))
  (Rendering|SetVisibility (Variables|/Game/MainCharacter/BP_MainCharacter.BP_MainCharacter_C|GetSword _asbp_main_character) true false)
  ;[1 1 1] New Heavy Attach Combo
  (if (not (Variables|Private|GetIsAttacking))
    (Variables|Private|SetIsAttacking true)
    (bind _returnvalue (Niagara|SpawnSystemAttached "/Game/VFX/NA_MeshSwordTrail.NA_MeshSwordTrail" _swordtraillocation "None" "0, 0, 0" "0, 0, 0" "SnapToTarget" true))
    (Variables|Default|SetMeshSwordTrail _returnvalue)
    (bind _returnvalue_2 (Niagara|SpawnSystemAttached "/Game/VFX/NA_SwordRibbon.NA_SwordRibbon" _swordtraillocation "None" "0, 0, 0" "0, 0, 0" "SnapToTarget" true))
    (Variables|Default|SetRibbonSwordTrail _returnvalue_2)
    (Animation|Montage|PlayMontage (Variables|/Script/Engine.Character|GetMesh (Variables|Player|GetMainCharacter)) (Utilities|Select :Index (Variables|Private|GetHeavy%20Attack%20Count) :Option%200 "/Game/CharacterModel/Folderforretarget/HeavyAttacks/RigHeavy1Short.RigHeavy1Short" :Option%201 "/Game/CharacterModel/Folderforretarget/HeavyAttacks/RigHeavy2Short.RigHeavy2Short" :Option%202 "/Game/CharacterModel/Folderforretarget/HeavyAttacks/RigHeavy3Short.RigHeavy3Short")
      (:then
        (Utilities|IsValid (Variables|/Game/MainCharacter/BP_MainCharacter.BP_MainCharacter_C|GetAttackWidgetRef (Variables|Player|GetMainCharacter))
          (:Is%20Valid
            (Variables|/Game/Widget/CombatWidget.CombatWidget_C|SetHeavyAttackIndex (Variables|/Game/MainCharacter/BP_MainCharacter.BP_MainCharacter_C|GetAttackWidgetRef (Variables|Player|GetMainCharacter)) (Variables|Private|GetHeavy%20Attack%20Count))
            (bind _result (Math|Integer|IncrementInt (Variables|Private|GetHeavy%20Attack%20Count))
              (:%20%20
                (switch int _result
                  (:0
                    (Variables|Private|SetHeavyComboProgress 1))
                  (:1
                    (if (== (Variables|Private|GetHeavyComboProgress) 1)
                      (Variables|Private|SetHeavyComboProgress 2)))
                  (:2
                    (if (== (Variables|Private|GetHeavyComboProgress) 2)
                      (Variables|/Game/MainCharacter/BP_MainCharacter.BP_MainCharacter_C|SetAttackWidgetRef (Variables|Player|GetMainCharacter) 0)
                      (bind _output_get (Variables|Private|SetHeavyComboProgress 3))
                      (Variables|/Game/Widget/CombatWidget.CombatWidget_C|SetAttackIndex (Variables|/Game/MainCharacter/BP_MainCharacter.BP_MainCharacter_C|GetAttackWidgetRef (Variables|Player|GetMainCharacter)) _output_get)))))))))
      (:OnCompleted
        (Variables|Private|SetHeavy%20Attack%20Count 0 :!label _label)
        (Utilities|FlowControl|Delay 3.0)
        (Rendering|SetVisibility (Variables|/Game/MainCharacter/BP_MainCharacter.BP_MainCharacter_C|GetSword _asbp_main_character) false false))
      (:OnInterrupted
        (Utilities|FlowControl|RetriggerableDelay 1.0)
        (Variables|Private|SetIsAttacking false)
        (goto _label)))))

(event EventBeginPlay
  (bind _asbp_main_character (Utilities|Casting|CastToBP_MainCharacter (Game|Player|GetPlayerPawn 0))
    (:then
      (Variables|Player|SetMainCharacter _asbp_main_character))
    (:CastFailed
      (Development|PrintString "ERROR[BPC_Player_Attacking]: Start Can't cast maincharacter" false false "(R=1.000000,G=0.023616,B=0.000000,A=1.000000)" 1.5e+02))))

(event EventTick
  (params (DeltaSeconds :type Float%20%28single-precision%29))
  (bind _meshswordtrail (Variables|Default|GetMeshSwordTrail))
  (Utilities|IsValid _meshswordtrail
    (:Is%20Valid
      (Niagara|SetNiagaraVariable(Vector3) _meshswordtrail "User_TrailLocation" (Transformation|GetWorldLocation _meshswordtrail))
      (Class|NiagaraComponent|SetVariableQuat _meshswordtrail "User_TrailRotation2" (Math|Conversions|ToQuaternion(Rotator) (Transformation|GetWorldRotation _meshswordtrail))))))

(fn GetIsAttacking
  (return (Variables|Private|GetIsAttacking)))

(fn SetIsAttacking
  (params (IsAttacking :type Boolean))
  (Variables|Private|SetIsAttacking IsAttacking))

(fn HitStop
  (params (Duration :type Float%20%28double-precision%29))
  (Variables|/Script/Engine.Actor|SetCustomTimeDilation (Variables|Player|GetMainCharacter) 0.0)
  (Utilities|Time|SetTimerbyFunctionName 0 "EndHitstop" Duration))

(fn EndHitstop
  (Variables|/Script/Engine.Actor|SetCustomTimeDilation (Variables|Player|GetMainCharacter) 0.6))