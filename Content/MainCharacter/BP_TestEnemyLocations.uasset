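; Test actor that exercises the EnemyLocations component, building and ordering ring-shaped move points around a ground origin.
; On BeginPlay it creates inner and outer angle-offset rings, then traces for an origin, falling back to the actor location.
; It orders the points by their computed positions and calls DelayPointsInOrder over one second.
; The trace end is not offset from the actor's location, and the per-frame DebugPoints path is disconnected from Tick.
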(event EventBeginPlay
  (bind _returnvalue (Transformation|GetActorLocation))
  (bind _enemylocations (Variables|Default|GetEnemyLocations))
  (bind _enemylocations_2 (Variables|Default|GetEnemyLocations))
  (bind _enemylocations_3 (Variables|Default|GetEnemyLocations))
  (bind _enemylocations_4 (Variables|Default|GetEnemyLocations))
  (Variables|/Game/MainCharacter/EnemyLocations.EnemyLocations_C|SetMovePoints (Variables|Default|GetEnemyLocations) (Utilities|Array|MakeArray))
  (Utilities|Array|AppendArray (Variables|/Game/MainCharacter/EnemyLocations.EnemyLocations_C|GetMovePoints _enemylocations) (Default|CreateRing _enemylocations 6 3e+01 2.5e+02))
  (Utilities|Array|AppendArray (Variables|/Game/MainCharacter/EnemyLocations.EnemyLocations_C|GetMovePoints _enemylocations_3) (Default|CreateRing _enemylocations_3 12 15.0 5e+02))
  (bind (_outhit _returnvalue_2) (Collision|LineTraceByChannel (Transformation|GetActorLocation) (* (Transformation|GetActorUpVector) -5e+03) "TraceTypeQuery1" false 0 "None"))
  (if _returnvalue_2
    (Default|OrderPoints _enemylocations_4 (Variables|/Game/MainCharacter/EnemyLocations.EnemyLocations_C|GetMovePoints _enemylocations_4) (Default|CalcAllPointPos _enemylocations_4 (.Location (Collision|BreakHitResult _outhit))))
    (Default|DelayPointsinOrder (Variables|Default|GetEnemyLocations) (.Location (Collision|BreakHitResult _outhit)) 1.0)
    (else
      (Default|OrderPoints _enemylocations_2 (Variables|/Game/MainCharacter/EnemyLocations.EnemyLocations_C|GetMovePoints _enemylocations_2) (Default|CalcAllPointPos _enemylocations_2 _returnvalue))
      (Default|DelayPointsinOrder (Variables|Default|GetEnemyLocations) _returnvalue 1.0))))

(event EventTick
  (params (DeltaSeconds :type Float%20%28single-precision%29)))

(fn ConstructionScript)