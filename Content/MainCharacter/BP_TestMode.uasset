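; Test game mode that tracks the grunt enemy count and handles player respawns.
; On BeginPlay it counts BP_AI_Grunt actors to set EnemiesLeft and TotalEnemies, then prints the total.
; Respawn destroys the current BP_MainCharacter, spawns a new one at the LastCheckpoint's POSSkeletalMesh transform and possesses it.
; Without a valid checkpoint, the new character spawns at the default transform.
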(event Custom|Respawn
  (Utilities|Casting|CastToBP_MainCharacter (Game|Player|GetPlayerPawn 0))
  (Actor|DestroyActor (Game|GetPlayerCharacter 0))
  (bind _last_checkpoint (Variables|Default|Getlast%20Checkpoint)
    (:then
      (bind _returnvalue (Game|SpawnActorfromClass "/Game/MainCharacter/BP_MainCharacter.BP_MainCharacter_C" (Math|Transform|MakeTransform (.location (Transformation|GetWorldTransform (Variables|/Game/Blueprints/BP_CheckPoint.BP_CheckPoint_C|GetPOSSkeletalMesh _last_checkpoint))) (.rotation (Transformation|GetWorldTransform (Variables|/Game/Blueprints/BP_CheckPoint.BP_CheckPoint_C|GetPOSSkeletalMesh _last_checkpoint))) "1.000000,1.000000,1.000000") "AlwaysSpawn" "MultiplyWithRoot" 0 0))
      (Pawn|Possess (Game|GetPlayerController 0) _returnvalue))
    (:else
      (bind _returnvalue_2 (Game|SpawnActorfromClass "/Game/MainCharacter/BP_MainCharacter.BP_MainCharacter_C" (Math|Transform|MakeTransform "0, 0, 0" "0, 0, 0" "1.000000,1.000000,1.000000") "Undefined" "MultiplyWithRoot" 0 0))
      (Pawn|Possess (Game|GetPlayerController 0) _returnvalue_2)))
  (Utilities|Casting|CastToBP_MainCharacter (Game|Player|GetPlayerPawn 0)))

(event EventBeginPlay
  ;[1 0.01606 0] EnemiesLeft
  (bind _outactors (Actor|GetAllActorsOfClass "/Game/Blueprints/AI/EnemyCatalog/Grunt/BP_AI_Grunt.BP_AI_Grunt_C"))
  (bind _output_get (Variables|Default|SetEnemiesLeft (Utilities|Array|Length _outactors)))
  (bind _output_get_2 (Variables|Default|SetTotalEnemies _output_get))
  (Development|PrintString (Utilities|String|ToString(Integer) _output_get_2) false false))

(fn ConstructionScript)