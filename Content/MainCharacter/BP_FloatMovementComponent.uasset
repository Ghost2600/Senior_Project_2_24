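; Actor component for BP_MainCharacter that toggles a floating movement state and handles vertical float input.
; EnableFloatMovement zeroes gravity and switches to Flying; DisableFloatMovement restores the gravity scale cached at BeginPlay and returns to Walking.
; While floating, FloatUp and FloatDown add a single vertical movement input per press, with no continuous update on Tick.
; Direction flags are set but never read here, and FloatDown's release leaves IsMovingDown true.
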(event EventBeginPlay
  (bind _asbp_main_character (Utilities|Casting|CastToBP_MainCharacter (Components|GetOwner)))
  (Variables|Default|SetMainCharacter _asbp_main_character)
  (Variables|Default|SetDefaultGravityScale (Variables|/Script/Engine.CharacterMovementComponent|GetGravityScale (Variables|/Script/Engine.Character|GetCharacterMovement _asbp_main_character))))

(event EventTick
  (params (DeltaSeconds :type Float%20%28single-precision%29)))

(event Input|ActionEvents|InputActionFloatUp
  (params (Key :type Key%20Structure :default "None"))
  (:Pressed
    (Variables|Default|SetisMovingUp true)
    (if (Variables|Default|GetIsFloating?)
      (Pawn|Input|AddMovementInput (Variables|/Script/Engine.Actor|GetInstigator (Components|GetOwner)) (Math|Vector|GetUpVector "0.000000,1.000000,0.000000") 1.0 false)))
  (:Released
    (Variables|Default|SetisMovingUp false)))

(event Input|ActionEvents|InputActionFloatDown
  (params (Key :type Key%20Structure :default "None"))
  (:Pressed
    (Variables|Default|SetisMovingDown true)
    (if (Variables|Default|GetIsFloating?)
      (Pawn|Input|AddMovementInput (Variables|/Script/Engine.Actor|GetInstigator (Components|GetOwner)) (Math|Vector|MakeVector 0.0 0.0 -1.0) 1.0 false)))
  (:Released
    (Variables|Default|SetisMovingDown true)))

(fn EnableFloatMovement
  (if (not (Variables|Default|GetIsFloating?))
    (bind _asbp_main_character (Utilities|Casting|CastToBP_MainCharacter (Components|GetOwner)))
    (Variables|/Script/Engine.CharacterMovementComponent|SetGravityScale (Variables|/Script/Engine.Character|GetCharacterMovement _asbp_main_character) 0.0)
    (Pawn|Components|CharacterMovement|SetMovementMode (Variables|/Script/Engine.Character|GetCharacterMovement _asbp_main_character) "MOVE_Flying" 0)
    (Variables|Default|SetIsFloating? true)
    (Development|PrintString "Enable Floating Called")))

(fn DisableFloatMovement
  (if (Variables|Default|GetIsFloating?)
    (bind _asbp_main_character (Utilities|Casting|CastToBP_MainCharacter (Components|GetOwner)))
    (Variables|/Script/Engine.CharacterMovementComponent|SetGravityScale (Variables|/Script/Engine.Character|GetCharacterMovement _asbp_main_character) (Variables|Default|GetDefaultGravityScale))
    (Pawn|Components|CharacterMovement|SetMovementMode (Variables|/Script/Engine.Character|GetCharacterMovement _asbp_main_character) "MOVE_Walking" 0)
    (Variables|Default|SetIsFloating? false)
    (Development|PrintString "Disable Float")))