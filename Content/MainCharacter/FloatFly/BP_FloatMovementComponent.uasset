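; Actor component that gives BP_MainCharacter a free-rotating float/fly mode.
; Enable and disable functions switch gravity, movement mode, camera and mesh animation.
; Tick derives forward and right directions on the character's local up-vector plane; Movement uses them for swept SetActorLocation moves and spawns a Niagara trail.
; Rotation and Roll events apply local pitch, yaw and roll; some older vertical-input and reticle logic is unconnected.
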(event Custom|Movement
  (params (X%20Val :type Float%20%28double-precision%29) (Y%20Val :type Float%20%28double-precision%29))
  (bind _returnvalue (Class|KismetMathLibrary|VectorNormal2D (Math|Vector|MakeVector X%20Val Y%20Val 0.0) 0.0001))
  (Utilities|FlowControl|Sequence
    (:then_0
      (Transformation|SetActorLocation (Variables|Default|GetMainCharacter) (+ (* (+ (* (Variables|Movement|GetRightDir) (.x _returnvalue)) (* (Variables|Movement|GetForwardDir) (.y _returnvalue))) (Variables|Movement|GetMoveSpeed) (Variables|Default|GetDeltaTime)) (Transformation|GetActorLocation (Variables|Default|GetMainCharacter))) true false))
    (:then_2
      ;[1 1 1] Particle Effect
      (Niagara|SpawnSystematLocation "/Game/VFX/Placeholder/NS_PlayerTrail.NS_PlayerTrail" (Transformation|GetWorldLocation (Variables|/Game/MainCharacter/BP_MainCharacter.BP_MainCharacter_C|GetPlayer%20Trail (Variables|Default|GetMainCharacter)))))))

(event Custom|Rotation
  (params (X%20Val :type Float%20%28double-precision%29) (Y%20Val :type Float%20%28double-precision%29))
  (Utilities|FlowControl|Sequence
    (:then_0
      (Transformation|AddActorLocalRotation (Variables|Default|GetMainCharacter) (Math|Rotator|MakeRotator 0.0 (* Y%20Val (Variables|Default|GetRotationSpeed) (Variables|Default|GetDeltaTime) -1.0) 0.0) false false))
    (:then_1
      (Transformation|AddActorLocalRotation (Variables|Default|GetMainCharacter) (Math|Rotator|MakeRotator 0.0 0.0 (* X%20Val (Variables|Default|GetRotationSpeed) (Variables|Default|GetDeltaTime))) false false))))

(event Custom|Roll
  (params (Val :type Float%20%28double-precision%29))
  (Transformation|AddActorLocalRotation (Variables|Default|GetMainCharacter) (Math|Rotator|MakeRotator (* Val (Variables|Default|GetRotationSpeed) (Variables|Default|GetDeltaTime)) 0.0 0.0) false false))

(event EventBeginPlay
  (bind _asbp_main_character (Utilities|Casting|CastToBP_MainCharacter (Components|GetOwner)))
  (Variables|Default|SetMainCharacter _asbp_main_character)
  (Variables|Default|SetDefaultGravityScale (Variables|/Script/Engine.CharacterMovementComponent|GetGravityScale (Variables|/Script/Engine.Character|GetCharacterMovement _asbp_main_character)))
  (if (Variables|Default|GetIsFloating?)
    (bind _returnvalue (UserInterface|CreateWidget "/Game/Widget/ReticleWdiget.ReticleWdiget_C"))
    (UserInterface|Viewport|AddtoViewport _returnvalue 0)))

(event EventTick
  (params (DeltaSeconds :type Float%20%28single-precision%29))
  (bind _maincharacter (Variables|Default|GetMainCharacter))
  (Variables|Default|SetDeltaTime DeltaSeconds)
  (Variables|Movement|SetPlaneOfMovement (CallFunction|CreatePlane (Transformation|GetActorUpVector _maincharacter) (Transformation|GetActorLocation _maincharacter)))
  (Variables|Movement|SetForwardDir (Math|Vector|Normalize (- (CallFunction|GetClosestPointtoPlane (Variables|Movement|GetPlaneOfMovement) (Transformation|GetActorForwardVector (Variables|Default|GetMainCharacter))) (CallFunction|GetClosestPointtoPlane (Variables|Movement|GetPlaneOfMovement) "0, 0, 0"))))
  (Variables|Movement|SetRightDir (Math|Vector|Normalize (- (CallFunction|GetClosestPointtoPlane (Variables|Movement|GetPlaneOfMovement) (Transformation|GetActorRightVector (Variables|Default|GetMainCharacter))) (CallFunction|GetClosestPointtoPlane (Variables|Movement|GetPlaneOfMovement) "0, 0, 0")))))

(fn EnableFloatMovement
  (bind _maincharacter (Variables|Default|GetMainCharacter))
  (bind _maincharacter_2 (Variables|Default|GetMainCharacter))
  (bind _player_camera (Variables|/Game/MainCharacter/BP_MainCharacter.BP_MainCharacter_C|GetPlayer_Camera _maincharacter_2))
  (bind _mesh (Variables|/Script/Engine.Character|GetMesh _maincharacter))
  (Default|PuzzleLockOff _player_camera)
  (Default|SetCamera _player_camera "NewEnumerator2")
  (Default|SetCameraBehindPlayer (Variables|/Game/MainCharacter/BP_MainCharacter.BP_MainCharacter_C|GetPlayer_Camera (Variables|Default|GetMainCharacter)))
  (if (not (Variables|Default|GetIsFloating?))
    (bind _asbp_main_character (Utilities|Casting|CastToBP_MainCharacter (Components|GetOwner)))
    (Variables|/Script/Engine.CharacterMovementComponent|SetGravityScale (Variables|/Script/Engine.Character|GetCharacterMovement _asbp_main_character) 0.0)
    (Pawn|Components|CharacterMovement|SetMovementMode (Variables|/Script/Engine.Character|GetCharacterMovement _asbp_main_character) "MOVE_Flying" 0)
    (Variables|Default|SetIsFloating? true)
    (Development|PrintString "Enable Floating Called")
    (Components|Animation|PlayAnimation _mesh "/Game/CharacterModel/Folderforretarget/Anims/TakingOff.TakingOff" false)
    (bind _asbp_main_character_2 (Utilities|Casting|CastToBP_MainCharacter (Game|GetPlayerCharacter 0)))
    (if (< (Math|Vector|VectorLength (Transformation|GetVelocity _asbp_main_character_2)) 0.2)
      (Components|Animation|PlayAnimation _mesh "/Game/CharacterModel/Folderforretarget/Anims/FlyingIdle__1_.FlyingIdle__1_" true)
      (else
        (Components|Animation|PlayAnimation _mesh "/Game/CharacterModel/Folderforretarget/Anims/FlyingMoving__1_.FlyingMoving__1_" true)))))

(fn DisableFloatMovement
  (Default|SetCamera (Variables|/Game/MainCharacter/BP_MainCharacter.BP_MainCharacter_C|GetPlayer_Camera (Variables|Default|GetMainCharacter)) "NewEnumerator0")
  (if (Variables|Default|GetIsFloating?)
    (bind _asbp_main_character (Utilities|Casting|CastToBP_MainCharacter (Components|GetOwner)))
    (Variables|/Script/Engine.CharacterMovementComponent|SetGravityScale (Variables|/Script/Engine.Character|GetCharacterMovement _asbp_main_character) (Variables|Default|GetDefaultGravityScale))
    (Pawn|Components|CharacterMovement|SetMovementMode (Variables|/Script/Engine.Character|GetCharacterMovement _asbp_main_character) "MOVE_Walking" 0)
    (Variables|Default|SetIsFloating? false)
    (Development|PrintString "Disable Float")
    (Components|Animation|SetAnimationMode (Variables|/Script/Engine.Character|GetMesh (Variables|Default|GetMainCharacter)) "AnimationBlueprint" true)
    (bind _asbp_main_character_2 (Utilities|Casting|CastToBP_MainCharacter (Game|GetPlayerCharacter 0)))
    (Utilities|IsValid (Variables|/Game/MainCharacter/BP_MainCharacter.BP_MainCharacter_C|GetReticleRef _asbp_main_character_2)
      (:Is%20Valid
        (Widget|RemovefromParent (Variables|/Game/MainCharacter/BP_MainCharacter.BP_MainCharacter_C|GetReticleRef _asbp_main_character_2))))))

(fn GetForward
  (return (Variables|Movement|GetForwardDir)))