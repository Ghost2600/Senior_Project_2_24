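; BP_StatueBlessing is an interactable blessing statue that gives audio and on-screen feedback, with no gameplay effect in this graph.
; Box overlap toggles player input on the actor and shows the prompt widget while WidgetBegone allows it.
; Interact, limited to BP_MainCharacter, plays a chorus sound, shows the activated widget and suppresses the prompt for a timed cooldown.
; A Timeline-driven pedestal material pulse exists but never runs.
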(event OnComponentBeginOverlap(Box)
  (params (OverlappedComponent :type Primitive%20Component%20Object%20Reference) (OtherActor :type Actor%20Object%20Reference) (OtherComp :type Primitive%20Component%20Object%20Reference) (OtherBodyIndex :type Integer) (bFromSweep :type Boolean) (SweepResult :type Hit%20Result%20Structure%20%28by%20ref%29))
  ;[1 1 1] Widget
  (if (Variables|Default|GetWidgetBegone)
    (Rendering|SetVisibility (Variables|Default|GetWidget) true false)
    (Input|EnableInput (Game|GetPlayerController 0))))

(event OnComponentEndOverlap(Box)
  (params (OverlappedComponent :type Primitive%20Component%20Object%20Reference) (OtherActor :type Actor%20Object%20Reference) (OtherComp :type Primitive%20Component%20Object%20Reference) (OtherBodyIndex :type Integer))
  ;[1 1 1] Widget
  (Rendering|SetVisibility (Variables|Default|GetWidget) false false)
  (Input|DisableInput (Game|GetPlayerController 0)))

(event EventInteract
  (params (Character :type BP%20Main%20Character%20Object%20Reference))
  (Utilities|Casting|CastToBP_MainCharacter Character)
  ;[1 1 1] Interact
  (Variables|Default|SetWidgetBegone false)
  (Utilities|FlowControl|Sequence
    (:then_0
      (Audio|PlaySound2D "/Game/Audio/Statues/chorus-low-note-43701.chorus-low-note-43701" 1.0 1.0 0.0 0 0)
      (Rendering|SetVisibility (Variables|Default|GetActivatedWidget) true false)
      (Utilities|FlowControl|Delay 12.0)
      (Rendering|SetVisibility (Variables|Default|GetActivatedWidget) false false)
      (Utilities|FlowControl|Delay 8.0))
    (:then_1
      (Rendering|SetVisibility (Variables|Default|GetWidget) false false)
      (Utilities|FlowControl|Delay 12.0)
      (Variables|Default|SetWidgetBegone true))))

(fn ConstructionScript)