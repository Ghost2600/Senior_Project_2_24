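; Beam reflector actor that, when hit by a light beam, re-casts it along its Arrow's forward direction with strength increased by one.
; ReflectLight line-traces up to CastDistance and sends a BeamHit message to the hit actor with the new strength, so receivers can continue the chain.
; Niagara effects show the loop and cast at the reflector, plus an impact on blocking hits; the trace also draws timed debug lines.
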(event EventBeginPlay)

(event Collision|EventActorBeginOverlap
  (params (OtherActor :type Actor%20Object%20Reference)))

(event EventBeamHit
  (params (BeamStrength :type Integer))
  (bind _arrow (Variables|Default|GetArrow))
  (CallFunction|ReflectLight (Transformation|GetWorldLocation _arrow) (Math|Vector|GetForwardVector _arrow) (Variables|Default|GetCastDistance) (+ BeamStrength 1)))

(fn ConstructionScript)

(fn ReflectLight
  (params (BeamOrigin :type Vector) (BeamDirection :type Vector) (CastDistance :type Float%20%28double-precision%29) (BeamStrength :type Integer))
  (bind _director (Variables|Default|GetDirector))
  (bind _returnvalue (Transformation|GetWorldLocation _director))
  (bind _returnvalue_2 (Transformation|GetWorldRotation _director))
  (LocalVariables|SetL_BeamOrigin BeamOrigin)
  (LocalVariables|SetL_BeamDirection BeamDirection)
  (LocalVariables|SetL_CastDistance CastDistance)
  (bind _outhit (Collision|LineTraceByChannel (LocalVariables|GetL_BeamOrigin) (+ (LocalVariables|GetL_BeamOrigin) (* (LocalVariables|GetL_BeamDirection) (LocalVariables|GetL_CastDistance))) "TraceTypeQuery4" false 0 "ForDuration" true "(R=1.000000,G=0.000000,B=0.000000,A=1.000000)" "(R=0.000000,G=1.000000,B=0.000000,A=1.000000)" 0.1))
  (Niagara|SpawnSystematLocation "/Game/VFX/Placeholder/NS_LightBeamLoop.NS_LightBeamLoop" (Math|Vector|MakeVector (.x _returnvalue) (.y _returnvalue) (.z _returnvalue)) _returnvalue_2)
  (Niagara|SpawnSystematLocation "/Game/VFX/Placeholder/NS_BeamCast.NS_BeamCast" (Transformation|GetWorldLocation (Variables|Default|GetSphere)) _returnvalue_2)
  (Class|BPIBeamHit|BeamHit(Message) (.HitActor (Collision|BreakHitResult _outhit)) BeamStrength)
  (if (.bBlockingHit (Collision|BreakHitResult _outhit))
    (Niagara|SpawnSystematLocation "/Game/VFX/Placeholder/NS_BeamHit.NS_BeamHit" (.ImpactPoint (Collision|BreakHitResult _outhit)) (* (LocalVariables|GetL_BeamDirection) -1.0))))