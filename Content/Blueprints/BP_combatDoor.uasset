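; Combat door actor that unlocks and slides open when its OpenDoor event is called.
; OpenDoor swaps two door material slots to an energy material, plays a 2D unlock sound and starts a timeline that lerps the door mesh downward.
; An unconnected BP_TestMode EnemiesLeft check never runs, so the trigger must come from outside this Blueprint.
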(event Custom|OpenDoor
  (params (Player :type Actor%20Object%20Reference))
  (Rendering|Material|SetMaterial (Variables|Default|GetDoor) 1 "/Game/Materials/M_Energy.M_Energy")
  (Rendering|Material|SetMaterial (Variables|Default|GetDoor) 3 "/Game/Materials/M_Energy.M_Energy")
  (Audio|PlaySound2D "/Game/Audio/Placeholders/Cues/SFX_SoundEffects/SFX_EnvironmentActors/Interactables/SFX_Door_Unlock_Head_Cue.SFX_Door_Unlock_Head_Cue" 1.0 1.0 0.0 0 0)
  (bind _openpuzzledoor (Timeline|Timeline Play)
    (:Update
      (Utilities|FlowControl|Sequence
        (:then_0
          (Transformation|SetRelativeLocation (Variables|Default|GetDoor) (Math|Vector|Lerp(Vector) "0, 0, 0" "0.000000,0.000000,-100.000000" _openpuzzledoor) false false))))))

(event EventBeginPlay)

(event Collision|EventActorBeginOverlap
  (params (OtherActor :type Actor%20Object%20Reference)))

(event EventTick
  (params (DeltaSeconds :type Float%20%28single-precision%29)))

(fn ConstructionScript)