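; BP_Mushroom is a mushroom actor that releases spores when the player touches it.
; Overlapping its Box with an actor tagged Player spawns the NS_MushroomSpores Niagara system at the SporeSpawn component, using the actor's rotation and the SporeSize scale.
; A timeline that would recolor its SpotLight and RectLight is present but never runs.
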(event OnComponentBeginOverlap(Box)
  (params (OverlappedComponent :type Primitive%20Component%20Object%20Reference) (OtherActor :type Actor%20Object%20Reference) (OtherComp :type Primitive%20Component%20Object%20Reference) (OtherBodyIndex :type Integer) (bFromSweep :type Boolean) (SweepResult :type Hit%20Result%20Structure%20%28by%20ref%29))
  (if (Actor|ActorHasTag OtherActor "Player")
    (Niagara|SpawnSystematLocation "/Game/VFX/Placeholder/NS_MushroomSpores.NS_MushroomSpores" (Transformation|GetWorldLocation (Variables|Default|GetSpore%20Spawn)) (Transformation|GetActorRotation) (Math|Conversions|ToVector(Float) (Variables|Default|GetSpore%20Size)))))

(fn ConstructionScript)