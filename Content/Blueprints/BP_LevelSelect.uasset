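; BP_LevelSelect is a level-select Blueprint that opens one of eight hard-coded maps, many apparently test or prototype levels such as combat rooms and look-and-feel spaces.
; Each LoadLevel function calls Open Level by Object Reference on a fixed world, with no parameters or shared logic.
; The event graph and construction script are empty, and nothing in the Blueprint calls these functions itself.
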(event EventBeginPlay)

(event EventTick
  (params (DeltaSeconds :type Float%20%28single-precision%29)))

(fn ConstructionScript)

(fn LoadLevel1
  (Game|OpenLevel(byObjectReference) "/Game/Levels/FinalLevels/MixedWorld.MixedWorld"))

(fn LoadLevel2
  (Game|OpenLevel(byObjectReference) "/Game/Levels/Testing/IsaacTestWorld.IsaacTestWorld"))

(fn LoadLevel3
  (Game|OpenLevel(byObjectReference) "/Game/Levels/PastRefrences/Level1_1.Level1_1"))

(fn LoadLevel4
  (Game|OpenLevel(byObjectReference) "/Game/Blueprints/AI/EnemyCatalog/TestingNewBase.TestingNewBase"))

(fn LoadLevel5
  (Game|OpenLevel(byObjectReference) "/Game/Levels/PastRefrences/MixedRoom.MixedRoom"))

(fn LoadLevel6
  (Game|OpenLevel(byObjectReference) "/Game/Levels/PastRefrences/CombatRoom4.CombatRoom4"))

(fn LoadLevel7
  (Game|OpenLevel(byObjectReference) "/Game/Levels/PastRefrences/RoomLookAndFeel.RoomLookAndFeel"))

(fn LoadLevel8
  (Game|OpenLevel(byObjectReference) "/Game/Levels/PastRefrences/MultiGravCombat.MultiGravCombat"))