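; BP_MovingPlatform2 is a platform that moves vertically when its BeamPlatformUp or BeamPlatformDown event is called with a number matching its PlatformValue.
; Each event restarts its own timeline, lerping the static mesh's relative location from zero to a fixed offset above or below.
; Both moves start from the relative origin, so moving down does not retrace a previous rise.
; BeginPlay caches Down and Up world positions, but the movement ignores them.
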(event EventBeginPlay
  (bind _output_get (Variables|Default|SetDown (Transformation|GetWorldLocation (Variables|Default|GetStaticMesh))))
  (Variables|Default|SetUp (Math|Vector|MakeVector (.x _output_get) (.y _output_get) (+ (.z _output_get) 6e+02))))

(event EventBeamPlatformUp
  (params (PlatformNumber :type Integer))
  (if (== PlatformNumber (Variables|Default|GetPlatformValue))
    (bind _platformupward (Timeline|Timeline_1 PlayFromStart)
      (:Update
        (Transformation|SetRelativeLocation (Variables|Default|GetStaticMesh) (Math|Vector|Lerp(Vector) "0, 0, 0" "0.000000,0.000000,400.000000" _platformupward) false false)))))

(event EventBeamPlatformDown
  (params (PlatformNumber :type Integer))
  (if (== PlatformNumber (Variables|Default|GetPlatformValue))
    (bind _platformupward (Timeline|Timeline PlayFromStart)
      (:Update
        (Transformation|SetRelativeLocation (Variables|Default|GetStaticMesh) (Math|Vector|Lerp(Vector) "0, 0, 0" "0.000000,0.000000,-400.000000" _platformupward) false false)))))

(fn ConstructionScript)