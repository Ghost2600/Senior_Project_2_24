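; BP_pathLights is a path light actor whose symbol holder mesh lights up when its number is called.
; BeginPlay creates a dynamic material instance from M_EvilSymbolHolder_Inst for the SymbolHolderBlenderCube mesh.
; BeamLighton compares the passed LightNum with the actor's LightValue and, on a match, plays a timeline.
; Each timeline update drives the material's ColorAVisibility parameter from the ON track and reapplies the material.
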(event EventBeginPlay
  (Rendering|Material|SetMaterial (Variables|Default|GetSymbolHolderBlender_Cube) 0 "/Game/Models/Details/M_EvilSymbolHolder1.M_EvilSymbolHolder1")
  (bind _returnvalue (Rendering|Material|CreateDynamicMaterialInstance (Variables|Default|GetSymbolHolderBlender_Cube) 0 "/Game/Models/Details/M_EvilSymbolHolder_Inst.M_EvilSymbolHolder_Inst" "None" :!class /Script/Engine.PrimitiveComponent))
  (bind _output_get (Variables|Default|SetLightMaterial _returnvalue))
  (Rendering|Material|SetScalarParameterValue _output_get "ColorAVisibility" (stale EventBeamLighton _on) :!class /Script/Engine.MaterialInstanceDynamic)
  (Rendering|Material|SetMaterial (Variables|Default|GetSymbolHolderBlender_Cube) 0 (Variables|Default|GetLightMaterial)))

(event EventBeamLighton
  (params (LightNum :type Integer))
  (if (== LightNum (Variables|Default|GetLight%20Value))
    (bind _on (Timeline|Timeline Play)
      (:Update
        (Rendering|Material|SetScalarParameterValue (stale EventBeginPlay _output_get) "ColorAVisibility" _on :!class /Script/Engine.MaterialInstanceDynamic)
        (Rendering|Material|SetMaterial (Variables|Default|GetSymbolHolderBlender_Cube) 0 (Variables|Default|GetLightMaterial))))))

(fn ConstructionScript)