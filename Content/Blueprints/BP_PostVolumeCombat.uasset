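; Combat post-process volume actor that fades post-process blend weight through a box trigger and a signal receiver.
; BP_MainCharacter entering the Box calls StartVolume, whose timeline drives blend weight from its track, though this call passes no volumes.
; SignalReceiver activation calls ReleaseVolume on PostProcess, using a second timeline to lerp blend weight from full to zero.
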(event OnComponentBeginOverlap(Box)
  (params (OverlappedComponent :type Primitive%20Component%20Object%20Reference) (OtherActor :type Actor%20Object%20Reference) (OtherComp :type Primitive%20Component%20Object%20Reference) (OtherBodyIndex :type Integer) (bFromSweep :type Boolean) (SweepResult :type Hit%20Result%20Structure%20%28by%20ref%29))
  (Utilities|Casting|CastToBP_MainCharacter OtherActor)
  (CallFunction|StartVolume))

(event ActivateReceiver(SignalReceiver)
  (CallFunction|ReleaseVolume (Utilities|Array|MakeArray (Variables|Default|GetPostProcess))))

(event Custom|StartVolume
  (params (Volume :type Array%20of%20Post%20Process%20Component%20Object%20References))
  (bind _newtrack_0 (Timeline|Timeline_0 Play)
    (:Update
      (for _array_element Volume
        (Variables|/Script/Engine.PostProcessComponent|SetBlendWeight _array_element _newtrack_0)))))

(event Custom|ReleaseVolume
  (params (Volume :type Array%20of%20Post%20Process%20Component%20Object%20References))
  (bind _newtrack_0 (Timeline|Timeline Play)
    (:Update
      (for _array_element Volume
        (Variables|/Script/Engine.PostProcessComponent|SetBlendWeight _array_element (Math|Float|Lerp 1.0 0.0 _newtrack_0))))))

(fn ConstructionScript)