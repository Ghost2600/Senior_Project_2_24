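; Beam receptor that raises numbered moving platforms when hit by a strong enough beam.
; BeamHit spawns an activation effect and sends up messages to all BP_MovingPlatform actors with its platform number, or down messages when strength falls short.
; BeamMissing repeats the activation when missing strength meets the requirement, but leaves AcceptorActivated unset.
; ReflectLight, uncalled here, line-traces onward and forwards beam strength.
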(event Custom|BeamMissing
  (params (StrengthMissing :type Integer))
  (bind _cube (Variables|Default|GetCube))
  (if (>= StrengthMissing (Variables|Default|GetStrengthRequirement))
    (if (not (Variables|Default|GetAcceptorActivated))
      (Niagara|SpawnSystematLocation "/Game/VFX/Placeholder/NS_ReceptorOn.NS_ReceptorOn" (Transformation|GetWorldLocation _cube) (Transformation|GetWorldRotation _cube))
      (bind _outactors (Actor|GetAllActorsOfClass "/Game/Blueprints/BP_MovingPlatform.BP_MovingPlatform_C"))
      (Class|BPIBeamPlatformUp|BeamPlatformUp(Message) _outactors (Variables|Default|GetBeamPlatformNumber)))))

(event EventBeginPlay)

(event Collision|EventActorBeginOverlap
  (params (OtherActor :type Actor%20Object%20Reference)))

(event EventBeamHit
  (params (BeamStrength :type Integer))
  (bind _cube (Variables|Default|GetCube))
  (if (>= BeamStrength (Variables|Default|GetStrengthRequirement))
    (if (not (Variables|Default|GetAcceptorActivated))
      (Niagara|SpawnSystematLocation "/Game/VFX/Placeholder/NS_ReceptorOn.NS_ReceptorOn" (Transformation|GetWorldLocation _cube) (Transformation|GetWorldRotation _cube))
      (bind _outactors (Actor|GetAllActorsOfClass "/Game/Blueprints/BP_MovingPlatform.BP_MovingPlatform_C"))
      (Class|BPIBeamPlatformUp|BeamPlatformUp(Message) _outactors (Variables|Default|GetBeamPlatformNumber))
      (Variables|Default|SetAcceptorActivated true)
      (Development|PrintString "Accepted"))
    (else
      (Variables|Default|SetAcceptorActivated false)
      (bind _outactors_2 (Actor|GetAllActorsOfClass "/Game/Blueprints/BP_MovingPlatform.BP_MovingPlatform_C"))
      (Class|BPIBeamPlatformDown|BeamPlatformDown(Message) _outactors_2 (Variables|Default|GetBeamPlatformNumber))
      (Development|PrintString "Gone"))))

(fn ConstructionScript)

(fn ReflectLight
  (params (BeamOrigin :type Vector) (BeamDirection :type Vector) (CastDistance :type Float%20%28double-precision%29) (BeamStrength :type Integer))
  (Development|PrintString (Utilities|String|ToString(Integer) BeamStrength))
  (LocalVariables|SetL_BeamOrigin BeamOrigin)
  (LocalVariables|SetL_BeamDirection BeamDirection)
  (LocalVariables|SetL_CastDistance CastDistance)
  (bind _outhit (Collision|LineTraceByChannel (LocalVariables|GetL_BeamOrigin) (+ (LocalVariables|GetL_BeamOrigin) (* (LocalVariables|GetL_BeamDirection) (LocalVariables|GetL_CastDistance))) "TraceTypeQuery1" false 0 "ForDuration" true "(R=1.000000,G=0.000000,B=0.000000,A=1.000000)" "(R=0.000000,G=1.000000,B=0.000000,A=1.000000)" 0.1))
  (Class|BPIBeamHit|BeamHit(Message) (.HitActor (Collision|BreakHitResult _outhit)) BeamStrength))