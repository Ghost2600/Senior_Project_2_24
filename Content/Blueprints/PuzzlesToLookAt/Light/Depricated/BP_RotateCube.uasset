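; Deprecated light-puzzle cube that rotates when the main character interacts with it.
; Box overlap shows a widget and enables player input on the actor, and leaving hides and disables both.
; The Interact event casts to BP_MainCharacter, then calls RotateCube, which adds an instant 90-degree local rotation to the root component.
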(event OnComponentBeginOverlap(Box)
  (params (OverlappedComponent :type Primitive%20Component%20Object%20Reference) (OtherActor :type Actor%20Object%20Reference) (OtherComp :type Primitive%20Component%20Object%20Reference) (OtherBodyIndex :type Integer) (bFromSweep :type Boolean) (SweepResult :type Hit%20Result%20Structure%20%28by%20ref%29))
  ;[1 1 1] Widget
  (Rendering|SetVisibility (Variables|Default|GetWidget) true false)
  (Input|EnableInput (Game|GetPlayerController 0)))

(event OnComponentEndOverlap(Box)
  (params (OverlappedComponent :type Primitive%20Component%20Object%20Reference) (OtherActor :type Actor%20Object%20Reference) (OtherComp :type Primitive%20Component%20Object%20Reference) (OtherBodyIndex :type Integer))
  ;[1 1 1] Widget
  (Rendering|SetVisibility (Variables|Default|GetWidget) false false)
  (Input|DisableInput (Game|GetPlayerController 0)))

(event Custom|RotateCube
  (Transformation|AddLocalRotation (Variables|Default|GetDefaultSceneRoot) "0.000000,90.000000,0.000000" false false))

(event EventInteract
  (params (Character :type BP%20Main%20Character%20Object%20Reference))
  (Utilities|Casting|CastToBP_MainCharacter Character)
  (CallFunction|RotateCube))

(fn ConstructionScript)