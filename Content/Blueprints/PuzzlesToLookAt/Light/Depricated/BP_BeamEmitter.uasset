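; Light puzzle beam emitter, kept in a deprecated folder, that casts a beam along its Arrow component.
; Every Tick, ReflectLight line-traces forward and sends BeamOnMessage with beam strength to the hit actor.
; It spawns fresh cast and loop Niagara effects at the Sphere each frame, plus an impact effect on blocking hits.
; Despite the function's name, it performs a single trace with no bounce.
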(event EventTick
  (params (DeltaSeconds :type Float%20%28single-precision%29))
  (bind _arrow (Variables|Default|GetArrow))
  (CallFunction|ReflectLight (Transformation|GetWorldLocation _arrow) (Math|Vector|GetForwardVector _arrow) (Variables|Default|GetCastDistance) 1))

(fn ConstructionScript)

(fn ReflectLight
  (params (BeamOrigin :type Vector) (BeamDirection :type Vector) (CastDistance :type Float%20%28double-precision%29) (BeamStrength :type Integer))
  (bind _sphere (Variables|Default|GetSphere))
  (bind _sphere_2 (Variables|Default|GetSphere))
  (bind _returnvalue (Transformation|GetWorldLocation _sphere_2))
  (bind _returnvalue_2 (Transformation|GetWorldLocation _sphere))
  (LocalVariables|SetL_BeamOrigin BeamOrigin)
  (LocalVariables|SetL_BeamDirection BeamDirection)
  (LocalVariables|SetL_CastDistance CastDistance)
  (bind _outhit (Collision|LineTraceByChannel (LocalVariables|GetL_BeamOrigin) (+ (LocalVariables|GetL_BeamOrigin) (* (LocalVariables|GetL_BeamDirection) (LocalVariables|GetL_CastDistance))) "TraceTypeQuery4" false 0 "None" true "(R=1.000000,G=0.000000,B=0.000000,A=1.000000)" "(R=0.000000,G=1.000000,B=0.000000,A=1.000000)" 0.1))
  (Niagara|SpawnSystematLocation "/Game/VFX/Placeholder/NS_BeamCast.NS_BeamCast" (Math|Vector|MakeVector (.x _returnvalue) (.y _returnvalue) (.z _returnvalue)) (Transformation|GetWorldRotation (Variables|Default|GetDirector)))
  (Niagara|SpawnSystematLocation "/Game/VFX/Placeholder/NS_LightBeamLoop.NS_LightBeamLoop" (Math|Vector|MakeVector (.x _returnvalue_2) (.y _returnvalue_2) (.z _returnvalue_2)) (Transformation|GetWorldRotation (Variables|Default|GetDirector)))
  (Class|BPIBeamHit|Beamon(Message) (.HitActor (Collision|BreakHitResult _outhit)) (Variables|Default|GetBeamStrength))
  (if (.bBlockingHit (Collision|BreakHitResult _outhit))
    (Niagara|SpawnSystematLocation "/Game/VFX/Placeholder/NS_BeamHit.NS_BeamHit" (.ImpactPoint (Collision|BreakHitResult _outhit)) (* (LocalVariables|GetL_BeamDirection) -1.0))))