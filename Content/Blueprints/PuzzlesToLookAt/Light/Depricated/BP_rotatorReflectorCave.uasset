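; Cave light-puzzle reflector that relays an incoming beam along its arrow and can act as a signal trigger.
; Each Beamon call line-traces forward from the arrow, spawns a Niagara beam at VFXDistance and messages the hit actor with strength raised by one, letting reflectors chain.
; When incoming strength meets StrengthRequirement, it switches its SignalSender on; nothing here switches it off or rotates the reflector.
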(event EventBeamon
  (params (BeamStrength :type Integer) (SenderActor :type Actor%20Object%20Reference))
  (bind _arrow (Variables|Default|GetArrow))
  (Utilities|FlowControl|Sequence
    (:then_0
      (CallFunction|ReflectLight (Transformation|GetWorldLocation _arrow) (Math|Vector|GetForwardVector _arrow) (Variables|Default|GetCastDistance) (+ BeamStrength 1)))
    (:then_1
      (if (>= BeamStrength (Variables|Default|GetStrengthRequirement))
        ;[1 1 1] Activate
        (if (not (Default|GetSignal (Variables|Default|GetSignalSender)))
          (Utilities|FlowControl|Sequence
            (:then_0
              (Default|SetSignal (Variables|Default|GetSignalSender) true))))))))

(fn ConstructionScript)

(fn ReflectLight
  (params (BeamOrigin :type Vector) (BeamDirection :type Vector) (CastDistance :type Float%20%28double-precision%29) (BeamStrength :type Integer))
  (bind _vfxdistance (Variables|Default|GetVFXDistance))
  (bind _returnvalue (Transformation|GetWorldLocation _vfxdistance))
  (LocalVariables|SetL_BeamOrigin BeamOrigin)
  (LocalVariables|SetL_BeamDirection BeamDirection)
  (LocalVariables|SetL_CastDistance CastDistance)
  (bind _outhit (Collision|LineTraceByChannel (LocalVariables|GetL_BeamOrigin) (+ (LocalVariables|GetL_BeamOrigin) (* (LocalVariables|GetL_BeamDirection) (LocalVariables|GetL_CastDistance))) "TraceTypeQuery4" false 0 "None" true "(R=1.000000,G=0.000000,B=0.000000,A=1.000000)" "(R=0.000000,G=1.000000,B=0.000000,A=1.000000)" 0.1))
  (Niagara|SpawnSystematLocation "/Game/VFX/Placeholder/NS_LightBeamLoop.NS_LightBeamLoop" (Math|Vector|MakeVector (.x _returnvalue) (.y _returnvalue) (.z _returnvalue)) (Transformation|GetWorldRotation _vfxdistance))
  (Class|BPIBeamHit|Beamon(Message) (.HitActor (Collision|BreakHitResult _outhit)) BeamStrength))