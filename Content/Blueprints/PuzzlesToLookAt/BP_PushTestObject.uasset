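; Test physics cube that reacts to Push and Lift force events, simulating physics from BeginPlay.
; Push applies a velocity-change impulse away from the push origin and spawns a Niagara effect facing that direction.
; Lift, gated by a short downward trace, launches the cube upward with an effect, then hovers it by disabling gravity and zeroing velocity after a delay, restoring gravity later.
; Both events print debug strings.
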(event EventBeginPlay
  (Physics|SetSimulatePhysics (Variables|Default|GetCube) true))

(event Collision|EventActorBeginOverlap
  (params (OtherActor :type Actor%20Object%20Reference)))

(event EventTick
  (params (DeltaSeconds :type Float%20%28single-precision%29)))

(event EventPush
  (params (PushOrigin :type Vector :default "0, 0, 0") (Power :type Float%20%28double-precision%29))
  (bind _cube (Variables|Default|GetCube))
  (bind _returnvalue (Transformation|GetWorldLocation _cube))
  (bind _returnvalue_2 (- _returnvalue PushOrigin))
  (bind _returnvalue_3 (Math|Vector|Normalize _returnvalue_2))
  (bind _returnvalue_4 (* _returnvalue_3 Power))
  ;[1 1 1] Push Force Application
  (Development|PrintString "Push Applied")
  (Physics|SetSimulatePhysics (Variables|Default|GetCube) true)
  (Physics|AddImpulse (Variables|Default|GetCube) _returnvalue_4 "None" true)
  (Niagara|SpawnSystematLocation "/Game/VFX/Placeholder/NS_PushRecieved.NS_PushRecieved" (Transformation|GetWorldLocation (Variables|Default|GetCube)) (Math|Conversions|RotationFromXVector _returnvalue_4)))

(event EventLift
  (params (LiftHeight :type Float%20%28double-precision%29) (LiftOrigin :type Vector :default "0, 0, 0"))
  (bind _cube (Variables|Default|GetCube))
  (bind _cube_2 (Variables|Default|GetCube))
  (bind _cube_3 (Variables|Default|GetCube))
  (bind _returnvalue (Transformation|GetWorldLocation _cube_2))
  (bind _returnvalue_2 (Transformation|GetWorldLocation _cube))
  ;[1 1 1] Lift Force Application
  (Development|PrintString "lift received")
  (bind _returnvalue_3 (Collision|LineTraceByChannel _returnvalue_2 (- _returnvalue_2 "0.000000,0.000000,300.000000") "TraceTypeQuery1" false 0 "None"))
  (if _returnvalue_3
    (Physics|SetSimulatePhysics _cube_3 true)
    (Class|PrimitiveComponent|AddVelocityChangeImpulseatLocation _cube_3 (Math|Vector|MakeVector 0.0 0.0 LiftHeight) _returnvalue "None")
    (Niagara|SpawnSystematLocation "/Game/VFX/Placeholder/NS_LiftRecieved.NS_LiftRecieved" _returnvalue)
    ;[1 1 1] Hovering?
    (Utilities|FlowControl|Delay 1.0)
    (Physics|SetEnableGravity (Variables|Default|GetCube) false)
    (Physics|SetPhysicsLinearVelocity (Variables|Default|GetCube) "0, 0, 0" false "None")
    (Utilities|FlowControl|Delay 5.0)
    (Physics|SetEnableGravity (Variables|Default|GetCube) true)))

(fn ConstructionScript)