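; BP_PushableBlock1 is a puzzle block the main character shoves a fixed distance along a rounded axis direction.
; On a head-on hit, unless locked or the character is floating, a line trace confirms the block is faced and a box trace checks the destination is clear.
; During the MoveBlock timeline the player is attached with movement disabled, then released.
; Puzzle events lock, unlock or reset it to its starting location.
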(event Custom|Push
  (Variables|Default|SetCurrentLocation (Transformation|GetActorLocation))
  (bind _position (Timeline|MoveBlock PlayFromStart)
    (:Update
      (Transformation|SetActorRelativeLocation (+ (* _position (Variables|Default|GetPushableDirection) (Variables|Default|GetTravelDistance)) (Variables|Default|GetCurrentLocation))))
    (:Finished
      (CallFunction|StopPush))))

(event Custom|StopPush
  (Pawn|Components|CharacterMovement|SetMovementMode (Variables|/Script/Engine.Character|GetCharacterMovement (Game|GetPlayerCharacter 0)) "MOVE_Walking" 0)
  (Transformation|DetachFromActor (Game|GetPlayerCharacter 0) "KeepWorld" "KeepWorld" "KeepWorld"))

(event EventPuzzleLock
  (Variables|Default|SetLocked true))

(event Collision|EventHit
  (params (MyComp :type Primitive%20Component%20Object%20Reference) (Other :type Actor%20Object%20Reference) (OtherComp :type Primitive%20Component%20Object%20Reference) (bSelfMoved :type Boolean) (HitLocation :type Vector :default "0, 0, 0") (HitNormal :type Vector :default "0, 0, 0") (NormalImpulse :type Vector :default "0, 0, 0") (Hit :type Hit%20Result%20Structure%20%28by%20ref%29))
  (bind _returnvalue (Transformation|GetActorForwardVector Other))
  (bind (_x _y _z) (Math|Vector|BreakVector _returnvalue))
  ;[1 1 1] Comment
  (bind _asbp_main_character (Utilities|Casting|CastToBP_MainCharacter Other))
  (if (Math|Boolean|ANDBoolean (not (Variables|Default|GetLocked)) (not (Variables|/Game/MainCharacter/FloatFly/BP_FloatMovementComponent.BP_FloatMovementComponent_C|GetIsFloating? (Variables|/Game/MainCharacter/BP_MainCharacter.BP_MainCharacter_C|GetBP_FloatMovementComponent _asbp_main_character))) (> (Math|Vector|DotProduct HitNormal _returnvalue) 0.93))
    (Variables|Default|SetPushableDirection (Math|Vector|MakeVector (Math|Conversions|ToFloat(Integer) (Math|Float|Round _x)) (Math|Conversions|ToFloat(Integer) (Math|Float|Round _y)) (Math|Conversions|ToFloat(Integer) (Math|Float|Round _z))))
    (bind _canbepushed (CallFunction|CanbePushed))
    (if _canbepushed
      (Pawn|Components|CharacterMovement|DisableMovement (Variables|/Script/Engine.Character|GetCharacterMovement (Game|GetPlayerCharacter 0)))
      (Transformation|AttachActorToActor (Game|GetPlayerCharacter 0) self "None" "KeepWorld" "KeepWorld" "KeepWorld" true)
      (CallFunction|Push))))

(event EventBeginPlay
  ;[1 1 1] Spawn Position
  (Variables|Default|SetStartingLocation (Transformation|GetWorldLocation (Variables|Default|GetDefaultSceneRoot))))

(event EventPuzzleReset
  ;[1 0.08115 0] Resets position (NOT USED?)
  (Development|PrintString "P pressed")
  (Transformation|SetWorldLocation (Variables|Default|GetDefaultSceneRoot) (Variables|Default|GetStartingLocation) false false))

(event EventPuzzleUnlock
  (Variables|Default|SetLocked false))

(fn ConstructionScript)

(fn CanbePushed
  (bind _returnvalue (Game|GetPlayerCharacter 0))
  (bind _returnvalue_2 (Transformation|GetActorLocation))
  (bind _returnvalue_3 (Transformation|GetActorLocation _returnvalue))
  (bind (_outhit _returnvalue_4) (Collision|LineTraceByChannel _returnvalue_3 (+ _returnvalue_3 (* (Transformation|GetActorForwardVector _returnvalue) 1e+02)) "TraceTypeQuery1" false (Utilities|Array|MakeArray _returnvalue) "None" false "(R=1.000000,G=0.000000,B=0.000000,A=1.000000)" "(R=0.000000,G=1.000000,B=0.000000,A=1.000000)" 1.0))
  (if _returnvalue_4
    (if (== (.HitActor (Collision|BreakHitResult _outhit)) self)
      (bind (_outhit_2 _returnvalue_5) (Collision|BoxTraceByChannel (+ _returnvalue_2 (Math|Vector|MakeVector 0.0 0.0 1e+02)) (+ (* (Variables|Default|GetPushableDirection) (Variables|Default|GetTravelDistance)) _returnvalue_2 (Math|Vector|MakeVector 0.0 0.0 1e+02)) (* (.boxextent (StaticMesh|GetBounds (Variables|/Script/Engine.StaticMeshComponent|GetStaticMesh (Variables|Default|GetCube)))) (Variables|/Script/Engine.SceneComponent|GetRelativeScale3D (Variables|Default|GetCube)) "0.800000,0.800000,0.800000") "0, 0, 0" "TraceTypeQuery1" false (Utilities|Array|MakeArray self) "ForDuration" true "(R=1.000000,G=0.000000,B=0.000000,A=1.000000)" "(R=0.000000,G=1.000000,B=0.000000,A=1.000000)" 1.0))
      (Development|PrintString (Utilities|GetDisplayName (.HitComponent (Collision|BreakHitResult _outhit_2))))
      (return (not _returnvalue_5))
      (else
        (return false)))))