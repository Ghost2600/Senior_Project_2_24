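; BP_PushTestObject is a physics puzzle block that can be pushed, lifted, highlighted and locked against both forces.
; Tick applies custom gravity along GravityDir; Push applies a velocity impulse away from its origin with a Niagara effect.
; Lift requires a trace hit along gravity, launches the cube against it, then stops it and suspends custom gravity for several seconds over a platform effect.
; Highlight events toggle custom depth rendering.
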(event EventBeginPlay
  (Physics|SetSimulatePhysics (Variables|Default|GetCube) true))

(event EventTick
  (params (DeltaSeconds :type Float%20%28single-precision%29))
  (if (Variables|Default|GetEnableGravity)
    (Physics|AddImpulse (Variables|Default|GetCube) (* (Math|Vector|Normalize (Variables|Default|GetGravityDir)) 9.81 DeltaSeconds) "None" true)))

(event EventLiftHighlighton
  ;[1 1 1] Highlight
  (Rendering|SetRenderCustomDepth (Variables|Default|GetCube) true))

(event EventPushHighlightOff
  ;[1 1 1] Highlight
  (Rendering|SetRenderCustomDepth (Variables|Default|GetCube) false))

(event EventPushHighlighton
  ;[1 1 1] Highlight
  (Rendering|SetRenderCustomDepth (Variables|Default|GetCube) true))

(event EventPush
  (params (PushOrigin :type Vector :default "0, 0, 0") (Power :type Float%20%28double-precision%29))
  (bind _cube (Variables|Default|GetCube))
  (bind _returnvalue (Transformation|GetWorldLocation _cube))
  (bind _returnvalue_2 (- _returnvalue PushOrigin))
  (bind _returnvalue_3 (Math|Vector|Normalize _returnvalue_2))
  (bind _returnvalue_4 (* _returnvalue_3 Power))
  ;[1 1 1] Push Force Application
  (if (not (Variables|Default|GetLocked))
    (Physics|SetSimulatePhysics (Variables|Default|GetCube) true)
    (Physics|AddImpulse (Variables|Default|GetCube) _returnvalue_4 "None" true)
    (Niagara|SpawnSystematLocation "/Game/VFX/Placeholder/NS_PushRecieved.NS_PushRecieved" (Transformation|GetWorldLocation (Variables|Default|GetCube)) (Math|Conversions|RotationFromXVector _returnvalue_4))))

(event EventPuzzleLock
  (Variables|Default|SetLocked true))

(event EventLift
  (params (LiftHeight :type Float%20%28double-precision%29) (LiftOrigin :type Vector :default "0, 0, 0"))
  (bind _cube (Variables|Default|GetCube))
  (bind _cube_2 (Variables|Default|GetCube))
  (bind _cube_3 (Variables|Default|GetCube))
  (bind _returnvalue (Transformation|GetWorldLocation _cube_2))
  (bind _returnvalue_2 (Transformation|GetWorldLocation _cube_3))
  (bind _returnvalue_3 (Transformation|GetWorldScale _cube_3))
  (bind _returnvalue_4 (Transformation|GetWorldLocation _cube))
  ;[1 1 1] Lift Force Application
  (if (not (Variables|Default|GetLocked))
    (bind _returnvalue_5 (Collision|LineTraceByChannel _returnvalue_4 (- _returnvalue_4 (* (Variables|Default|GetGravityDir) -3e+02)) "TraceTypeQuery1" false 0 "None"))
    (if _returnvalue_5
      (Physics|SetSimulatePhysics (Variables|Default|GetCube) true)
      (Class|PrimitiveComponent|AddVelocityChangeImpulseatLocation (Variables|Default|GetCube) (* (Variables|Default|GetGravityDir) LiftHeight -1 1.0) _returnvalue "None")
      (Niagara|SpawnSystematLocation "/Game/VFX/Placeholder/NS_LiftRecieved.NS_LiftRecieved" _returnvalue)
      (Variables|Default|SetEnableGravity false)
      ;[1 1 1] Hovering?
      (Utilities|FlowControl|Delay 0.5)
      (Physics|SetPhysicsLinearVelocity (Variables|Default|GetCube) "0, 0, 0" false "None")
      (Utilities|FlowControl|Delay 0.1)
      (Niagara|SpawnSystematLocation "/Game/FreeNiagaraPack/Effects/NS_LiftForcePlatform.NS_LiftForcePlatform" (Math|Vector|MakeVector (.x _returnvalue_2) (.y _returnvalue_2) (- (.z _returnvalue_2) (/ (.z (* (.z (Class|KismetMathLibrary|GetBoxSize (StaticMesh|GetBoundingBox (Variables|/Script/Engine.StaticMeshComponent|GetStaticMesh _cube_3)))) (.z _returnvalue_3))) 2.0))) (Math|Rotator|MakeRotator 0.0 0.0 (.yaw (Variables|/Script/Engine.SceneComponent|GetRelativeRotation _cube_3))) (Math|Vector|MakeVector (.x _returnvalue_3) (.y _returnvalue_3) (.z _returnvalue_3)))
      (Utilities|FlowControl|Delay 5.0)
      (Variables|Default|SetEnableGravity true))))

(event EventPuzzleUnlock
  (Variables|Default|SetLocked false))

(event EventLiftHighlightOff
  ;[1 1 1] Highlight
  (Rendering|SetRenderCustomDepth (Variables|Default|GetCube) false))

(fn ConstructionScript)