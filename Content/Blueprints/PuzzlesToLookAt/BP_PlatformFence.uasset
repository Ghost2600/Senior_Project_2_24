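; A puzzle platform with a bridge and front and back fence pieces that responds to signal receiver activate and deactivate events.
; Activation applies an energy material, plays a sound and runs a timeline that lerps the pieces' relative Y positions.
; Deactivation applies red energy, plays a sound and reverses the timeline, whose delayed update branch restores default materials.
; BeginPlay stores raised and lowered bridge positions, which the movement leaves unused.
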(event ActivateReceiver(SignalReceiver)
  (Rendering|Material|SetMaterial (Variables|Default|GetBridge) 0 "/Game/Materials/M_Energy.M_Energy")
  (Rendering|Material|SetMaterial (Variables|Default|GetFront) 1 "/Game/Materials/M_Energy.M_Energy")
  (Rendering|Material|SetMaterial (Variables|Default|GetFront) 2 "/Game/Materials/M_Energy.M_Energy")
  (Audio|PlaySoundatLocation 0 "0, 0, 0" "0, 0, 0" 1.0 1.0 0.0 0 0 0 0)
  (bind _platformupward (Timeline|Timeline_1 Play)
    (:Update
      (Utilities|FlowControl|Sequence
        (:then_0
          (Transformation|SetRelativeLocation (Variables|Default|GetBack) (Math|Vector|Lerp(Vector) "0.000000,15227.593165,0.000000" "0.000000,-431.270495,0.000000" _platformupward) false false)
          (Utilities|FlowControl|Delay 1.0)
          (Rendering|Material|SetMaterial (Variables|Default|GetBridge) 0 "/Game/Materials/M_Grey.M_Grey")
          (Rendering|Material|SetMaterial (Variables|Default|GetFront) 1 "/Game/Models/Pipes/blinn1.blinn1")
          (Rendering|Material|SetMaterial (Variables|Default|GetFront) 2 "/Game/CharacterModel/standardSurface1.standardSurface1"))
        (:then_1
          (Transformation|SetRelativeLocation (Variables|Default|GetBridge) (Math|Vector|Lerp(Vector) "0.000000,-15227.593165,0.000000" "0.000000,431.270495,0.000000" _platformupward) false false))))))

(event DeactiveReceiver(SignalReceiver)
  (Rendering|Material|SetMaterial (Variables|Default|GetBridge) 0 "/Game/Materials/M_RedEnergy.M_RedEnergy")
  (Rendering|Material|SetMaterial (Variables|Default|GetFront) 1 "/Game/Materials/M_RedEnergy.M_RedEnergy")
  (Rendering|Material|SetMaterial (Variables|Default|GetFront) 2 "/Game/Materials/M_RedEnergy.M_RedEnergy")
  (Audio|PlaySoundatLocation 0 "0, 0, 0" "0, 0, 0" 1.0 1.0 0.0 0 0 0 0)
  (bind _platformupward (Timeline|Timeline_1 Reverse)
    (:Update
      (Utilities|FlowControl|Sequence
        (:then_0
          (Transformation|SetRelativeLocation (Variables|Default|GetBack) (Math|Vector|Lerp(Vector) "0.000000,15227.593165,0.000000" "0.000000,-431.270495,0.000000" _platformupward) false false)
          (Utilities|FlowControl|Delay 1.0)
          (Rendering|Material|SetMaterial (Variables|Default|GetBridge) 0 "/Game/Materials/M_Grey.M_Grey")
          (Rendering|Material|SetMaterial (Variables|Default|GetFront) 1 "/Game/Models/Pipes/blinn1.blinn1")
          (Rendering|Material|SetMaterial (Variables|Default|GetFront) 2 "/Game/CharacterModel/standardSurface1.standardSurface1"))
        (:then_1
          (Transformation|SetRelativeLocation (Variables|Default|GetBridge) (Math|Vector|Lerp(Vector) "0.000000,-15227.593165,0.000000" "0.000000,431.270495,0.000000" _platformupward) false false))))))

(event EventBeginPlay
  (bind _output_get (Variables|Default|SetDown (Transformation|GetWorldLocation (Variables|Default|GetBridge))))
  (Variables|Default|SetUp (Math|Vector|MakeVector (.x _output_get) (.y _output_get) (+ (.z _output_get) 6e+02))))

(fn ConstructionScript)