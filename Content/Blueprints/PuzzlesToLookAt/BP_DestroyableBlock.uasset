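; BP_DestroyableBlock is a physics-driven puzzle block that loses hit points on collision and explodes when they drop below zero.
; Tick pushes the Cube every frame along the offset from the Arrow to the Cube.
; Hit waits on a short Delay, which absorbs repeat hits, then decrements and prints HitPoints.
; Below zero, it spawns a large explosion emitter, plays a sound and destroys itself.
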(event Collision|EventActorBeginOverlap
  (params (OtherActor :type Actor%20Object%20Reference)))

(event EventBeginPlay
  (Variables|Default|SetHitPoints 3.0))

(event Collision|EventHit
  (params (MyComp :type Primitive%20Component%20Object%20Reference) (Other :type Actor%20Object%20Reference) (OtherComp :type Primitive%20Component%20Object%20Reference) (bSelfMoved :type Boolean) (HitLocation :type Vector :default "0, 0, 0") (HitNormal :type Vector :default "0, 0, 0") (NormalImpulse :type Vector :default "0, 0, 0") (Hit :type Hit%20Result%20Structure%20%28by%20ref%29))
  (bind _returnvalue (Transformation|GetActorLocation))
  (Utilities|FlowControl|Delay 0.5)
  (Variables|Default|SetHitPoints (- (Variables|Default|GetHitPoints) 1.0))
  (Development|PrintText (Utilities|Text|ToText(Float) (Variables|Default|GetHitPoints) "HalfToEven"))
  (if (< (Variables|Default|GetHitPoints) 0.0)
    (Effects|SpawnEmitteratLocation "/Game/StarterContent/Particles/P_Explosion.P_Explosion" _returnvalue "0, 0, 0" "20.000000,20.000000,20.000000")
    (Audio|PlaySoundatLocation "/Game/StarterContent/Audio/Explosion02.Explosion02" _returnvalue "0, 0, 0" 1.0 1.0 0.0 0 0 0 0)
    (Actor|DestroyActor)
    (else
      (Utilities|FlowControl|Delay 1.0))))

(event EventTick
  (params (DeltaSeconds :type Float%20%28single-precision%29))
  (bind _cube (Variables|Default|GetCube))
  (bind _returnvalue (Transformation|GetWorldLocation _cube))
  (Class|PrimitiveComponent|AddVelocityChangeImpulseatLocation (Variables|Default|GetCube) (- _returnvalue (Transformation|GetWorldLocation (Variables|Default|GetArrow))) _returnvalue "None"))

(fn ConstructionScript)