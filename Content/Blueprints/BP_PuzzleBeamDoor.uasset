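; Puzzle door, presumably beam-driven, with top and bottom halves that slide apart vertically when OpenDoor is called.
; OpenDoor plays a 2D sound and a timeline that lerps both halves' relative locations, setting the energy material on each update.
; CloseDoor reverses that same timeline, so the energy material stays applied while closing.
; A second timeline sequence with red energy material is disconnected and never runs.
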(event Custom|OpenDoor
  (params (Player :type Actor%20Object%20Reference))
  (Audio|PlaySound2D 0 1.0 1.0 0.0 0 0)
  (bind _openpuzzledoor (Timeline|Timeline Play)
    (:Update
      (Utilities|FlowControl|Sequence
        (:then_0
          (Transformation|SetRelativeLocation (Variables|Default|GetTopDoor) (Math|Vector|Lerp(Vector) "0.000000,0.000000,0.000000" "0.000000,0.000000,238.519959" _openpuzzledoor) false false)
          (Rendering|Material|SetMaterial (Variables|Default|GetTopDoor) 1 "/Game/Materials/M_Energy.M_Energy"))
        (:then_1
          (Transformation|SetRelativeLocation (Variables|Default|GetBottomDoor) (Math|Vector|Lerp(Vector) "0, 0, 0" "0.000000,0.000000,-267.226659" _openpuzzledoor) false false)
          (Rendering|Material|SetMaterial (Variables|Default|GetBottomDoor) 1 "/Game/Materials/M_Energy.M_Energy"))))))

(event Custom|CloseDoor
  (bind _openpuzzledoor (Timeline|Timeline Reverse)
    (:Update
      (Utilities|FlowControl|Sequence
        (:then_0
          (Transformation|SetRelativeLocation (Variables|Default|GetTopDoor) (Math|Vector|Lerp(Vector) "0.000000,0.000000,0.000000" "0.000000,0.000000,238.519959" _openpuzzledoor) false false)
          (Rendering|Material|SetMaterial (Variables|Default|GetTopDoor) 1 "/Game/Materials/M_Energy.M_Energy"))
        (:then_1
          (Transformation|SetRelativeLocation (Variables|Default|GetBottomDoor) (Math|Vector|Lerp(Vector) "0, 0, 0" "0.000000,0.000000,-267.226659" _openpuzzledoor) false false)
          (Rendering|Material|SetMaterial (Variables|Default|GetBottomDoor) 1 "/Game/Materials/M_Energy.M_Energy"))))))

(fn ConstructionScript)