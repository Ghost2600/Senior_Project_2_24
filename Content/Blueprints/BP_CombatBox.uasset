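; BP_CombatBox is an overlap volume that opens a combat door once no enemies remain inside it.
; Begin and end overlaps with actors tagged Enemy raise and lower EnemyCount, printing the new value each time.
; When an exit drops the count below one, it finds a BP_CombatDoorActual through GetActorOfClass, with no direct reference, and calls OpenCombatDoor on it.
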(event EventBeginPlay)

(event Collision|EventActorBeginOverlap
  (params (OtherActor :type Actor%20Object%20Reference))
  (if (Actor|ActorHasTag OtherActor "Enemy")
    (bind _output_get (Variables|Default|SetEnemyCount (+ (Variables|Default|GetEnemyCount) 1)))
    (Development|PrintString (Utilities|String|ToString(Integer) _output_get))))

(event EventTick
  (params (DeltaSeconds :type Float%20%28single-precision%29)))

(event Collision|EventActorEndOverlap
  (params (OtherActor :type Actor%20Object%20Reference))
  (if (Actor|ActorHasTag OtherActor "Enemy")
    (bind _output_get (Variables|Default|SetEnemyCount (- (Variables|Default|GetEnemyCount) 1)))
    (Development|PrintString (Utilities|String|ToString(Integer) _output_get))
    (if (< (Variables|Default|GetEnemyCount) 1)
      (bind _returnvalue (Actor|GetActorOfClass "/Game/Blueprints/BP_CombatDoor-Actual.BP_CombatDoor-Actual_C"))
      (Default|OpenCombatDoor _returnvalue))))

(fn ConstructionScript)