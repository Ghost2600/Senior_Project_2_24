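; BP_BeamEmitter is an actor that fires a light beam along its arrow component's forward vector every tick.
; Each tick calls ReflectLight, which line-traces on a custom channel over CastDistance and draws a short-lived debug line.
; The hit actor receives a BeamHitMessage carrying the beam strength.
; Despite the function name, it traces a single segment and computes no reflection itself.
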(event EventBeginPlay)

(event Collision|EventActorBeginOverlap
  (params (OtherActor :type Actor%20Object%20Reference)))

(event EventTick
  (params (DeltaSeconds :type Float%20%28single-precision%29))
  (bind _arrow (Variables|Default|GetArrow))
  (if true
    (CallFunction|ReflectLight (Transformation|GetWorldLocation _arrow) (Math|Vector|GetForwardVector _arrow) (Variables|Default|GetCastDistance) 1)))

(fn ConstructionScript)

(fn ReflectLight
  (params (BeamOrigin :type Vector) (BeamDirection :type Vector) (CastDistance :type Float%20%28double-precision%29) (BeamStrength :type Integer))
  (LocalVariables|SetL_BeamOrigin BeamOrigin)
  (LocalVariables|SetL_BeamDirection BeamDirection)
  (LocalVariables|SetL_CastDistance CastDistance)
  (bind _outhit (Collision|LineTraceByChannel (LocalVariables|GetL_BeamOrigin) (+ (LocalVariables|GetL_BeamOrigin) (* (LocalVariables|GetL_BeamDirection) (LocalVariables|GetL_CastDistance))) "TraceTypeQuery4" false 0 "ForDuration" true "(R=1.000000,G=0.000000,B=0.000000,A=1.000000)" "(R=0.000000,G=1.000000,B=0.000000,A=1.000000)" 0.1))
  (Class|BPIBeamHit|BeamHit(Message) (.HitActor (Collision|BreakHitResult _outhit)) (Variables|Default|GetBeamStrength)))