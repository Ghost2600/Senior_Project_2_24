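; Test enemy AI actor that chases the player over a custom NavGraph, with debug drawing and prints throughout.
; Tick follows a smoothed A* path and periodically recomputes it to the player, identically in both states, while Spawn seeds the first path.
; Hits deal damage and briefly stun it, and death drops a health pack.
; Random patrol, player detection and attack-range positioning functions exist but are not wired into live logic.
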(event Custom|Stunned
  (params (Wait%20Time :type Float%20%28double-precision%29))
  (Variables|Default|SetIsStunned true)
  (Development|PrintString "STUNNED" true true "(R=1.000000,G=0.947368,B=0.000000,A=1.000000)" Wait%20Time)
  (Utilities|Time|SetTimerbyEvent (delegate Custom|Unstunned) Wait%20Time))

(event Custom|Unstunned
  (Development|PrintString "UNSTUNNED" true true "(R=1.000000,G=0.295313,B=0.000000,A=1.000000)")
  (Variables|Default|SetIsStunned false))

(event Collision|EventHit
  (params (MyComp :type Primitive%20Component%20Object%20Reference) (Other :type Actor%20Object%20Reference) (OtherComp :type Primitive%20Component%20Object%20Reference) (bSelfMoved :type Boolean) (HitLocation :type Vector :default "0, 0, 0") (HitNormal :type Vector :default "0, 0, 0") (NormalImpulse :type Vector :default "0, 0, 0") (Hit :type Hit%20Result%20Structure%20%28by%20ref%29))
  (Combat|TakeDamage 5.0)
  (Audio|PlaySoundatLocation (Variables|Sounds|GetDamage%20Sound) (Transformation|GetActorLocation) "0, 0, 0" 1.0 1.0 0.0 0 0 0 0))

(event EventBeginPlay)

(event EventTick
  (params (DeltaSeconds :type Float%20%28single-precision%29))
  (bind _state (Variables|Other|GetState))
  (Variables|Default|SetDelta%20Time DeltaSeconds)
  (if (not (Variables|Default|GetIsStunned))
    (Development|PrintString (Utilities|String|EnumtoString _state) true false "(R=0.000000,G=0.660000,B=1.000000,A=1.000000)" 2.0 "AiState")
    (switch Utilities|FlowControl|Switch|SwitchonAIDummy_SM _state
      (:NewEnumerator0
        _)
      (:NewEnumerator3
        _))
    (CallFunction|FollowPath (Variables|Default|GetDelta%20Time))
    (Debug|DebugPatrol)
    (bind _output_get (Variables|Pathfinding|SetPathing%20Timer (+ (Variables|Pathfinding|GetPathing%20Timer) (Variables|Default|GetDelta%20Time))))
    (if (>= _output_get (Variables|Pathfinding|GetUpdate%20Time%20for%20Pathing))
      (Variables|Pathfinding|SetPathing%20Timer 0.0)
      (CallFunction|GetPath (Transformation|GetActorLocation (Game|GetPlayerCharacter 0))))))

(fn ConstructionScript)

(fn Spawn
  (Variables|Other|SetAverageAttackDistance (/ (+ (Variables|Other|GetMaxAttackDistance) (Variables|Other|GetMinAttackDistance)) 2))
  (CallFunction|UpdateLocation (Variables|Pathfinding|GetUpdate%20Time%20for%20Pathing))
  (bind _output_get (Variables|Other|SetMoveTarget (Transformation|GetActorLocation (Game|GetPlayerCharacter 0))))
  (Development|PrintString (Utilities|String|ToString(Integer) (Utilities|Array|Length (Variables|Pathfinding|GetNavGraph))) true true "(R=0.272809,G=0.000000,B=1.000000,A=1.000000)" 5e+01)
  (CallFunction|GetPath _output_get))

(fn TakeDamage
  (params (Damage :type Float%20%28double-precision%29))
  ;[1 1 1] Take Damage
  (bind _output_get (Variables|Stats|SetHealth (- (Variables|Stats|GetHealth) Damage)))
  (CallFunction|Stunned (Variables|Default|GetStun%20Time))
  ;[1 1 1] Kill if HP <= 0
  (if (<= _output_get 0.0)
    (Variables|Stats|SetHealth 0.0)
    (Development|PrintString "Dead")
    (Combat|Kill)
    (else
      (Development|PrintString (Utilities|String|ToString(Float) (Variables|Stats|GetHealth))))))

(fn Kill
  (Combat|DropHealthPack)
  (Actor|DestroyActor))

(fn DropHealthPack
  (Game|SpawnActorfromClass "/Game/Blueprints/BP_Health_Pick_Ups.BP_Health_Pick_Ups_C" (Transformation|GetActorTransform) "Undefined" "MultiplyWithRoot" 0 0))

(fn MovetoPlayer
  (params (Delta%20Time :type Float%20%28double-precision%29) (Debug%20Text :type Boolean))
  ;[1 1 1] Set Local Variables
  (LocalVariables|SetDeltaTime Delta%20Time)
  (LocalVariables|SetPlayerLoc (Transformation|GetActorLocation (Game|GetPlayerCharacter 0)))
  (bind _output_get (LocalVariables|SetCurrentLoc (Transformation|GetActorLocation)))
  ;[1 1 1] Determie if the enemy is in the proper range of the player
  (Development|PrintString (Utilities|String|ToString(Float) (Math|Vector|Distance(Vector) _output_get (LocalVariables|GetPlayerLoc))) Debug%20Text Debug%20Text "(R=0.000000,G=0.660000,B=1.000000,A=1.000000)" 2.0 "Distance")
  (if (not (and (> (Math|Vector|Distance(Vector) _output_get (LocalVariables|GetPlayerLoc)) (Variables|Other|GetMinAttackDistance)) (< (Math|Vector|Distance(Vector) _output_get (LocalVariables|GetPlayerLoc)) (Variables|Other|GetMaxAttackDistance))))
    (Rendering|Debug|DrawDebugLine (LocalVariables|GetPlayerLoc) (+ (* (Math|Vector|Normalize (- (LocalVariables|GetCurrentLoc) (LocalVariables|GetPlayerLoc))) (Variables|Other|GetAverageAttackDistance)) (LocalVariables|GetPlayerLoc)) "(R=0.561992,G=0.000000,B=1.000000,A=1.000000)" 0.0 5.0)
    (Variables|Other|SetMoveTarget (+ (* (Math|Vector|Normalize (- (LocalVariables|GetCurrentLoc) (LocalVariables|GetPlayerLoc))) (Variables|Other|GetAverageAttackDistance)) (LocalVariables|GetPlayerLoc)))
    (Other|Move (LocalVariables|GetDeltaTime) Debug%20Text)))

(fn Patrol
  (params (Delta%20Time :type Float%20%28double-precision%29) (Debug%20Text :type Boolean))
  (bind _returnvalue (Math|Random|RandomFloatinRange -1.0 1.0))
  (bind _returnvalue_2 (Math|Random|RandomFloatinRange -1.0 1.0))
  (bind _returnvalue_3 (Transformation|GetActorLocation))
  (bind _patrol_range (Variables|Patrol|GetPatrol%20Range))
  (bind _returnvalue_4 (Math|Vector|Normalize (Math|Vector|MakeVector _returnvalue_2 _returnvalue 0.0)))
  (bind _returnvalue_5 (Math|Random|RandomFloatinRange 15.0 _patrol_range))
  (bind _returnvalue_6 (* _returnvalue_4 _returnvalue_5))
  (bind _returnvalue_7 (+ _returnvalue_6 _returnvalue_3))
  (bind (_x _y) (Math|Vector|BreakVector _returnvalue_7))
  ;[1 1 1] If the at target, get new target
  (if (< (Math|Vector|Distance(Vector) (Transformation|GetActorLocation) (Variables|Other|GetMoveTarget)) 1e+01)
    ;[1 1 1] Get new Location to move to
    (Variables|Other|SetMoveTarget (Math|Vector|MakeVector _x _y (.Z (Math|Vector|BreakVector (Transformation|GetActorLocation)))))
    (Other|Move Delta%20Time Debug%20Text)
    (else
      (Other|Move Delta%20Time Debug%20Text))))

(fn Move
  (params (Delta%20Time :type Float%20%28double-precision%29) (Debug%20Text :type Boolean))
  (bind _returnvalue (Transformation|GetActorLocation))
  (bind _pathloc (Variables|Pathfinding|GetPathLoc))
  (bind _returnvalue_2 (- _pathloc _returnvalue))
  (bind _returnvalue_3 (Math|Vector|Normalize _returnvalue_2))
  ;[1 1 1] Get Normal Vector in Target Direction
  (LocalVariables|SetDeltaTime Delta%20Time)
  (LocalVariables|SetDebugText Debug%20Text)
  (Development|PrintString (Utilities|String|Append "Move Direction: " (Utilities|String|ToString(Vector) _returnvalue_3)) (LocalVariables|GetDebugText) (LocalVariables|GetDebugText) "(R=1.000000,G=0.000000,B=0.113725,A=1.000000)" 0.0 "Move Direction")
  ;[1 1 1] Move Dummy towards target
  (Development|PrintString (Utilities|String|Append "Target Move Loc: " (Utilities|String|ToString(Vector) (+ (Transformation|GetActorLocation) (* _returnvalue_3 (Variables|Stats|GetSpeed) (LocalVariables|GetDeltaTime))))) (LocalVariables|GetDebugText) (LocalVariables|GetDebugText) "(R=1.000000,G=0.000000,B=0.113725,A=1.000000)" 0.0 "Target Move Loc")
  (Transformation|SetActorLocation (+ (Transformation|GetActorLocation) (* _returnvalue_3 (Variables|Stats|GetSpeed) (LocalVariables|GetDeltaTime))) false false))

(fn DetectPlayer
  (bind _distancefromplayer (Other|DistancefromPlayer))
  (bind _output_get (LocalVariables|SetDistance%20From%20Player _distancefromplayer))
  ;[0.09088 0.8013 1] If player is outside furthest detection range, return false
  (if (< (Variables|Patrol|GetMaxDetect) _output_get)
    (return false)
    (else
      ;[1 1 1] Else If the player is in min dection range, dect them
      (if (< (LocalVariables|GetDistance%20From%20Player) (Variables|Patrol|GetMinDetect))
        (Variables|Other|SetState "NewEnumerator3")
        (return true)
        (else
          ;[1 0.5931 0] Else, cast a ray towards the player
          (bind _outhit (Collision|LineTraceByChannel (Transformation|GetWorldLocation (Variables|Default|GetFacing%20Direction)) (Transformation|GetActorLocation (Game|GetPlayerCharacter 0)) "TraceTypeQuery1" false 0 "ForDuration" true "(R=1.000000,G=0.000000,B=0.000000,A=1.000000)" "(R=0.000000,G=1.000000,B=0.000000,A=1.000000)" 1.0))
          ;[1 0.5931 0] If the ray doesn't hit object and
          (if (and (not (.bBlockingHit (Collision|BreakHitResult _outhit))) (or (<= (- (LocalVariables|GetDistance%20From%20Player) (.Distance (Collision|BreakHitResult _outhit))) 25.0) (== (.Distance (Collision|BreakHitResult _outhit)) 0.0)))
            (Variables|Other|SetState "NewEnumerator3")
            (return (and (not (.bBlockingHit (Collision|BreakHitResult _outhit))) (or (<= (- (LocalVariables|GetDistance%20From%20Player) (.Distance (Collision|BreakHitResult _outhit))) 25.0) (== (.Distance (Collision|BreakHitResult _outhit)) 0.0))))))))))

(fn DistancefromPlayer
  (return (Math|Vector|Distance(Vector) (Transformation|GetActorLocation) (Transformation|GetActorLocation (Game|GetPlayerCharacter 0)))))

(fn DebugPatrol
  (Rendering|Debug|DrawDebugSphere (Transformation|GetActorLocation) (Variables|Patrol|GetMinDetect) 24 "(R=1.000000,G=0.000000,B=0.009844,A=1.000000)" 0.0 1.0)
  (Rendering|Debug|DrawDebugSphere (Transformation|GetActorLocation) (Variables|Patrol|GetMaxDetect) 24 "(R=0.000000,G=1.000000,B=0.317042,A=1.000000)" 0.0 1.0))

(fn DebugMovetoPlayer
  (bind _output_get (LocalVariables|SetPlayerLoc (Transformation|GetActorLocation (Game|GetPlayerCharacter 0))))
  (Rendering|Debug|DrawDebugSphere _output_get (Variables|Other|GetMinAttackDistance) 24 "(R=1.000000,G=0.000000,B=0.009844,A=1.000000)" 0.0 1.0)
  (Rendering|Debug|DrawDebugSphere (LocalVariables|GetPlayerLoc) (Variables|Other|GetAverageAttackDistance) 24 "(R=1.000000,G=0.991669,B=0.000000,A=1.000000)" 0.0 1.0)
  (Rendering|Debug|DrawDebugSphere (LocalVariables|GetPlayerLoc) (Variables|Other|GetMaxAttackDistance) 24 "(R=0.000000,G=1.000000,B=0.031698,A=1.000000)" 0.0 1.0))

(fn UpdateLocation
  (params (DeltaTime :type Float%20%28double-precision%29))
  (bind _output_get (Variables|Pathfinding|SetPathing%20Timer (+ DeltaTime (Variables|Pathfinding|GetPathing%20Timer))))
  (if (>= _output_get (Variables|Pathfinding|GetUpdate%20Time%20for%20Pathing))
    (Variables|Pathfinding|SetPathing%20Timer 0.0)))

(fn GetNextPathTarget
  (bind _travelpath (Variables|Pathfinding|GetTravelPath))
  (bind _returnvalue (Utilities|Array|LastIndex _travelpath))
  (Variables|Pathfinding|SetPathLoc (.Position (Utilities|Struct|BreakAStarNode (Utilities|Array|Get(acopy) _travelpath _returnvalue))))
  (Utilities|Array|RemoveIndex (Variables|Pathfinding|GetTravelPath) _returnvalue))

(fn GetPath
  (params (TargetLoc :type Vector))
  (bind _nodeindex (CallFunction|GetNearestPointtoTarget (Variables|Pathfinding|GetNavGraph) TargetLoc "0, 0, 0"))
  (bind _nodeindex_2 (CallFunction|GetNearestPointtoTarget (Variables|Pathfinding|GetNavGraph) (Transformation|GetActorLocation) "0, 0, 0"))
  (Development|PrintString (Utilities|String|ToString(Integer) _nodeindex_2) true true "(R=0.000000,G=0.660000,B=1.000000,A=1.000000)" 2e+02)
  (bind (_path _iserror) (CallFunction|AStar (Variables|Pathfinding|GetNavGraph) (Utilities|Array|Get(acopy) (Variables|Pathfinding|GetNavGraph) _nodeindex_2) (Utilities|Array|Get(acopy) (Variables|Pathfinding|GetNavGraph) _nodeindex)))
  (LocalVariables|SetPath _path)
  (if _iserror
    (Development|PrintString "ERROR[AIDummy]: Pathfinding Error" true true "(R=1.000000,G=0.051660,B=0.000000,A=1.000000)" 1.2e+02)
    (else
      (Utilities|Array|Insert (LocalVariables|GetPath) (Utilities|Struct|MakeAStarNode -2 0 "()" TargetLoc))
      (Utilities|Array|Add (LocalVariables|GetPath) (Utilities|Struct|MakeAStarNode -3 0 "()" (Transformation|GetActorLocation)))
      (bind _newpath (CallFunction|PathSmoothing (LocalVariables|GetPath)))
      (CallFunction|DebugPath _newpath (Variables|Pathfinding|GetUpdate%20Time%20for%20Pathing) "0, 0, 0")
      (bind _output_get (Variables|Pathfinding|SetTravelPath _newpath))
      (Variables|Pathfinding|SetPathLoc (.Position (Utilities|Struct|BreakAStarNode (Utilities|Array|Get(acopy) _output_get (- (Utilities|Array|Length _newpath) 1)))))
      (Variables|Pathfinding|SetPathIndex (- (Utilities|Array|Length _newpath) 1)))))

(fn FollowPath
  (params (DeltaTime :type Float%20%28double-precision%29))
  (if (not (Variables|Pathfinding|GetdontMove))
    (if (<= (Math|Vector|Distance(Vector) (Variables|Pathfinding|GetPathLoc) (Transformation|GetActorLocation)) 15.0)
      (bind _output_get (Variables|Pathfinding|SetPathIndex (+ (Variables|Pathfinding|GetPathIndex) -1)))
      (if (< _output_get 0)
        (Variables|Pathfinding|SetdontMove true)
        (else
          (Variables|Pathfinding|SetPathLoc (.Position (Utilities|Struct|BreakAStarNode (Utilities|Array|Get(acopy) (Variables|Pathfinding|GetTravelPath) (Variables|Pathfinding|GetPathIndex)))))
          (Other|Move DeltaTime false)))
      (else
        (Other|Move DeltaTime false)))))