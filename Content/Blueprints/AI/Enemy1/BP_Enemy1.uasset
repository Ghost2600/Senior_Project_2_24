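; BP_Enemy1 is an AI enemy that spots the player, fights with hand and foot hitboxes, and can be stunned or killed.
; Sight triggers CombatManager to alert enemies; the alert event sets a blackboard flag and disables sensing.
; Runtime-spawned bone capsules feed CombatBase hits, while the defense component handles incoming damage, health bar and stun.
; On death it drops a health pack, decrements the game mode's enemy count and shows the enemies-to-beat widget.
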(event OnSeePawn(PawnSensing)
  (params (Pawn :type Pawn%20Object%20Reference))
  ;[0.9602 1 0] Spot Player
  (Default|AlertEnemiesEvent (Variables|Default|GetCombatManager)))

(event Death(BP_AIDefenseBase)
  ;[1 0 0.06983] Defense Base
  (CallFunction|DropHealthPack)
  (Actor|DestroyActor)
  (bind _asbp_test_mode (Utilities|Casting|CastToBP_TestMode (Game|GetGameMode)))
  (bind _result (Math|Integer|DecrementInt (Variables|/Game/MainCharacter/BP_TestMode.BP_TestMode_C|GetEnemiesLeft _asbp_test_mode))
    (:%20%20
      (Variables|/Game/MainCharacter/BP_TestMode.BP_TestMode_C|SetEnemiesLeft _asbp_test_mode _result)
      (bind _returnvalue (UserInterface|CreateWidget "/Game/Widget/WB_EnemiesToBeat.WB_EnemiesToBeat_C"))
      (UserInterface|Viewport|AddtoViewport _returnvalue 0))))

(event UpdateHealthUI(BP_AIDefenseBase)
  (params (Current%20Health :type Float%20%28double-precision%29) (Max%20Health :type Float%20%28double-precision%29))
  ;[1 0 0.06983] Defense Base
  (bind _asenemy_health_bar (Utilities|Casting|CastToEnemyHealthBar (UserInterface|GetWidget (Variables|Default|GetHealthBar))))
  (Development|PrintString "Hello")
  (Default|UpdateHealthBarEvent _asenemy_health_bar Current%20Health Max%20Health))

(event Stun(BP_AIDefenseBase)
  ;[1 0 0.06983] Defense Base
  (AI|Components|Blackboard|SetValueasBool (AI|GetBlackboard 0) (Utilities|String|StringToName "IsStunned") true)
  (Development|PrintString "STUNNED" true true "(R=0.971268,G=1.000000,B=0.000000,A=1.000000)"))

(event Custom|Alerted_Event
  ;[0.9602 1 0] Spot Player
  (AI|Components|Blackboard|SetValueasBool (AI|GetBlackboard 0) (Utilities|String|StringToName "hasSeenPlayer") true)
  (Audio|PlaySoundatLocation "/Game/Audio/Placeholders/Cues/SFX_SoundEffects/Enemies/SFX_E_Hurt_Gasp_Cue.SFX_E_Hurt_Gasp_Cue" (Transformation|GetActorLocation) "0, 0, 0" 1.0 1.0 0.0 0 0 0 0)
  (Class|PawnSensingComponent|SetSensingUpdatesEnabled (Variables|Default|GetPawnSensing) false))

(event Custom|PlayerHit_Event
  (params (AttackDamage :type Float%20%28double-precision%29) (Player :type BP%20Main%20Character%20Object%20Reference))
  ;[1 0 0.06983] Defense Base
  (Default|OnHitEvent (Variables|Default|GetBP_AIDefenseBase) AttackDamage Player self))

(event Custom|CombatBase_HitPlayer
  (params (OverlappedComponent :type Primitive%20Component%20Object%20Reference) (OtherActor :type Actor%20Object%20Reference) (OtherComp :type Primitive%20Component%20Object%20Reference) (OtherBodyIndex :type Integer) (bFromSweep :type Boolean) (SweepResult :type Hit%20Result%20Structure%20%28by%20ref%29))
  ;[0.1807 0 1] Combat Base
  ;;[0.08228 0.0137 0.3564] Hit Player
  (Default|HitPlayerEvent (Variables|Default|GetCombatBase) OtherActor))

(event EventBeginPlay
  (bind _combatbase (Variables|Default|GetCombatBase))
  ;[0.1807 0 1] Combat Base
  ;;[0.225 0.03682 1] Add Colliders for parts of the body
  ;;;[1 1 1] Left Hand
  (bind _addedcomponet (CallFunction|AddCollidertoBone "middle_01_l" 1e+01 1e+01))
  (Collision|BindEventtoOnComponentBeginOverlap _addedcomponet (EventDispatchers|CreateEvent :!event Custom|CombatBase_HitPlayer))
  ;;;[1 1 1] Right Hand
  (bind _addedcomponet_2 (CallFunction|AddCollidertoBone "middle_01_r" 1e+01 1e+01))
  (Collision|BindEventtoOnComponentBeginOverlap _addedcomponet_2 (EventDispatchers|CreateEvent :!event Custom|CombatBase_HitPlayer))
  ;;;[1 1 1] Left Foot
  (bind _addedcomponet_3 (CallFunction|AddCollidertoBone "ball_l" 1e+01 1e+01))
  (Collision|BindEventtoOnComponentBeginOverlap _addedcomponet_3 (EventDispatchers|CreateEvent :!event Custom|CombatBase_HitPlayer))
  ;;;[1 1 1] Right Foot
  (bind _addedcomponet_4 (CallFunction|AddCollidertoBone "ball_r" 1e+01 1e+01))
  (Collision|BindEventtoOnComponentBeginOverlap _addedcomponet_4 (EventDispatchers|CreateEvent :!event Custom|CombatBase_HitPlayer))
  (Variables|/Game/Blueprints/AI/Enemy1/CombatBase/CombatBase.CombatBase_C|SetColliders _combatbase (Variables|Default|GetCombatBaseColliders))
  (Default|TurnonColliders _combatbase (Utilities|Struct|MakeToggleBoneColliders false false false false)))

(fn ConstructionScript)

(fn GetNavMesh
  (bind _navmesh (Default|GetNavMesh (Variables|Pathfinding|GetNavMesh)))
  (return _navmesh))

(fn DropHealthPack
  (Game|SpawnActorfromClass "/Game/Blueprints/BP_Health_Pick_Ups.BP_Health_Pick_Ups_C" (Transformation|GetActorTransform) "Undefined" "MultiplyWithRoot" 0 0))

(fn AddCollidertoBone
  (params (BoneName :type Name) (Radius :type Float%20%28double-precision%29) (HalfHeight :type Float%20%28double-precision%29))
  (bind _returnvalue (AddComponent|AddCapsuleComponent false))
  (Transformation|AttachComponentToComponent _returnvalue (Variables|Character|GetMesh) (Utilities|Name|MakeLiteralName BoneName) "SnapToTarget" "SnapToTarget" "KeepRelative" true)
  (Components|Capsule|SetCapsuleSize _returnvalue Radius HalfHeight true)
  (Utilities|Array|Add (Variables|Default|GetCombatBaseColliders) _returnvalue)
  (return _returnvalue))