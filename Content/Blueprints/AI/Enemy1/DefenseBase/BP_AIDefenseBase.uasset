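; Base defense Blueprint for Enemy1 AI that decides whether an incoming hit is blocked or damages the enemy.
; Optional frontal invincibility blocks player attacks within 75 degrees of forward while the last hit type is default.
; Unblocked hits outside the invincibility window apply damage, VFX and sound, then restart invincibility.
; Push or lift hit types set a weak flag on susceptible enemies; the timed combo reset that clears it is disconnected.
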(event Custom|OnHit_Event
  (params (Damage :type Float%20%28double-precision%29) (Player :type BP%20Main%20Character%20Object%20Reference) (Enemy :type Pawn%20Object%20Reference))
  (bind _returnvalue (Transformation|GetActorLocation Enemy))
  (bind _attackedblocked (CallFunction|IsAttackedBlocked Player Enemy))
  (if _attackedblocked
    (Development|PrintString "Attack Blocked" true true "(R=0.000000,G=0.660000,B=1.000000,A=1.000000)" 1e+01)
    (Default|CallAttackedBlocked)
    (else
      (bind _invincible (CallFunction|GetInvincible))
      (if (not _invincible)
        (CallFunction|TakeDamage Damage)
        (Niagara|SpawnSystematLocation "/Game/VFX/Placeholder/NS_EnemyHit.NS_EnemyHit" _returnvalue)
        (Audio|PlaySoundatLocation "/Game/Audio/Placeholders/Cues/SFX_SoundEffects/SFX_AI_Enemies/AI_Combat/SFX_AI_Hurt_PH_Cue.SFX_AI_Hurt_PH_Cue" _returnvalue "0, 0, 0" 1.0 1.0 0.0 0 0 0 0)
        (CallFunction|DebugHealth "Tim")
        (CallFunction|StartInvincible)
        (Variables|Default|SetTimer 0.0)))))

(event EventBeginPlay
  (|CallParentFunction) ; This node is disabled and will not be called.\nDrag off pins to build functionality.
)

(event EventTick
  (params (DeltaSeconds :type Float%20%28single-precision%29))
  (|CallParentFunction DeltaSeconds)
  (if (Variables|Default|GetStopTimer)
    _))

(fn InvinciblefromFront
  (params (Player :type BP%20Main%20Character%20Object%20Reference) (Enemy :type Pawn%20Object%20Reference))
  (bind _angle_deg (CallFunction|AngleBetweenVectors (- (Transformation|GetActorLocation Player) (Transformation|GetActorLocation Enemy)) (Transformation|GetActorForwardVector Enemy)))
  (if (>= _angle_deg 75.0)
    (return false)
    (else
      (return true))))

(fn IsAttackedBlocked
  (params (Player :type BP%20Main%20Character%20Object%20Reference) (Enemy :type Pawn%20Object%20Reference))
  (if (Utilities|Enum|Equal(Enum) (Variables|Weakness|GetLastHitType) "NewEnumerator0")
    (if (Variables|Strengthes|GetisInvincibleFromFront)
      (bind _blocked (CallFunction|InvinciblefromFront Player Enemy))
      (if _blocked
        (return true)
        (else
          _)))
    (return false)))

(fn ResetLastHitType
  (if (and (Utilities|Enum|Equal(Enum) (Variables|Weakness|GetLastHitType) "NewEnumerator1") (Variables|Weakness|GetisWeakToPush))
    (Variables|Weakness|SetIsWeak false)
    (Variables|Weakness|SetLastHitType "NewEnumerator0")
    (elif (and (Utilities|Enum|Equal(Enum) (Variables|Weakness|GetLastHitType) "NewEnumerator2") (Variables|Weakness|GetisWeakToLift))
      (Variables|Weakness|SetIsWeak false)
      (Variables|Weakness|SetLastHitType "NewEnumerator0")
      (else
        (Variables|Weakness|SetLastHitType "NewEnumerator0")))))

(fn SetLastHitType
  (params (LastHitType :type Enum_AI_Base_HitType%20Enum :default "NewEnumerator0"))
  (Variables|Weakness|SetLastHitType LastHitType)
  (if (and (Utilities|Enum|Equal(Enum) (Variables|Weakness|GetLastHitType) "NewEnumerator1") (Variables|Weakness|GetisWeakToPush))
    (Variables|Weakness|SetIsWeak true)
    (elif (and (Utilities|Enum|Equal(Enum) (Variables|Weakness|GetLastHitType) "NewEnumerator2") (Variables|Weakness|GetisWeakToLift))
      (Variables|Weakness|SetIsWeak true))))