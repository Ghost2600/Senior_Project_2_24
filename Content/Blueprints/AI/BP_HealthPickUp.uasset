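; BP_HealthPickUp is a pickup actor that restores a fixed amount of the player's health on contact.
; On BeginPlay it plays a power-up sound and a creature roar cue at its location.
; On overlap with BP_MainCharacter, it checks the PlayerHealth component and, only if health is below max, restores health, plays a coin sound and destroys itself.
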(event EventBeginPlay
  (Audio|PlaySoundatLocation "/Game/Audio/Interface_And_Item_Sounds/WAV/Special_Powerup_02.Special_Powerup_02" (Transformation|GetActorLocation) "0, 0, 0" 1.0 1.0 0.0 0 0 0 0)
  (Audio|PlaySoundatLocation "/Game/Audio/Creatures_-_Roars_007Deat_Cue.Creatures_-_Roars_007Deat_Cue" (Transformation|GetActorLocation) "0, 0, 0" 1.0 1.0 0.0 0 0 0 0))

(event Collision|EventActorBeginOverlap
  (params (OtherActor :type Actor%20Object%20Reference))
  (bind _asbp_main_character (Utilities|Casting|CastToBP_MainCharacter OtherActor))
  (if (not (Default|GetIsMaxHealth (Variables|/Game/MainCharacter/BP_MainCharacter.BP_MainCharacter_C|GetPlayer_Health _asbp_main_character)))
    (Default|RestoreHealth (Variables|/Game/MainCharacter/BP_MainCharacter.BP_MainCharacter_C|GetPlayer_Health _asbp_main_character) 2e+01)
    (Audio|PlaySoundatLocation "/Game/Audio/Interface_And_Item_Sounds/Cues/Coins_12_Cue.Coins_12_Cue" (Transformation|GetActorLocation) "0, 0, 0" 1.0 1.0 0.0 0 0 0 0)
    (Actor|DestroyActor)))

(fn ConstructionScript)