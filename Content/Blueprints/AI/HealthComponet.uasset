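; Health component that tracks an actor's current and maximum health and provides timed invincibility.
; TakeDamage and RestoreHealth reject non-positive amounts, clamp health, and fire dispatchers for UI updates, with damage also firing Stun, or only Death at zero.
; StartInvincible, not called within the component, blocks damage until a countdown in Tick expires.
; DebugHealth prints the health of a named actor on screen.
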(event EventTick
  (params (DeltaSeconds :type Float%20%28single-precision%29))
  (if (Variables|Default|GetInvincible)
    (if (<= (Variables|Default|GetInvincibleCountDown) 0.0)
      (Variables|Default|SetInvincible false)
      (else
        (Variables|Default|SetInvincibleCountDown (- (Variables|Default|GetInvincibleCountDown) DeltaSeconds))))))

(event EventBeginPlay
  (Variables|Default|SetCurrentHealth (Variables|Default|GetMaxHealth)))

(fn RestoreHealth
  (params (HealthToRestore :type Float%20%28double-precision%29))
  (if (<= HealthToRestore 0.0)
    (Development|PrintString "ERROR[RestoreHealth]: Please Use TakeDamage to Remove Health" true true "(R=1.000000,G=0.000000,B=0.034201,A=1.000000)" 5e+02)
    (else
      (bind _output_get (Variables|Default|SetCurrentHealth (Math|Float|Clamp(Float) (+ HealthToRestore (Variables|Default|GetCurrentHealth)) 0.0 (Variables|Default|GetMaxHealth))))
      (Default|CallUpdateHealthUI _output_get (Variables|Default|GetMaxHealth)))))

(fn TakeDamage
  (params (Damage :type Float%20%28double-precision%29))
  (if (<= Damage 0.0)
    (Development|PrintString "ERROR[TakeDamage]: Please Use RestoreHealth to Gain Health" true true "(R=1.000000,G=0.000000,B=0.034201,A=1.000000)" 5e+02)
    (elif (not (Variables|Default|GetInvincible))
      (bind _output_get (Variables|Default|SetCurrentHealth (Math|Float|Clamp(Float) (- (Variables|Default|GetCurrentHealth) Damage) 0.0 (Variables|Default|GetMaxHealth))))
      (if (<= _output_get 0.0)
        (Default|CallDeath)
        (else
          (Default|CallUpdateHealthUI (Variables|Default|GetCurrentHealth) (Variables|Default|GetMaxHealth))
          (Default|CallStun))))))

(fn DebugHealth
  (params (ActorName :type String))
  (Development|PrintString (Utilities|String|Append ActorName "'s HP: " (Utilities|String|ToString(Float) (Variables|Default|GetCurrentHealth)) "/" (Utilities|String|ToString(Float) (Variables|Default|GetMaxHealth))) true true "(R=0.000000,G=1.000000,B=0.038661,A=1.000000)" 4.0))

(fn StartInvincible
  (Variables|Default|SetInvincible true)
  (Variables|Default|SetInvincibleCountDown (Variables|Default|GetInvincibleTime))
  (Development|PrintString "STARTING INVINSIBALE STATE"))

(fn GetInvincible
  (return (Variables|Default|GetInvincible)))