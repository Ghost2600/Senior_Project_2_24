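; Base enemy AI actor that patrols, alerts other enemies through the CombatManager on sight, and fights the player.
; At start it takes gravity from its section NavMesh, flattens patrol points onto that plane and attaches hit capsules to hand and foot bones.
; Defense component events update the health bar, set blackboard hit states and handle death.
; Death drops a health pack, updates the test-mode enemy count and returns combat tokens.
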(event EventTick
  (params (DeltaSeconds :type Float%20%28single-precision%29)))

(event EventBeginPlay
  (bind _currentgravitydirection (Variables|Default|GetCurrentGravityDirection))
  (Utilities|FlowControl|Sequence
    (:then_0
      ;[1 1 1] If NavMesh is not set, kill enemy
      (Utilities|IsValid (Variables|SetUp|GetSectionNavMesh)
        (:Is%20Not%20Valid
          (Development|PrintString "ERROR[BP_AI_Base]: NO NAV MESH ADDED" true true "(R=1.000000,G=0.000000,B=0.033689,A=1.000000)" 3e+01)
          (bind _asbp_main_character (Utilities|Casting|CastToBP_MainCharacter (Game|Player|GetPlayerPawn 0)))
          (CallFunction|PlayerHitEvent (Variables|/Game/Blueprints/AI/HealthComponet.HealthComponet_C|GetMaxHealth (Variables|Default|GetBP_AIDefenseBase)) _asbp_main_character))))
    (:then_1
      (CallFunction|GravityStart))
    (:then_2
      ;[1 1 1] If Patrol Points not set, set point to self
      (if (== (Utilities|Array|Length (Variables|Patrol|GetPatrolPoints)) 0)
        (Utilities|Array|Add (Variables|Patrol|GetPatrolPoints) (Transformation|GetActorLocation)))
      ;[1 1 1] Cast All Points to Enemy Height
      (for (_array_element _array_index) (Variables|Patrol|GetPatrolPoints)
        (Utilities|Array|SetArrayElem (Variables|Patrol|GetPatrolPoints) _array_index (- _array_element (* (/ (Math|Vector|DotProduct _currentgravitydirection (- _array_element (Transformation|GetActorLocation))) (Math|Vector|VectorLength _currentgravitydirection)) _currentgravitydirection)))))
    (:then_3
      (CallFunction|CombatBaseStart))))

(event OnSeePawn(PawnSensing)
  (params (Pawn :type Pawn%20Object%20Reference))
  ;[0.9602 1 0] Spot Player
  (CallFunction|AlertfromThisEnemy))

(event Custom|AlertFromOthers
  ;[0.9602 1 0] Alert Enmey - Set to Combat State
  (AI|Components|Blackboard|SetValueasEnum (AI|GetBlackboard 0) (Utilities|String|StringToName "GeneralState") (Utilities|Enum|LiteralenumEnum_Ai_Base_GeneralStates "NewEnumerator1"))
  (Class|PawnSensingComponent|SetSensingUpdatesEnabled (Variables|Default|GetPawnSensing) false))

(event Custom|AlertFromThisEnemy
  (Default|AlertEnemiesEvent (Variables|CombatManager|GetCombatManager))
  (Audio|PlaySoundatLocation (Variables|SoundList|GetAlert%20Sound) (Transformation|GetActorLocation) "0, 0, 0" 1.0 1.0 0.0 0 0 0 0))

(event Stun(BP_AIDefenseBase)
  ;[1 0 0.07036] Hit
  (AI|Components|Blackboard|SetValueasEnum (AI|GetBlackboard 0) (Utilities|String|StringToName "GeneralState") (Utilities|Enum|LiteralenumEnum_Ai_Base_GeneralStates "NewEnumerator2"))
  (AI|Components|Blackboard|SetValueasEnum (AI|GetBlackboard 0) (Utilities|String|StringToName "HitState") (Utilities|Enum|LiteralenumEnum_AI_Base_HitType "NewEnumerator0")))

(event Death(BP_AIDefenseBase)
  (bind _combatmanager (Variables|CombatManager|GetCombatManager))
  ;[1 0 0.07036] Health Bar
  (Other|DropHealthPack)
  (Actor|DestroyActor)
  (bind _asbp_test_mode (Utilities|Casting|CastToBP_TestMode (Game|GetGameMode)))
  (bind _result (Math|Integer|DecrementInt (Variables|/Game/MainCharacter/BP_TestMode.BP_TestMode_C|GetEnemiesLeft _asbp_test_mode))
    (:%20%20
      (Variables|/Game/MainCharacter/BP_TestMode.BP_TestMode_C|SetEnemiesLeft _asbp_test_mode _result)
      (bind _returnvalue (UserInterface|CreateWidget "/Game/Widget/WB_EnemiesToBeat.WB_EnemiesToBeat_C"))
      (UserInterface|Viewport|AddtoViewport _returnvalue 0)
      (Development|PrintString "Warning[BP_AI_Base - Death] - Needs Reworked to go through Combat Manager " true true "(R=1.000000,G=0.906157,B=0.000000,A=1.000000)" 1e+01)
      (bind _outactors (Actor|GetAllActorsOfClass "BP_AI_Base_C"))
      (Variables|/Game/Blueprints/AI/CombatManager/NewCombatManager.NewCombatManager_C|SetEnemies (Variables|CombatManager|GetCombatManager) _outactors)
      (Default|RegainTokenEvent (Variables|/Game/Blueprints/AI/CombatManager/NewCombatManager.NewCombatManager_C|GetTokenManager _combatmanager) self)
      (Default|RegainToken (Variables|/Game/Blueprints/AI/CombatManager/NewCombatManager.NewCombatManager_C|GetMovementTokenManager _combatmanager) (Variables|CombatManager|GetMovementToken)))))

(event UpdateHealthUI(BP_AIDefenseBase)
  (params (Current%20Health :type Float%20%28double-precision%29) (Max%20Health :type Float%20%28double-precision%29))
  ;[1 0 0.07036] Health Bar
  (bind _asenemy_health_bar (Utilities|Casting|CastToEnemyHealthBar (UserInterface|GetWidget (Variables|Default|GetHealthBar)))
    (:then
      (Default|UpdateHealthBarEvent _asenemy_health_bar Current%20Health Max%20Health))
    (:CastFailed
      (Development|PrintString "ERROR[BP_AI_Base - Update Health UI ]: Failed to Cast to Enemy Health Bar" true true "(R=1.000000,G=0.001384,B=0.000000,A=1.000000)" 3e+01))))

(event Custom|PlayerHit_Event
  (params (AttackDamage :type Float%20%28double-precision%29) (Player :type BP%20Main%20Character%20Object%20Reference))
  ;[1 0 0.07036] Enemy is Hit
  (Default|OnHitEvent (Variables|Default|GetBP_AIDefenseBase) AttackDamage Player self))

(event EventPush
  (params (PushOrigin :type Vector :default "0, 0, 0") (Power :type Float%20%28double-precision%29))
  (Development|PrintString "Push" true true "(R=0.119962,G=0.000000,B=1.000000,A=1.000000)" 1e+01)
  (AI|Components|Blackboard|SetValueasEnum (AI|GetBlackboard 0) (Utilities|String|StringToName "GeneralState") (Utilities|Enum|LiteralenumEnum_Ai_Base_GeneralStates "NewEnumerator2"))
  (AI|Components|Blackboard|SetValueasEnum (AI|GetBlackboard 0) (Utilities|String|StringToName "HitState") (Utilities|Enum|LiteralenumEnum_AI_Base_HitType "NewEnumerator1")))

(event EventLift
  (params (LiftHeight :type Float%20%28double-precision%29) (LiftOrigin :type Vector :default "0, 0, 0"))
  (Development|PrintString "Lift" true true "(R=0.119962,G=0.000000,B=1.000000,A=1.000000)" 1e+01)
  (AI|Components|Blackboard|SetValueasEnum (AI|GetBlackboard 0) (Utilities|String|StringToName "GeneralState") (Utilities|Enum|LiteralenumEnum_Ai_Base_GeneralStates "NewEnumerator2"))
  (AI|Components|Blackboard|SetValueasEnum (AI|GetBlackboard 0) (Utilities|String|StringToName "HitState") (Utilities|Enum|LiteralenumEnum_AI_Base_HitType "NewEnumerator2")))

(event Custom|CombatBaseStart
  ;[0.2232 0.03689 1] Add Colliders for parts of the body
  ;;[1 1 1] Left Hand
  (bind _addedcomponet (CombatBase|AddCollidertoBone "middle_01_l" 1e+01 1e+01))
  (Collision|BindEventtoOnComponentBeginOverlap _addedcomponet (EventDispatchers|CreateEvent :!event Custom|CombatBase_HitPlayer))
  ;;[1 1 1] Right Hand
  (bind _addedcomponet_2 (CombatBase|AddCollidertoBone "middle_01_r" 1e+01 1e+01))
  (Collision|BindEventtoOnComponentBeginOverlap _addedcomponet_2 (EventDispatchers|CreateEvent :!event Custom|CombatBase_HitPlayer))
  ;;[1 1 1] Left Foot
  (bind _addedcomponet_3 (CombatBase|AddCollidertoBone "ball_l" 1e+01 1e+01))
  (Collision|BindEventtoOnComponentBeginOverlap _addedcomponet_3 (EventDispatchers|CreateEvent :!event Custom|CombatBase_HitPlayer))
  ;;[1 1 1] Right Foot
  (bind _addedcomponet_4 (CombatBase|AddCollidertoBone "ball_r" 1e+01 1e+01))
  (Collision|BindEventtoOnComponentBeginOverlap _addedcomponet_4 (EventDispatchers|CreateEvent :!event Custom|CombatBase_HitPlayer))
  (Default|TurnonColliders (Variables|Default|GetCombatBase) (Utilities|Struct|MakeToggleBoneColliders false false false false)))

(event Custom|ReleaseMovementToken
  (Default|RegainToken (Variables|/Game/Blueprints/AI/CombatManager/NewCombatManager.NewCombatManager_C|GetMovementTokenManager (Variables|CombatManager|GetCombatManager)) (Variables|CombatManager|GetMovementToken))
  (Variables|CombatManager|SetMovementToken -1))

(event Custom|CombatBase_HitPlayer
  (params (OverlappedComponent :type Primitive%20Component%20Object%20Reference) (OtherActor :type Actor%20Object%20Reference) (OtherComp :type Primitive%20Component%20Object%20Reference) (OtherBodyIndex :type Integer) (bFromSweep :type Boolean) (SweepResult :type Hit%20Result%20Structure%20%28by%20ref%29))
  ;[0.2232 0.03689 1] Hit Player
  (Default|HitPlayerEvent (Variables|Default|GetCombatBase) OtherActor (Variables|CombatManager|GetCombatManager)))

(event Custom|Gravity%20Start
  (bind _returnvalue (Transformation|GetActorLocation))
  (bind _values (Utilities|Map|Values (.GravityConnections (Utilities|Struct|BreakAStarNode (Utilities|Array|Get(acopy) (Variables|/Game/Blueprints/AI/Pathfind/MyNavMesh.MyNavMesh_C|GetNavMesh (Variables|/Game/Blueprints/AI/Pathfind/SectionNavMesh.SectionNavMesh_C|GetMyNavMesh (Variables|SetUp|GetSectionNavMesh))))))))
  (for _array_element _values
    _)
  (Variables|Default|SetCurrentGravityDirection (Utilities|Array|Get(acopy) _values))
  (CallFunction|RotateinMoveDirection self (Variables|Default|GetCurrentGravityDirection) (+ (Transformation|GetActorForwardVector) _returnvalue) _returnvalue))

(event Custom|UpdateGravity)

(fn ConstructionScript)

(fn CalcPatrolTime
  (bind _patrol_idledelta (Variables|Patrol|GetPatrol_IdleDelta))
  (bind _patrol_idletime (Variables|Patrol|GetPatrol_IdleTime))
  (bind _returnvalue (Math|Random|RandomFloatinRange 0.0 _patrol_idledelta))
  (bind _returnvalue_2 (/ _patrol_idledelta 2.0))
  (bind _returnvalue_3 (- _returnvalue _returnvalue_2))
  (bind _returnvalue_4 (+ _patrol_idletime _returnvalue_3))
  (if (< _returnvalue_4 0.0)
    (return 0.0)
    (else
      (return _returnvalue_4))))

(fn GetGravityDirection
  (return (Variables|/Script/Engine.CharacterMovementComponent|GetGravityDirection (Variables|Character|GetCharacterMovement))))

(fn GetNavMesh
  (bind _navmesh (Default|GetNavMesh (Variables|SetUp|GetSectionNavMesh)))
  (return _navmesh))

(fn DropHealthPack
  (Game|SpawnActorfromClass "/Game/Blueprints/BP_Health_Pick_Ups.BP_Health_Pick_Ups_C" (Transformation|GetActorTransform) "Undefined" "MultiplyWithRoot" 0 0))

(fn AddCollidertoBone
  (params (BoneName :type Name) (Radius :type Float%20%28double-precision%29) (HalfHeight :type Float%20%28double-precision%29))
  (bind _returnvalue (AddComponent|AddCapsuleComponent false))
  (Transformation|AttachComponentToComponent _returnvalue (Variables|Character|GetMesh) (Utilities|Name|MakeLiteralName BoneName) "SnapToTarget" "SnapToTarget" "KeepRelative" true)
  (Components|Capsule|SetCapsuleSize _returnvalue Radius HalfHeight true)
  (Utilities|Array|Add (Variables|/Game/Blueprints/AI/Enemy1/CombatBase/CombatBase.CombatBase_C|GetColliders (Variables|Default|GetCombatBase)) _returnvalue)
  (return _returnvalue))