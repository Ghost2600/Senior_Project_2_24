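; DummySpawner is an actor that keeps one AiDummy enemy alive at its location.
; Each tick it checks whether the spawned enemy is still valid and, if not, spawns a replacement at the spawner's position.
; The new dummy receives the nav graph from the referenced NavMesh before its Spawn routine is called.
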(event EventTick
  (params (DeltaSeconds :type Float%20%28single-precision%29))
  (if (not (Utilities|IsValid (Variables|Default|GetEnemySpawned)))
    (bind _returnvalue (Game|SpawnActorfromClass "/Game/Blueprints/AI/AiDummy.AiDummy_C" (Math|Conversions|ToTransform(Vector) (Transformation|GetActorLocation)) "Undefined" "MultiplyWithRoot" 0 0))
    (bind _output_get (Variables|Default|SetEnemySpawned _returnvalue))
    (bind _asai_dummy (Utilities|Casting|CastToAiDummy _output_get))
    (Variables|/Game/Blueprints/AI/AiDummy.AiDummy_C|SetNavGraph _asai_dummy (Variables|/Game/Blueprints/AI/Pathfind/MyNavMesh.MyNavMesh_C|GetNavMesh (Variables|/Game/Blueprints/AI/Pathfind/worldNavMeshThing.worldNavMeshThing_C|GetMyNavMesh (Variables|Default|GetNavMesh))))
    (Default|Spawn _asai_dummy)))

(fn ConstructionScript)