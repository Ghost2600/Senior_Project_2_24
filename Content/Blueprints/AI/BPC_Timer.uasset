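; BPC_Timer is a timer component in the AI folder that can start on BeginPlay and signals completion when its time limit is reached.
; Tick accumulates delta time while the timer is on, then calls TimerComplete and restarts if Repeatable.
; ResetAndStartTimer zeroes and enables the clock, and Pause disables it.
; A non-repeatable timer stays on at completion, so it signals every tick until paused or reset.
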(event EventBeginPlay
  (if (Variables|Default|GetStartOn)
    (Timer(Public)|ResetandStartTimer)))

(event EventTick
  (params (DeltaSeconds :type Float%20%28single-precision%29))
  (if (Variables|Default|GetIsOn)
    (bind _output_get (Variables|Default|SetTimeOnClock (+ DeltaSeconds (Variables|Default|GetTimeOnClock))))
    (if (>= _output_get (Variables|Default|GetTimeLimit))
      (Default|CallTimerComplete)
      (if (Variables|Default|GetRepeatable)
        (Timer(Public)|ResetandStartTimer)))))

(fn ResetandStartTimer
  (Variables|Default|SetIsOn true)
  (Variables|Default|SetTimeOnClock 0.0))

(fn Pause
  (Variables|Default|SetIsOn false))