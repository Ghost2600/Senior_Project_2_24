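; BPC_Projectile is a projectile Blueprint in the AI folder that supplies movement and hit detection for a projectile actor passed into it.
; Move offsets that actor along Direction by Speed and delta time, sweeping for collisions.
; A blocking hit or initial overlap only prints whether the hit actor carries the Player tag.
; The event graph is empty, so Move relies on an external caller.
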(event EventBeginPlay)

(event EventTick
  (params (DeltaSeconds :type Float%20%28single-precision%29)))

(fn Move
  (params (ProjectileActor :type Actor%20Object%20Reference) (DeltaTime :type Float%20%28double-precision%29))
  (bind _sweephitresult (Transformation|AddActorWorldOffset ProjectileActor (* (Variables|Default|GetDirection) (Variables|Default|GetSpeed) DeltaTime) true))
  (if (or (.bBlockingHit (Collision|BreakHitResult _sweephitresult)) (.bInitialOverlap (Collision|BreakHitResult _sweephitresult)))
    (if (Actor|ActorHasTag (.HitActor (Collision|BreakHitResult _sweephitresult)) "Player")
      (Development|PrintString "Projectile - Hit Player")
      (else
        (Development|PrintString "Projectile - Hit Other")))))