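; Unit conversion helper functions that translate floats and vectors between "UU" units and Unreal units at a factor of 100.
; The float functions multiply to go into Unreal units and divide to go back, and the vector functions apply them to each component, returning separate axis outputs.
; UnrealtoUUVector computes the converted Y but does not return it, so only its X and Z outputs carry converted values.
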(fn UUtoUnrealFloat
  (params (Input :type Float%20%28double-precision%29))
  (return (* Input 1e+02)))

(fn UUtoUnrealVector
  (params (Input :type Vector))
  (bind _output (CallFunction|UUtoUnrealFloat (.x Input)))
  (bind _output_2 (CallFunction|UUtoUnrealFloat (.y Input)))
  (bind _output_3 (CallFunction|UUtoUnrealFloat (.z Input)))
  (return (Math|Vector|MakeVector _output _output_2 _output_3)))

(fn UnrealtoUUFloat
  (params (Input :type Float%20%28double-precision%29))
  (return (/ Input 1e+02)))

(fn UnrealtoUUVector
  (params (Input :type Vector))
  (bind _output (CallFunction|UnrealtoUUFloat (.x Input)))
  (CallFunction|UnrealtoUUFloat (.y Input))
  (bind _output_2 (CallFunction|UnrealtoUUFloat (.z Input)))
  (return (Math|Vector|MakeVector _output 0.0 _output_2)))