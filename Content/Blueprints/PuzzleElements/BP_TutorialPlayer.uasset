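; Tutorial puzzle pressure plate that only responds to the main character standing on it.
; Overlap begin and end on PlayerBox swap the plate material, play a switch sound and run separate timelines that lower or raise the plate.
; Each timeline's update also sets the SignalSender on or off, so the signal follows the animation.
; PuzzleLock makes the plate ignore overlaps until PuzzleUnlock.
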(event OnComponentEndOverlap(PlayerBox)
  (params (OverlappedComponent :type Primitive%20Component%20Object%20Reference) (OtherActor :type Actor%20Object%20Reference) (OtherComp :type Primitive%20Component%20Object%20Reference) (OtherBodyIndex :type Integer))
  ;[1 1 1] Deactivate
  (if (not (Variables|Default|GetLocked))
    (Utilities|FlowControl|Sequence
      (:then_1
        (Utilities|Casting|CastToBP_MainCharacter OtherActor)
        (Rendering|Material|SetMaterial (Variables|Default|GetPlate) 0 "/Game/Materials/M_orange.M_orange")
        (Audio|PlaySoundatLocation "/Game/Audio/Interface_And_Item_Sounds/Cues/Flick_Switch_03_Cue.Flick_Switch_03_Cue" (Transformation|GetActorLocation) "0, 0, 0" 1.0 1.0 0.0 0 0 0 0)
        (bind _pressureplateheight (Timeline|Timeline_0 Play)
          (:Update
            (Transformation|SetRelativeLocation (Variables|Default|GetPlate) (Math|Vector|MakeVector 0.0 0.0 (Math|Float|Lerp 6.0 13.0 _pressureplateheight)) false false)
            (Default|SetSignal (Variables|Default|GetSignalSender) false)))))))

(event OnComponentBeginOverlap(PlayerBox)
  (params (OverlappedComponent :type Primitive%20Component%20Object%20Reference) (OtherActor :type Actor%20Object%20Reference) (OtherComp :type Primitive%20Component%20Object%20Reference) (OtherBodyIndex :type Integer) (bFromSweep :type Boolean) (SweepResult :type Hit%20Result%20Structure%20%28by%20ref%29))
  ;[1 1 1] Activated
  (if (not (Variables|Default|GetLocked))
    (Utilities|FlowControl|Sequence
      (:then_1
        (Utilities|Casting|CastToBP_MainCharacter OtherActor)
        (Rendering|Material|SetMaterial (Variables|Default|GetPlate) 0 "/Game/Materials/M_Green.M_Green")
        (Audio|PlaySoundatLocation "/Game/Audio/Interface_And_Item_Sounds/Cues/Flick_Switch_05_Cue.Flick_Switch_05_Cue" (Transformation|GetActorLocation) "0, 0, 0" 1.0 1.0 0.0 0 0 0 0)
        (bind _pressureplateheight (Timeline|Timeline Play)
          (:Update
            (Transformation|SetRelativeLocation (Variables|Default|GetPlate) (Math|Vector|MakeVector 0.0 0.0 (Math|Float|Lerp 13.0 6.0 _pressureplateheight)) false false)
            (Default|SetSignal (Variables|Default|GetSignalSender) true)))))))

(event EventPuzzleLock
  (Variables|Default|SetLocked true))

(event EventPuzzleUnlock
  (Variables|Default|SetLocked false))

(fn ConstructionScript)