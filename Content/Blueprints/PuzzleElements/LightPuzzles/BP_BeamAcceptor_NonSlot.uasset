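; Light-puzzle beam receptor that converts an incoming beam into a puzzle signal.
; Beam on and off events drive SignalSender, with optional inversion via InverseSignal, and swap the crystal material between blue and red.
; Activation also spawns a Niagara receptor effect.
; ReflectLight can relay a beam by line trace but is not called here, and GetSignal returns AcceptorActivated, which these graphs never set.
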(event EventBeamon
  (params (BeamStrength :type Integer) (SenderActor :type Actor%20Object%20Reference))
  (bind _cube (Variables|Default|GetCube))
  ;[1 1 1] Activate
  (Utilities|FlowControl|Sequence
    (:then_0
      (Default|SetSignal (Variables|Default|GetSignalSender) (not (Variables|Default|GetInverseSignal)))
      (Rendering|Material|SetMaterial (Variables|Default|GetCube) 1 "/Game/DreamscapeSeries/DreamscapeTower/Materials/Crystals/MI_Crystal_Base_Blue.MI_Crystal_Base_Blue"))
    (:then_1
      (Niagara|SpawnSystematLocation "/Game/VFX/Placeholder/NS_ReceptorOn.NS_ReceptorOn" (Transformation|GetWorldLocation _cube) (Transformation|GetWorldRotation _cube)))))

(event EventBeamOff
  (params (SenderActor :type Actor%20Object%20Reference))
  (Default|SetSignal (Variables|Default|GetSignalSender) (Variables|Default|GetInverseSignal))
  (Rendering|Material|SetMaterial (Variables|Default|GetCube) 1 "/Game/DreamscapeSeries/DreamscapeTower/Materials/Crystals/MI_CrystaGroup_02_Red.MI_CrystaGroup_02_Red"))

(fn ConstructionScript)

(fn ReflectLight
  (params (BeamOrigin :type Vector) (BeamDirection :type Vector) (CastDistance :type Float%20%28double-precision%29) (BeamStrength :type Integer))
  (LocalVariables|SetL_BeamOrigin BeamOrigin)
  (LocalVariables|SetL_BeamDirection BeamDirection)
  (LocalVariables|SetL_CastDistance CastDistance)
  (bind _outhit (Collision|LineTraceByChannel (LocalVariables|GetL_BeamOrigin) (+ (LocalVariables|GetL_BeamOrigin) (* (LocalVariables|GetL_BeamDirection) (LocalVariables|GetL_CastDistance))) "TraceTypeQuery1" false 0 "None" true "(R=1.000000,G=0.000000,B=0.000000,A=1.000000)" "(R=0.000000,G=1.000000,B=0.000000,A=1.000000)" 0.1))
  (Class|BPIBeamHit|Beamon(Message) (.HitActor (Collision|BreakHitResult _outhit)) BeamStrength))

(fn GetSignal
  (return (Variables|Default|GetAcceptorActivated)))