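; Tall light-puzzle reflector that relays incoming beams along its arrow and rotates when a nearby player interacts.
; Beam on/off events maintain a sender-to-strength map, choosing the lowest value as BestSender and forwarding it plus one, like a hop count.
; While a sender exists, Tick line-traces, notifies hit actors on change and spawns Niagara beam VFX every frame.
; Box overlap toggles the prompt widget and input; rotating sends beam-off to the current target.
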(event OnComponentBeginOverlap(Box)
  (params (OverlappedComponent :type Primitive%20Component%20Object%20Reference) (OtherActor :type Actor%20Object%20Reference) (OtherComp :type Primitive%20Component%20Object%20Reference) (OtherBodyIndex :type Integer) (bFromSweep :type Boolean) (SweepResult :type Hit%20Result%20Structure%20%28by%20ref%29))
  ;[1 1 1] Widget
  (Rendering|SetVisibility (Variables|Default|GetWidget) true false)
  (Input|EnableInput (Game|GetPlayerController 0)))

(event OnComponentEndOverlap(Box)
  (params (OverlappedComponent :type Primitive%20Component%20Object%20Reference) (OtherActor :type Actor%20Object%20Reference) (OtherComp :type Primitive%20Component%20Object%20Reference) (OtherBodyIndex :type Integer))
  ;[1 1 1] Widget
  (Rendering|SetVisibility (Variables|Default|GetWidget) false false)
  (Input|DisableInput (Game|GetPlayerController 0)))

(event Custom|RotateCube
  ;[1 1 1] Rotate
  (Transformation|AddLocalRotation (Variables|Default|GetDefaultSceneRoot) (Math|Rotator|MakeRotator 0.0 0.0 (Variables|Default|GetRotationAngle)) false false))

(event EventTick
  (params (DeltaSeconds :type Float%20%28single-precision%29))
  (bind _arrow (Variables|Default|GetArrow))
  (if (Utilities|IsValid (Variables|Default|GetBestSender))
    (CallFunction|ReflectLight (Transformation|GetWorldLocation _arrow) (Math|Vector|GetForwardVector _arrow) (Variables|Default|GetCastDistance) (+ (.Value (Utilities|Map|Find (Variables|Default|GetBeamsHiting) (Variables|Default|GetBestSender))) 1))))

(event EventBeamon
  (params (BeamStrength :type Integer) (SenderActor :type Actor%20Object%20Reference))
  (bind _arrow (Variables|Default|GetArrow))
  (bind _bestsender (Variables|Default|GetBestSender))
  (bind _beamshiting (Variables|Default|GetBeamsHiting))
  (bind _value (Utilities|Map|Find _beamshiting _bestsender))
  (bind _returnvalue (+ _value 1))
  (bind _newbestsender (CallFunction|AddNewSender BeamStrength SenderActor))
  (if _newbestsender
    (CallFunction|ReflectLight (Transformation|GetWorldLocation _arrow) (Math|Vector|GetForwardVector _arrow) (Variables|Default|GetCastDistance) _returnvalue)
    (Variables|Default|SetBeamStrength _returnvalue)))

(event EventBeamOff
  (params (SenderActor :type Actor%20Object%20Reference))
  (bind _arrow (Variables|Default|GetArrow))
  (bind _bestsender (Variables|Default|GetBestSender))
  (bind _beamshiting (Variables|Default|GetBeamsHiting))
  (bind _debug (Variables|Default|GetDebug))
  (bind _debug_2 (Variables|Default|GetDebug))
  (bind _debug_3 (Variables|Default|GetDebug))
  (bind _value (Utilities|Map|Find _beamshiting _bestsender))
  (bind _returnvalue (+ _value 1))
  (bind (_turnoff _updaterecevier) (CallFunction|RemoveSender SenderActor))
  (if _turnoff
    (Development|PrintString "Turn Off" _debug_2 _debug_2)
    (bind _actorhit (Variables|Default|GetActorHit)
      (:then
        (Class|BPIBeamHit|BeamOff(Message) _actorhit self)
        (Variables|Default|SetActorHit 0))
      (:else))
    (elif _updaterecevier
      (Development|PrintString "Update" _debug_3 _debug_3)
      (CallFunction|ReflectLight (Transformation|GetWorldLocation _arrow) (Math|Vector|GetForwardVector _arrow) (Variables|Default|GetCastDistance) _returnvalue)
      (Variables|Default|SetBeamStrength _returnvalue)
      (else
        (Development|PrintString "Nothing" _debug _debug)))))

(event EventInteract
  (params (Character :type BP%20Main%20Character%20Object%20Reference))
  ;[1 1 1] Interact
  (Utilities|Casting|CastToBP_MainCharacter Character)
  (CallFunction|RotateCube)
  (Audio|PlaySoundatLocation "/Game/Audio/Placeholders/Cues/SFX_SoundEffects/SFX_AI_Enemies/AI_Movement/SFX_AI_Idle_Head_PH_Cue.SFX_AI_Idle_Head_PH_Cue" "0, 0, 0" "0, 0, 0" 1.0 1.0 0.0 0 0 0 0)
  (bind _actorhit (Variables|Default|GetActorHit)
    (:then
      (Class|BPIBeamHit|BeamOff(Message) _actorhit self))
    (:else)))

(fn ConstructionScript)

(fn ReflectLight
  (params (BeamOrigin :type Vector) (BeamDirection :type Vector) (CastDistance :type Float%20%28double-precision%29) (BeamStrength :type Integer))
  (bind _vfxdistance (Variables|Default|GetVFXDistance))
  (bind _returnvalue (Transformation|GetWorldLocation _vfxdistance))
  (LocalVariables|SetL_BeamOrigin BeamOrigin)
  (LocalVariables|SetL_BeamDirection BeamDirection)
  (LocalVariables|SetL_CastDistance CastDistance)
  (bind _outhit (Collision|LineTraceByChannel (LocalVariables|GetL_BeamOrigin) (+ (LocalVariables|GetL_BeamOrigin) (* (LocalVariables|GetL_BeamDirection) (LocalVariables|GetL_CastDistance))) "TraceTypeQuery4" false 0 "None" true "(R=1.000000,G=0.000000,B=0.000000,A=1.000000)" "(R=0.000000,G=1.000000,B=0.000000,A=1.000000)" 0.1))
  (Niagara|SpawnSystematLocation "/Game/VFX/Placeholder/NS_LightBeamLoop.NS_LightBeamLoop" (Math|Vector|MakeVector (.x _returnvalue) (.y _returnvalue) (.z _returnvalue)) (Transformation|GetWorldRotation _vfxdistance))
  (if (!= (Variables|Default|GetActorHit) (.HitActor (Collision|BreakHitResult _outhit)))
    (bind _actorhit (Variables|Default|GetActorHit)
      (:then
        (Class|BPIBeamHit|BeamOff(Message) _actorhit self))
      (:else
        _))
    (Variables|Default|SetActorHit (.HitActor (Collision|BreakHitResult _outhit)))
    (Class|BPIBeamHit|Beamon(Message) (Variables|Default|GetActorHit) BeamStrength self)))

(fn AddNewSender
  (params (SenderStrength :type Integer) (NewSender :type Actor%20Object%20Reference))
  (bind _debug (Variables|Default|GetDebug))
  ;[1 1 1] If new, add to list
  (if (and (not (Utilities|IsValid NewSender)) (.ReturnValue (Utilities|Map|Find (Variables|Default|GetBeamsHiting) NewSender)))
    (Development|PrintString "Sender Already in List or Null" _debug _debug)
    (return false)
    (else
      (Utilities|Map|Add (Variables|Default|GetBeamsHiting) NewSender SenderStrength)
      ;[1 1 1] Update Best sender if stength is lower
      (if (or (not (Utilities|IsValid (Variables|Default|GetBestSender))) (< SenderStrength (.Value (Utilities|Map|Find (Variables|Default|GetBeamsHiting) (Variables|Default|GetBestSender)))))
        (Variables|Default|SetBestSender NewSender)
        (return true)
        (else
          (return false))))))

(fn RemoveSender
  (params (OldSender :type Actor%20Object%20Reference))
  (bind _debug (Variables|Default|GetDebug))
  ;[1 1 1] Remove Sender if in List
  (bind _returnvalue (Utilities|Map|Remove (Variables|Default|GetBeamsHiting) OldSender))
  (if _returnvalue
    (if (== (Utilities|Map|Length (Variables|Default|GetBeamsHiting)) 0)
      (Variables|Default|SetBestSender 0)
      (return true true)
      (elif (== (Variables|Default|GetBestSender) OldSender)
        (if (== (Utilities|Map|Length (Variables|Default|GetBeamsHiting)) 1)
          (bind _keys (Utilities|Map|Keys (Variables|Default|GetBeamsHiting)))
          (Variables|Default|SetBestSender (Utilities|Array|Get(acopy) _keys))
          (return false true)
          (else
            (bind _keys_2 (Utilities|Map|Keys (Variables|Default|GetBeamsHiting)))
            (LocalVariables|SetNewBest (Utilities|Array|Get(acopy) _keys_2))
            (bind _values (Utilities|Map|Values (Variables|Default|GetBeamsHiting)))
            (LocalVariables|SetNewValue (Utilities|Array|Get(acopy) _values))
            (for (_array_element _array_index) _values
              (if (< _array_element (LocalVariables|GetNewValue))
                (LocalVariables|SetNewValue _array_element)
                (bind _keys_3 (Utilities|Map|Keys (Variables|Default|GetBeamsHiting)))
                (LocalVariables|SetNewBest (Utilities|Array|Get(acopy) _keys_3 _array_index))))
            (Variables|Default|SetBestSender (LocalVariables|GetNewBest))
            (return false true)))
        (else
          (return false false))))
    (else
      (Development|PrintString "Sender Not Found" _debug _debug)
      (return false false))))