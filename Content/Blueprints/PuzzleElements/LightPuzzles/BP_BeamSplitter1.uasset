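; Light puzzle beam splitter that turns an incoming beam into two outgoing beams at configurable angles.
; It tracks all senders in a map, picks the lowest strength as best and passes that value plus one onward.
; A repeating timer re-runs both line traces, sending on/off messages as hit actors change, while Tick spawns beam Niagara effects.
; OLDReflectLight and the signal-activation branch are unused leftovers.
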(event TimerComplete(BPC_Timer)
  (bind _arrow1 (Variables|Default|GetArrow1))
  (bind _arrow (Variables|Default|GetArrow))
  (if (Utilities|IsValid (Variables|Default|GetBestSender))
    (CallFunction|ReflectLight (Transformation|GetWorldLocation _arrow) (Math|Vector|GetForwardVector _arrow) (Variables|Default|GetCastDistance) (+ (.Value (Utilities|Map|Find (Variables|Default|GetBeamsHiting) (Variables|Default|GetBestSender))) 1) (Variables|Default|GetDirector))
    (CallFunction|ReflectLight (Transformation|GetWorldLocation _arrow1) (Math|Vector|GetForwardVector _arrow1) (Variables|Default|GetCastDistance) (+ (.Value (Utilities|Map|Find (Variables|Default|GetBeamsHiting) (Variables|Default|GetBestSender))) 1) (Variables|Default|GetDirector1))
    (Default|ResetandStartTimer (Variables|Default|GetBPC_Timer))))

(event EventTick
  (params (DeltaSeconds :type Float%20%28single-precision%29))
  (bind _director (Variables|Default|GetDirector))
  (bind _director1 (Variables|Default|GetDirector1))
  (bind _returnvalue (Transformation|GetWorldLocation _director))
  (bind _returnvalue_2 (Transformation|GetWorldLocation _director1))
  (if (Utilities|IsValid (Variables|Default|GetBestSender))
    (Niagara|SpawnSystematLocation "/Game/VFX/Placeholder/NS_LightBeamLoop.NS_LightBeamLoop" (Math|Vector|MakeVector (.x _returnvalue) (.y _returnvalue) (.z _returnvalue)) (Transformation|GetWorldRotation _director))
    (Niagara|SpawnSystematLocation "/Game/VFX/Placeholder/NS_BeamCast.NS_BeamCast" (Transformation|GetWorldLocation (Variables|Default|GetSphere)) (Transformation|GetWorldRotation (Variables|Default|GetDirector)))
    (Niagara|SpawnSystematLocation "/Game/VFX/Placeholder/NS_LightBeamLoop.NS_LightBeamLoop" (Math|Vector|MakeVector (.x _returnvalue_2) (.y _returnvalue_2) (.z _returnvalue_2)) (Transformation|GetWorldRotation _director1))
    (Niagara|SpawnSystematLocation "/Game/VFX/Placeholder/NS_BeamCast.NS_BeamCast" (Transformation|GetWorldLocation (Variables|Default|GetSphere)) (Transformation|GetWorldRotation (Variables|Default|GetDirector1)))))

(event EventBeamon
  (params (BeamStrength :type Integer) (SenderActor :type Actor%20Object%20Reference))
  (bind _arrow (Variables|Default|GetArrow))
  (bind _bestsender (Variables|Default|GetBestSender))
  (bind _beamshiting (Variables|Default|GetBeamsHiting))
  (bind _arrow1 (Variables|Default|GetArrow1))
  (bind _value (Utilities|Map|Find _beamshiting _bestsender))
  (bind _returnvalue (+ _value 1))
  (bind _newbestsender (CallFunction|AddNewSender BeamStrength SenderActor))
  (if _newbestsender
    (Default|ResetandStartTimer (Variables|Default|GetBPC_Timer))
    (Transformation|SetRelativeRotation (Variables|Default|GetDirector) (Math|Rotator|MakeRotator (Variables|Default|GetBeamOneXRot) 0.0 (Variables|Default|GetBeamOneZRot)) false false)
    (Transformation|SetRelativeRotation (Variables|Default|GetDirector1) (Math|Rotator|MakeRotator (Variables|Default|GetBeamTwoXRot) 0.0 (Variables|Default|GetBeamTwoZRot)) false false)
    (CallFunction|ReflectLight (Transformation|GetWorldLocation _arrow) (Math|Vector|GetForwardVector _arrow) (Variables|Default|GetCastDistance) _returnvalue (Variables|Default|GetDirector))
    (CallFunction|ReflectLight (Transformation|GetWorldLocation _arrow1) (Math|Vector|GetForwardVector _arrow1) (Variables|Default|GetCastDistance) _returnvalue (Variables|Default|GetDirector1))
    (Variables|Default|SetBeamStrength _returnvalue)))

(event EventBeamOff
  (params (SenderActor :type Actor%20Object%20Reference))
  (bind _arrow (Variables|Default|GetArrow))
  (bind _bestsender (Variables|Default|GetBestSender))
  (bind _beamshiting (Variables|Default|GetBeamsHiting))
  (bind _debug (Variables|Default|GetDebug))
  (bind _debug_2 (Variables|Default|GetDebug))
  (bind _debug_3 (Variables|Default|GetDebug))
  (bind _arrow1 (Variables|Default|GetArrow1))
  (bind _value (Utilities|Map|Find _beamshiting _bestsender))
  (bind _returnvalue (+ _value 1))
  (bind (_turnoff _updaterecevier) (CallFunction|RemoveSender SenderActor))
  (if _turnoff
    (Development|PrintString "Turn Off" _debug_2 _debug_2)
    (bind _actorhit (Variables|Default|GetActorHit)
      (:then
        (Class|BPIBeamHit|BeamOff(Message) _actorhit self)
        (Variables|Default|SetActorHit 0))
      (:else
        _))
    (bind _actorhit2 (Variables|Default|GetActorHit2)
      (:then
        (Class|BPIBeamHit|BeamOff(Message) _actorhit2 self)
        (Variables|Default|SetActorHit2 0))
      (:else
        _))
    (Default|Pause (Variables|Default|GetBPC_Timer))
    (elif _updaterecevier
      (Development|PrintString "Update" _debug_3 _debug_3)
      (Default|ResetandStartTimer (Variables|Default|GetBPC_Timer))
      (CallFunction|ReflectLight (Transformation|GetWorldLocation _arrow) (Math|Vector|GetForwardVector _arrow) (Variables|Default|GetCastDistance) _returnvalue (Variables|Default|GetDirector))
      (CallFunction|ReflectLight (Transformation|GetWorldLocation _arrow1) (Math|Vector|GetForwardVector _arrow1) (Variables|Default|GetCastDistance) _returnvalue (Variables|Default|GetDirector1))
      (Variables|Default|SetBeamStrength _returnvalue)
      (else
        (Development|PrintString "Nothing" _debug _debug)))))

(event EventBeamHit
  (params (BeamStrength :type Integer)))

(fn ConstructionScript)

(fn OLDReflectLight
  (params (BeamOrigin :type Vector) (BeamDirection :type Vector) (CastDistance :type Float%20%28double-precision%29) (BeamStrength :type Integer))
  (bind _director (Variables|Default|GetDirector))
  (bind _returnvalue (Transformation|GetWorldLocation _director))
  (bind _returnvalue_2 (Transformation|GetWorldRotation _director))
  (LocalVariables|SetL_BeamOrigin BeamOrigin)
  (LocalVariables|SetL_BeamDirection BeamDirection)
  (LocalVariables|SetL_CastDistance CastDistance)
  (bind _outhit (Collision|LineTraceByChannel (LocalVariables|GetL_BeamOrigin) (+ (LocalVariables|GetL_BeamOrigin) (* (LocalVariables|GetL_BeamDirection) (LocalVariables|GetL_CastDistance))) "TraceTypeQuery4" false 0 "ForDuration" true "(R=1.000000,G=0.000000,B=0.000000,A=1.000000)" "(R=0.000000,G=1.000000,B=0.000000,A=1.000000)" 0.1))
  (Niagara|SpawnSystematLocation "/Game/VFX/Placeholder/NS_LightBeamLoop.NS_LightBeamLoop" (Math|Vector|MakeVector (.x _returnvalue) (.y _returnvalue) (.z _returnvalue)) _returnvalue_2)
  (Niagara|SpawnSystematLocation "/Game/VFX/Placeholder/NS_BeamCast.NS_BeamCast" (Transformation|GetWorldLocation (Variables|Default|GetSphere)) _returnvalue_2)
  (Class|BPIBeamHit|Beamon(Message) (.HitActor (Collision|BreakHitResult _outhit)) BeamStrength)
  (if (.bBlockingHit (Collision|BreakHitResult _outhit))
    (Niagara|SpawnSystematLocation "/Game/VFX/Placeholder/NS_BeamHit.NS_BeamHit" (.ImpactPoint (Collision|BreakHitResult _outhit)) (* (LocalVariables|GetL_BeamDirection) -1.0))))

(fn ReflectLight
  (params (BeamOrigin :type Vector) (BeamDirection :type Vector) (CastDistance :type Float%20%28double-precision%29) (BeamStrength :type Integer) (DirectorToUse :type Static%20Mesh%20Component%20Object%20Reference))
  (LocalVariables|SetL_BeamOrigin BeamOrigin)
  (LocalVariables|SetL_BeamDirection BeamDirection)
  (LocalVariables|SetL_CastDistance CastDistance)
  (bind _outhit (Collision|LineTraceByChannel (LocalVariables|GetL_BeamOrigin) (+ (LocalVariables|GetL_BeamOrigin) (* (LocalVariables|GetL_BeamDirection) (LocalVariables|GetL_CastDistance))) "TraceTypeQuery4" false 0 "None" true "(R=1.000000,G=0.000000,B=0.000000,A=1.000000)" "(R=0.000000,G=1.000000,B=0.000000,A=1.000000)" 0.1))
  (if (and (== DirectorToUse (Variables|Default|GetDirector)) (!= (Variables|Default|GetActorHit) (.HitActor (Collision|BreakHitResult _outhit))))
    (bind _actorhit (Variables|Default|GetActorHit)
      (:then
        (Class|BPIBeamHit|BeamOff(Message) _actorhit self))
      (:else
        _))
    (Variables|Default|SetActorHit (.HitActor (Collision|BreakHitResult _outhit)))
    (Class|BPIBeamHit|Beamon(Message) (Variables|Default|GetActorHit) BeamStrength self))
  (if (and (== DirectorToUse (Variables|Default|GetDirector1)) (!= (Variables|Default|GetActorHit2) (.HitActor (Collision|BreakHitResult _outhit))))
    (bind _actorhit2 (Variables|Default|GetActorHit2)
      (:then
        (Class|BPIBeamHit|BeamOff(Message) _actorhit2 self))
      (:else
        _))
    (Variables|Default|SetActorHit2 (.HitActor (Collision|BreakHitResult _outhit)))
    (Class|BPIBeamHit|Beamon(Message) (Variables|Default|GetActorHit2) BeamStrength self))
  (if (.bBlockingHit (Collision|BreakHitResult _outhit))
    (Niagara|SpawnSystematLocation "/Game/VFX/Placeholder/NS_BeamHit.NS_BeamHit" (.ImpactPoint (Collision|BreakHitResult _outhit)) (* (LocalVariables|GetL_BeamDirection) -1.0))))

(fn AddNewSender
  (params (SenderStrength :type Integer) (NewSender :type Actor%20Object%20Reference))
  (bind _debug (Variables|Default|GetDebug))
  ;[1 1 1] If new, add to list
  (if (and (not (Utilities|IsValid NewSender)) (.ReturnValue (Utilities|Map|Find (Variables|Default|GetBeamsHiting) NewSender)))
    (Development|PrintString "Sender Already in List or Null" _debug _debug)
    (return false)
    (else
      (Utilities|Map|Add (Variables|Default|GetBeamsHiting) NewSender SenderStrength)
      ;[1 1 1] Update Best sender if stength is lower
      (if (or (not (Utilities|IsValid (Variables|Default|GetBestSender))) (< SenderStrength (.Value (Utilities|Map|Find (Variables|Default|GetBeamsHiting) (Variables|Default|GetBestSender)))))
        (Variables|Default|SetBestSender NewSender)
        (return true)
        (else
          (return false))))))

(fn RemoveSender
  (params (OldSender :type Actor%20Object%20Reference))
  (bind _debug (Variables|Default|GetDebug))
  ;[1 1 1] Remove Sender if in List
  (bind _returnvalue (Utilities|Map|Remove (Variables|Default|GetBeamsHiting) OldSender))
  (if _returnvalue
    (if (== (Utilities|Map|Length (Variables|Default|GetBeamsHiting)) 0)
      (Variables|Default|SetBestSender 0)
      (return true true)
      (elif (== (Variables|Default|GetBestSender) OldSender)
        (if (== (Utilities|Map|Length (Variables|Default|GetBeamsHiting)) 1)
          (bind _keys (Utilities|Map|Keys (Variables|Default|GetBeamsHiting)))
          (Variables|Default|SetBestSender (Utilities|Array|Get(acopy) _keys))
          (return false true)
          (else
            (bind _keys_2 (Utilities|Map|Keys (Variables|Default|GetBeamsHiting)))
            (LocalVariables|SetNewBest (Utilities|Array|Get(acopy) _keys_2))
            (bind _values (Utilities|Map|Values (Variables|Default|GetBeamsHiting)))
            (LocalVariables|SetNewValue (Utilities|Array|Get(acopy) _values))
            (for (_array_element _array_index) _values
              (if (< _array_element (LocalVariables|GetNewValue))
                (LocalVariables|SetNewValue _array_element)
                (bind _keys_3 (Utilities|Map|Keys (Variables|Default|GetBeamsHiting)))
                (LocalVariables|SetNewBest (Utilities|Array|Get(acopy) _keys_3 _array_index))))
            (Variables|Default|SetBestSender (LocalVariables|GetNewBest))
            (return false true)))
        (else
          (return false false))))
    (else
      (Development|PrintString "Sender Not Found" _debug _debug)
      (return false false))))