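; BPC_SignalReceiver is a puzzle component that turns on only when every linked signal actor is sending a signal.
; On BeginPlay it binds to the BPC_SignalSender on each actor in SignalActors.
; Each update ANDs all sender signals and fires the activate or deactivate call only when the combined state changes.
; The current state is exposed through IsActivated.
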(event Custom|DetermineDoorStatus
  (Variables|Default|SetTempActivated true)
  (for _array_element (Variables|Default|GetSignalActors)
    (Variables|Default|SetTempActivated (and (Default|GetSignal (Actor|GetComponentbyClass _array_element "/Game/Blueprints/PuzzleElements/Signals/BPC_SignalSender.BPC_SignalSender_C")) (Variables|Default|GetTempActivated))))
  (if (and (Variables|Default|GetActivated) (not (Variables|Default|GetTempActivated)))
    (Default|CallDeactiveReceiver)
    (Variables|Default|SetActivated (Variables|Default|GetTempActivated) :!label _label)
    (elif (and (not (Variables|Default|GetActivated)) (Variables|Default|GetTempActivated))
      (Default|CallActivateReceiver)
      (goto _label))))

(event EventBeginPlay
  (for _array_element (Variables|Default|GetSignalActors)
    (EventDispatchers|BindEventtoUpdatedSignal (Actor|GetComponentbyClass _array_element "/Game/Blueprints/PuzzleElements/Signals/BPC_SignalSender.BPC_SignalSender_C") (delegate Custom|DetermineDoorStatus))))

(fn IsActivated
  (return (Variables|Default|GetActivated)))