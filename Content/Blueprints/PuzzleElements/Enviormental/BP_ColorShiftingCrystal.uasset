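; BP_ColorShiftingCrystal is an environmental puzzle element that changes its crystal material and light color in response to a SignalReceiver.
; It begins with the blue fade material.
; Activation stops Timeline_0, then plays the ON timeline, whose updates apply the energy material and play a timeline driving PointLight color.
; Deactivation uses the same nested-timeline pattern to restore blue fade and drive the color through a separate track.
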(event ActivateReceiver(SignalReceiver)
  (Utilities|FlowControl|Sequence
    (:then_0
      (bind _newtrack_0 (Timeline|Timeline_0 Stop)
        (:Update
          (Rendering|Components|Light|SetLightColor (Variables|Default|GetPointLight) _newtrack_0 true))))
    (:then_1
      (Timeline|ON Play
        (:Update
          (Rendering|Material|SetMaterial (Variables|Default|GetCrystalLight) 0 "/Game/Materials/M_Energy.M_Energy")
          (bind _newtrack_0_2 (Timeline|Timeline_1 Play)
            (:Update
              (Rendering|Components|Light|SetLightColor (Variables|Default|GetPointLight) _newtrack_0_2 true))))))))

(event DeactiveReceiver(SignalReceiver)
  (Timeline|Timeline Play
    (:Update
      (Rendering|Material|SetMaterial (Variables|Default|GetCrystalLight) 0 "/Game/Materials/M_BlueFade.M_BlueFade")
      (bind _newtrack_0 (Timeline|Timeline_2 Play)
        (:Update
          (Rendering|Components|Light|SetLightColor (Variables|Default|GetPointLight) _newtrack_0 true))))))

(event EventBeginPlay
  (Rendering|Material|SetMaterial (Variables|Default|GetCrystalLight) 0 "/Game/Materials/M_BlueFade.M_BlueFade"))

(fn ConstructionScript)