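; Puzzle platform that moves at constant speed through a list of path points, with its spawn location inserted as the first.
; Tick runs the selected move type while On: Simple stops at the last point, Complex ping-pongs, Circular loops back to the start.
; BPC_SignalReceiver events switch movement on or off according to the Togglable mode, which also sets the starting state.
; An empty path disables it with a debug warning.
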(event ActivateReceiver(BPC_SignalReceiver)
  (switch Utilities|FlowControl|Switch|SwitchonEnum_MoveablePlatform_Togglable (Variables|SetUp|GetTogglable)
    (:NewEnumerator2
      (Variables|Default|SetOn true :!label _label))
    (:NewEnumerator0
      (Variables|Default|SetOn false))
    (:NewEnumerator1
      (goto _label))))

(event DeactiveReceiver(BPC_SignalReceiver)
  (switch Utilities|FlowControl|Switch|SwitchonEnum_MoveablePlatform_Togglable (Variables|SetUp|GetTogglable)
    (:NewEnumerator2
      (Variables|Default|SetOn true :!label _label))
    (:NewEnumerator0
      (goto _label))
    (:NewEnumerator1
      (Variables|Default|SetOn false))))

(event EventBeginPlay
  (bind _debug (Variables|Default|GetDebug))
  (if (== (Utilities|Array|Length (Variables|SetUp|GetPath)) 0)
    (Development|PrintString "Warning[BP_MoveablePlatform]: Path empty. Path needs at least 1 point to be considered an end point." _debug _debug "(R=1.000000,G=0.577228,B=0.000000,A=1.000000)" 2e+01)
    (Variables|Default|SetOn false)
    (else
      ;[1 1 1] Insert Start Point
      (Utilities|Array|Insert (Variables|SetUp|GetPath) (Transformation|GetActorLocation))
      (TargetPoint|GetNextPoint)
      (switch Utilities|FlowControl|Switch|SwitchonEnum_MoveablePlatform_Togglable (Variables|SetUp|GetTogglable)
        (:NewEnumerator2
          (Variables|Default|SetOn true :!label _label))
        (:NewEnumerator0
          (goto _label))
        (:NewEnumerator1
          (Variables|Default|SetOn false))))))

(event EventTick
  (params (DeltaSeconds :type Float%20%28single-precision%29))
  (if (Variables|Default|GetOn)
    (switch Utilities|FlowControl|Switch|SwitchonEnum_MovablePlatform_Type (Variables|SetUp|GetMoveType)
      (:NewEnumerator0
        (|SimpleMovement DeltaSeconds))
      (:NewEnumerator1
        (|ComplexMovement DeltaSeconds))
      (:NewEnumerator2
        (|CircularMovement DeltaSeconds)))))

(fn ConstructionScript)

(fn MoveLoc
  (params (DeltaTime :type Float%20%28double-precision%29))
  (return (+ (* (Math|Vector|Normalize (- (Variables|Calculation|GetTarget) (Transformation|GetActorLocation))) (* DeltaTime (Variables|SetUp|GetSpeed))) (Transformation|GetActorLocation))))

(fn AtTarget
  (return (<= (Math|Vector|Distance(Vector) (Transformation|GetActorLocation) (Variables|Calculation|GetTarget)) (Variables|SetUp|GetTargetThreshold))))

(fn IsNextPoint
  (return (Utilities|Array|IsValidIndex (Variables|SetUp|GetPath) (+ (Variables|Calculation|GetTargetIndex) 1))))

(fn GetNextPoint
  (Variables|Calculation|SetTargetIndex (+ (Variables|Calculation|GetTargetIndex) 1))
  (Variables|Calculation|SetTarget (Utilities|Array|Get(acopy) (Variables|SetUp|GetPath) (Variables|Calculation|GetTargetIndex))))

(fn IsPreviousPoint
  (return (Utilities|Array|IsValidIndex (Variables|SetUp|GetPath) (+ (Variables|Calculation|GetTargetIndex) -1))))

(fn GetPreviousPoint
  (Variables|Calculation|SetTargetIndex (+ (Variables|Calculation|GetTargetIndex) -1))
  (Variables|Calculation|SetTarget (Utilities|Array|Get(acopy) (Variables|SetUp|GetPath) (Variables|Calculation|GetTargetIndex))))