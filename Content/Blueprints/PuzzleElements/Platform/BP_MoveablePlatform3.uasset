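; BP_MoveablePlatform3 is a puzzle platform Blueprint set up to travel between points stored in a Path array.
; Helper functions check whether a next or previous index is valid, and step TargetIndex forward or back to update Target.
; MoveLoc, AtTarget and the construction script are empty, so the file contains path navigation but no movement or arrival logic.
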(fn ConstructionScript)

(fn MoveLoc
  (params (DeltaTime :type Float%20%28double-precision%29)))

(fn AtTarget)

(fn IsNextPoint
  (return (Utilities|Array|IsValidIndex (Variables|SetUp|GetPath) (+ (Variables|Calculation|GetTargetIndex) 1))))

(fn GetNextPoint
  (Variables|Calculation|SetTargetIndex (+ (Variables|Calculation|GetTargetIndex) 1))
  (Variables|Calculation|SetTarget (Utilities|Array|Get(acopy) (Variables|SetUp|GetPath) (Variables|Calculation|GetTargetIndex))))

(fn IsPreviousPoint
  (return (Utilities|Array|IsValidIndex (Variables|SetUp|GetPath) (+ (Variables|Calculation|GetTargetIndex) -1))))

(fn GetPreviousPoint
  (Variables|Calculation|SetTargetIndex (+ (Variables|Calculation|GetTargetIndex) -1))
  (Variables|Calculation|SetTarget (Utilities|Array|Get(acopy) (Variables|SetUp|GetPath) (Variables|Calculation|GetTargetIndex))))