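; BP_PlatformFence is a platform fence actor whose mesh slides when triggered by platform number or by a signal receiver.
; Beam-up and receiver activation, or beam-down and deactivation, share paths that compare PlatformNumber with PlatformValue.
; A match plays one of two timelines, lerping the mesh's relative location from zero along negative or positive local Y.
; Both moves start from zero, and a world-Z target calculation is left unconnected.
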(event ActivateReceiver(SignalReceiver)
  (if (== (stale EventBeamPlatformUp PlatformNumber) (Variables|Default|GetPlatformValue))
    (bind _platformupward (Timeline|Timeline_1 PlayFromStart)
      (:Update
        (Transformation|SetRelativeLocation (Variables|Default|GetStaticMesh) (Math|Vector|Lerp(Vector) "0, 0, 0" "0.000000,-431.270495,0.000000" _platformupward) false false)))))

(event DeactiveReceiver(SignalReceiver)
  (if (== (stale EventBeamPlatformDown PlatformNumber) (Variables|Default|GetPlatformValue))
    (bind _platformupward (Timeline|Timeline PlayFromStart)
      (:Update
        (Transformation|SetRelativeLocation (Variables|Default|GetStaticMesh) (Math|Vector|Lerp(Vector) "0, 0, 0" "0.000000,431.270495,0.000000" _platformupward) false false)))))

(event EventBeginPlay)

(event EventBeamPlatformUp
  (params (PlatformNumber :type Integer))
  (if (== PlatformNumber (Variables|Default|GetPlatformValue))
    (bind _platformupward (Timeline|Timeline_1 PlayFromStart)
      (:Update
        (Transformation|SetRelativeLocation (Variables|Default|GetStaticMesh) (Math|Vector|Lerp(Vector) "0, 0, 0" "0.000000,-431.270495,0.000000" _platformupward) false false)))))

(event EventBeamPlatformDown
  (params (PlatformNumber :type Integer))
  (if (== PlatformNumber (Variables|Default|GetPlatformValue))
    (bind _platformupward (Timeline|Timeline PlayFromStart)
      (:Update
        (Transformation|SetRelativeLocation (Variables|Default|GetStaticMesh) (Math|Vector|Lerp(Vector) "0, 0, 0" "0.000000,431.270495,0.000000" _platformupward) false false)))))

(fn ConstructionScript)