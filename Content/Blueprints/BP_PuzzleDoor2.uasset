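; BP_PuzzleDoor2 is a two-piece puzzle door whose halves slide vertically apart to open.
; OpenDoor sets energy materials on both halves, plays a sound and runs a timeline that lerps their relative locations.
; CloseDoor swaps to red energy materials and reverses that same timeline, without sound.
; A second closing timeline with its own sound is left unconnected and never runs.
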(event Custom|OpenDoor
  (params (Player :type Actor%20Object%20Reference))
  (Rendering|Material|SetMaterial (Variables|Default|GetTopDoor) 1 "/Game/Materials/M_Energy.M_Energy")
  (Rendering|Material|SetMaterial (Variables|Default|GetBottomDoor) 2 "/Game/Materials/M_Energy.M_Energy")
  (Audio|PlaySound2D 0 1.0 1.0 0.0 0 0)
  (bind _openpuzzledoor (Timeline|Timeline Play)
    (:Update
      (Utilities|FlowControl|Sequence
        (:then_0
          (Transformation|SetRelativeLocation (Variables|Default|GetTopDoor) (Math|Vector|Lerp(Vector) "0.000000,0.000000,85.110051" "0.000000,0.000000,354.265822" _openpuzzledoor) false false))
        (:then_1
          (Transformation|SetRelativeLocation (Variables|Default|GetBottomDoor) (Math|Vector|Lerp(Vector) "0, 0, 0" "0.000000,0.000000,-445.946207" _openpuzzledoor) false false))))))

(event Custom|CloseDoor
  (Rendering|Material|SetMaterial (Variables|Default|GetBottomDoor) 2 "/Game/Materials/M_RedEnergy.M_RedEnergy")
  (Rendering|Material|SetMaterial (Variables|Default|GetTopDoor) 1 "/Game/Materials/M_RedEnergy.M_RedEnergy")
  (bind _openpuzzledoor (Timeline|Timeline Reverse)
    (:Update
      (Utilities|FlowControl|Sequence
        (:then_0
          (Transformation|SetRelativeLocation (Variables|Default|GetTopDoor) (Math|Vector|Lerp(Vector) "0.000000,0.000000,85.110051" "0.000000,0.000000,354.265822" _openpuzzledoor) false false))
        (:then_1
          (Transformation|SetRelativeLocation (Variables|Default|GetBottomDoor) (Math|Vector|Lerp(Vector) "0, 0, 0" "0.000000,0.000000,-445.946207" _openpuzzledoor) false false))))))

(fn ConstructionScript)