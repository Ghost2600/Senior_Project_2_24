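; Blueprint function library of plane math helpers.
; CreatePlane builds a plane from a normal and a point on it, storing their dot product as the plane's value.
; GetClosestPointToPlane projects an off-plane point onto the plane along its normal, dividing by the normal's squared length so the normal need not be unit length.
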(fn CreatePlane
  (params (Normal :type Vector) (Point%20On%20Plane :type Vector))
  (return (Utilities|Struct|MakePlane Normal (+ (* (.x Normal) (.x Point%20On%20Plane)) (* (.y Normal) (.y Point%20On%20Plane)) (* (.z Normal) (.z Point%20On%20Plane))))))

(fn GetClosestPointtoPlane
  (params (Plane :type Plane%20Structure) (PointOffPlane :type Vector))
  (bind _normal (Utilities|Struct|BreakPlane Plane))
  (bind _normal_2 (Utilities|Struct|BreakPlane Plane))
  (bind (_normal_3 _value) (Utilities|Struct|BreakPlane Plane))
  ;[1 1 1] Get t
  (LocalVariables|Sett (/ (Utilities|Operators|Subtract _value (* (.x _normal_3) (.x PointOffPlane)) (* (.y _normal_3) (.y PointOffPlane)) (* (.z _normal_3) (.z PointOffPlane))) (+ (Math|Float|Square (.x _normal_2)) (Math|Float|Square (.y _normal_2)) (Math|Float|Square (.z _normal_2)))))
  ;[1 1 1] Get Point On Plane
  (return (Math|Vector|MakeVector (+ (* (LocalVariables|Gett) (.x _normal)) (.x PointOffPlane)) (+ (* (LocalVariables|Gett) (.y _normal)) (.y PointOffPlane)) (+ (* (LocalVariables|Gett) (.z _normal)) (.z PointOffPlane)))))