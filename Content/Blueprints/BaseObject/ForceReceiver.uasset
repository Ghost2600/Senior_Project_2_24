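; Custom physics component that moves its owning actor using timed forces and a separate gravity force.
; Validated forces are summed with gravity into OverallForce whenever one is added or expires, or gravity is set.
; Tick integrates that over Mass into a MaxSpeed-capped Velocity, offsets the actor without sweep, then counts down force timers.
; If IsGrounded during a recalculation, CounterGravity strips velocity along the gravity axis.
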(event EventTick
  (params (DeltaSeconds :type Float%20%28single-precision%29))
  (CallFunction|CalcVelocity DeltaSeconds)
  (Transformation|AddActorWorldOffset (Variables|Standard|GetActor) (* (Variables|Standard|GetVelocity) DeltaSeconds))
  (bind _updatedforces (CallFunction|SubtractForceTime DeltaSeconds))
  (if _updatedforces
    (bind _finalforce (CallFunction|GetOutputForce))
    (Variables|Standard|SetOverallForce _finalforce)))

(event EventBeginPlay
  (Variables|Standard|SetActor (Components|GetOwner)))

(fn AddForce
  (params (NewForce :type Force%20Structure))
  (bind _forcevalid (CallFunction|ValidForce NewForce))
  (if _forcevalid
    (Utilities|Array|Add (Variables|Standard|GetForces) NewForce)
    (bind _finalforce (CallFunction|GetOutputForce))
    (Variables|Standard|SetOverallForce _finalforce)))

(fn ValidForce
  (params (Force :type Force%20Structure))
  (bind (_direction _magnitude _time) (Utilities|Struct|BreakForce Force))
  (if (not (Class|KismetMathLibrary|VectorIsNormal _direction)) ; True if not normal vector
    (Development|PrintString "Error: Force Invalid - Not Normal" true true "(R=1.000000,G=0.064578,B=0.000000,A=1.000000)" 5.0)
    (elif (<= _magnitude 0.0) ; True if mangitude <= 0
      (Development|PrintString "Error: Force Invalid - Mangitude <= 0" true true "(R=1.000000,G=0.064578,B=0.000000,A=1.000000)" 5.0)
      (elif (<= _time 0.0) ; True if time is <= 0
        (Development|PrintString "Error: Force Invalid - Time <= 0" true true "(R=1.000000,G=0.064578,B=0.000000,A=1.000000)" 5.0)
        (else
          (return true)))))
  (return false))

(fn GetOutputForce
  (bind _gravityforce (Variables|Gravity|GetGravityForce))
  (bind (_direction _magnitude) (Utilities|Struct|BreakForce _gravityforce))
  (bind _returnvalue (* _direction _magnitude))
  (for _array_element (Variables|Standard|GetForces)
    ;[1 1 1] Add forces into axis value
    (LocalVariables|SetXForce (+ (LocalVariables|GetXForce) (.x (* (.Direction (Utilities|Struct|BreakForce _array_element)) (.Magnitude (Utilities|Struct|BreakForce _array_element))))))
    (LocalVariables|SetYForce (+ (LocalVariables|GetYForce) (.y (* (.Direction (Utilities|Struct|BreakForce _array_element)) (.Magnitude (Utilities|Struct|BreakForce _array_element))))))
    (LocalVariables|SetZForce (+ (LocalVariables|GetZForce) (.z (* (.Direction (Utilities|Struct|BreakForce _array_element)) (.Magnitude (Utilities|Struct|BreakForce _array_element)))))))
  ;[1 1 1] Add Gravity
  (LocalVariables|SetXForce (+ (LocalVariables|GetXForce) (.x _returnvalue)))
  (LocalVariables|SetYForce (+ (LocalVariables|GetYForce) (.y _returnvalue)))
  (LocalVariables|SetZForce (+ (LocalVariables|GetZForce) (.z _returnvalue)))
  (if (Variables|Default|GetIsGrounded)
    (CallFunction|CounterGravity))
  (Development|PrintString "Calculating Forces")
  (return (Math|Vector|MakeVector (LocalVariables|GetXForce) (LocalVariables|GetYForce) (LocalVariables|GetZForce))))

(fn SubtractForceTime
  (params (DeltaTime :type Float%20%28double-precision%29))
  (bind (_arrayindex _arrayelement) (Utilities|Array|ReverseforEachLoop (Variables|Standard|GetForces))
    (:LoopBody
      (if (<= (- (.Time (Utilities|Struct|BreakForce _arrayelement)) DeltaTime) 0.0)
        (Utilities|Array|RemoveIndex (Variables|Standard|GetForces) _arrayindex)
        (LocalVariables|SetUpdated true)
        (else
          (Utilities|Array|SetArrayElem (Variables|Standard|GetForces) _arrayindex (Utilities|Struct|MakeForce (.Direction (Utilities|Struct|BreakForce _arrayelement)) (.Magnitude (Utilities|Struct|BreakForce _arrayelement)) (- (.Time (Utilities|Struct|BreakForce _arrayelement)) DeltaTime))))))
    (:Completed
      (return (LocalVariables|GetUpdated)))))

(fn SetGravityForce
  (params (GravityDirection :type Vector) (Magnitude :type Float%20%28double-precision%29))
  ;[1 1 1] ValidateForce
  (if (not (Class|KismetMathLibrary|VectorIsNormal GravityDirection)) ; True if not normal vector
    (Development|PrintString "Error: Force Invalid - Not Normal" true true "(R=1.000000,G=0.064578,B=0.000000,A=1.000000)" 5.0)
    (elif (<= Magnitude 0.0) ; True if mangitude <= 0
      (Development|PrintString "Error: Force Invalid - Mangitude <= 0" true true "(R=1.000000,G=0.064578,B=0.000000,A=1.000000)" 5.0)
      (else
        (Variables|Gravity|SetGravityForce (Utilities|Struct|MakeForce GravityDirection Magnitude -1.0))
        (bind _finalforce (CallFunction|GetOutputForce))
        (Variables|Standard|SetOverallForce _finalforce)
        (return true))))
  (return false))

(fn CalcVelocity
  (params (DeltaTime :type Float%20%28double-precision%29))
  ;[1 1 1] Calc Velocity
  (bind _output_get (Variables|Standard|SetVelocity (+ (Variables|Standard|GetVelocity) (* (/ (Variables|Standard|GetOverallForce) (Variables|Standard|GetMass)) DeltaTime))))
  ;[1 1 1] Set Max Speed in same Direction ig going faster than max speed
  (if (>= (Math|Vector|VectorLength _output_get) (Variables|Standard|GetMaxSpeed)) ; True if at above or max speed, else false
    (Variables|Standard|SetVelocity (* (Math|Vector|Normalize (Variables|Standard|GetVelocity)) (Variables|Standard|GetMaxSpeed)))))

(fn CounterGravity
  (bind _gravityforce (Variables|Gravity|GetGravityForce))
  (bind _gravityforce_2 (Variables|Gravity|GetGravityForce))
  (bind _direction (Utilities|Struct|BreakForce _gravityforce))
  (bind _direction_2 (Utilities|Struct|BreakForce _gravityforce_2))
  ;[1 1 1] Calc Vel without Gravity Direction
  (Variables|Standard|SetVelocity (- (Variables|Standard|GetVelocity) (* _direction_2 (Math|Vector|DotProduct _direction_2 (Variables|Standard|GetVelocity)))))
  (Variables|Standard|SetOverallForce (- (Variables|Standard|GetOverallForce) (* _direction (Math|Vector|DotProduct _direction (Variables|Standard|GetOverallForce))))))

(fn GetForceCount
  (return (Utilities|Array|Length (Variables|Standard|GetForces))))

(fn Reset
  (Utilities|Array|Clear (Variables|Standard|GetForces))
  (Variables|Standard|SetVelocity "0, 0, 0"))