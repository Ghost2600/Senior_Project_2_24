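; A test actor that exercises a ForceReceiver component for custom force-based movement.
; On BeginPlay it passes its Mass and MaxSpeed to the receiver and adds each force in StartingForces.
; Any Collider begin overlap marks the receiver grounded and calls CounterGravity; end overlap does nothing, as the logic clearing the grounded flag is unconnected.
; Debug prints show the actor's location every tick and report ground contact.
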(event OnComponentBeginOverlap(Collider)
  (params (OverlappedComponent :type Primitive%20Component%20Object%20Reference) (OtherActor :type Actor%20Object%20Reference) (OtherComp :type Primitive%20Component%20Object%20Reference) (OtherBodyIndex :type Integer) (bFromSweep :type Boolean) (SweepResult :type Hit%20Result%20Structure%20%28by%20ref%29))
  (Variables|/Game/Blueprints/BaseObject/ForceReceiver.ForceReceiver_C|SetIsGrounded (Variables|Default|GetForceReceiver) true)
  (Development|PrintString "Ground" true true "(R=0.000000,G=0.660000,B=1.000000,A=1.000000)" 5.0)
  (Default|CounterGravity (Variables|Default|GetForceReceiver)))

(event OnComponentEndOverlap(Collider)
  (params (OverlappedComponent :type Primitive%20Component%20Object%20Reference) (OtherActor :type Actor%20Object%20Reference) (OtherComp :type Primitive%20Component%20Object%20Reference) (OtherBodyIndex :type Integer)))

(event EventBeginPlay
  (Variables|/Game/Blueprints/BaseObject/ForceReceiver.ForceReceiver_C|SetMass (Variables|Default|GetForceReceiver) (Variables|Default|GetMass))
  (Variables|/Game/Blueprints/BaseObject/ForceReceiver.ForceReceiver_C|SetMaxSpeed (Variables|Default|GetForceReceiver) (Variables|Default|GetMaxSpeed))
  (for _array_element (Variables|Default|GetStarting%20Forces)
    (Default|AddForce (Variables|Default|GetForceReceiver) _array_element)))

(event EventTick
  (params (DeltaSeconds :type Float%20%28single-precision%29))
  (Development|PrintString (Utilities|String|ToString(Vector) (Transformation|GetActorLocation)) true true "(R=1.000000,G=0.871892,B=0.000000,A=1.000000)" 2.0 "BoxLoc"))

(fn ConstructionScript)