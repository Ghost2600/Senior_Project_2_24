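; A light-beam reflector puzzle actor that the player can rotate in 90-degree steps.
; When hit by a beam, it line-traces along its arrow, spawns a looping Niagara beam effect and forwards the hit with strength incremented by one, allowing chains.
; An overlap box toggles a widget and player input.
; Interact from the main character rotates the scene root, turning the outgoing beam.
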(event OnComponentBeginOverlap(Box)
  (params (OverlappedComponent :type Primitive%20Component%20Object%20Reference) (OtherActor :type Actor%20Object%20Reference) (OtherComp :type Primitive%20Component%20Object%20Reference) (OtherBodyIndex :type Integer) (bFromSweep :type Boolean) (SweepResult :type Hit%20Result%20Structure%20%28by%20ref%29))
  ;[1 1 1] Widget
  (Rendering|SetVisibility (Variables|Default|GetWidget) true false)
  (Input|EnableInput (Game|GetPlayerController 0)))

(event OnComponentEndOverlap(Box)
  (params (OverlappedComponent :type Primitive%20Component%20Object%20Reference) (OtherActor :type Actor%20Object%20Reference) (OtherComp :type Primitive%20Component%20Object%20Reference) (OtherBodyIndex :type Integer))
  ;[1 1 1] Widget
  (Rendering|SetVisibility (Variables|Default|GetWidget) false false)
  (Input|DisableInput (Game|GetPlayerController 0)))

(event Custom|RotateCube
  ;[1 1 1] Rotate
  (Transformation|AddLocalRotation (Variables|Default|GetDefaultSceneRoot) "0.000000,90.000000,0.000000" false false))

(event EventBeginPlay)

(event Collision|EventActorBeginOverlap
  (params (OtherActor :type Actor%20Object%20Reference)))

(event EventBeamHit
  (params (BeamStrength :type Integer))
  (bind _arrow (Variables|Default|GetArrow))
  (CallFunction|ReflectLight (Transformation|GetWorldLocation _arrow) (Math|Vector|GetForwardVector _arrow) (Variables|Default|GetCastDistance) (+ BeamStrength 1)))

(event EventInteract
  (params (Character :type BP%20Main%20Character%20Object%20Reference))
  ;[1 1 1] Interact
  (Utilities|Casting|CastToBP_MainCharacter Character)
  (CallFunction|RotateCube))

(fn ConstructionScript)

(fn ReflectLight
  (params (BeamOrigin :type Vector) (BeamDirection :type Vector) (CastDistance :type Float%20%28double-precision%29) (BeamStrength :type Integer))
  (bind _vfxdistance (Variables|Default|GetVFXDistance))
  (bind _returnvalue (Transformation|GetWorldLocation _vfxdistance))
  (LocalVariables|SetL_BeamOrigin BeamOrigin)
  (LocalVariables|SetL_BeamDirection BeamDirection)
  (LocalVariables|SetL_CastDistance CastDistance)
  (bind _outhit (Collision|LineTraceByChannel (LocalVariables|GetL_BeamOrigin) (+ (LocalVariables|GetL_BeamOrigin) (* (LocalVariables|GetL_BeamDirection) (LocalVariables|GetL_CastDistance))) "TraceTypeQuery4" false 0 "None" true "(R=1.000000,G=0.000000,B=0.000000,A=1.000000)" "(R=0.000000,G=1.000000,B=0.000000,A=1.000000)" 0.1))
  (Niagara|SpawnSystematLocation "/Game/VFX/Placeholder/NS_LightBeamLoop.NS_LightBeamLoop" (Math|Vector|MakeVector (.x _returnvalue) (.y _returnvalue) (.z _returnvalue)) (Transformation|GetWorldRotation _vfxdistance))
  (Class|BPIBeamHit|BeamHit(Message) (.HitActor (Collision|BreakHitResult _outhit)) BeamStrength))