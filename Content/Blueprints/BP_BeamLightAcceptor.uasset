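; BP_BeamLightAcceptor is a beam puzzle receptor that activates when hit by a strong enough light beam.
; On first qualifying BeamHit it spawns a Niagara effect, latches activated, and signals BP_BeamLight actors with its BeamLightNumber.
; Door open/close messaging to BP_BeamPuzzleDoor exists but is disconnected, and Tick is empty.
; A ReflectLight function, uncalled here, debug-traces and forwards beam strength to the hit actor.
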(event EventBeginPlay
  (Variables|Default|SetDoor%20Open false))

(event EventTick
  (params (DeltaSeconds :type Float%20%28single-precision%29))
  ;[1 1 1] Toggle State
)

(event EventBeamHit
  (params (BeamStrength :type Integer))
  (bind _cube (Variables|Default|GetCube))
  (if (>= BeamStrength (Variables|Default|GetStrengthRequirement))
    (if (not (Variables|Default|GetAcceptorActivated))
      (Niagara|SpawnSystematLocation "/Game/VFX/Placeholder/NS_ReceptorOn.NS_ReceptorOn" (Transformation|GetWorldLocation _cube) (Transformation|GetWorldRotation _cube))
      (bind _outactors (Actor|GetAllActorsOfClass "/Game/Blueprints/BP_BeamLight.BP_BeamLight_C"))
      (Default|BeamLighton _outactors (Variables|Default|GetBeamLightNumber))
      (Variables|Default|SetAcceptorActivated true))))

(fn ConstructionScript)

(fn ReflectLight
  (params (BeamOrigin :type Vector) (BeamDirection :type Vector) (CastDistance :type Float%20%28double-precision%29) (BeamStrength :type Integer))
  (Development|PrintString (Utilities|String|ToString(Integer) BeamStrength))
  (LocalVariables|SetL_BeamOrigin BeamOrigin)
  (LocalVariables|SetL_BeamDirection BeamDirection)
  (LocalVariables|SetL_CastDistance CastDistance)
  (bind _outhit (Collision|LineTraceByChannel (LocalVariables|GetL_BeamOrigin) (+ (LocalVariables|GetL_BeamOrigin) (* (LocalVariables|GetL_BeamDirection) (LocalVariables|GetL_CastDistance))) "TraceTypeQuery1" false 0 "ForDuration" true "(R=1.000000,G=0.000000,B=0.000000,A=1.000000)" "(R=0.000000,G=1.000000,B=0.000000,A=1.000000)" 0.1))
  (Class|BPIBeamHit|BeamHit(Message) (.HitActor (Collision|BreakHitResult _outhit)) BeamStrength))