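; BP_MonsterDoor is a double door that opens when its assigned CombatManager signals that combat is complete.
; On BeginPlay it binds OpenDoor to the manager's CombatComplete event, or prints a warning if no manager is set.
; OpenDoor plays a timeline that lerps the Left and Right panels between fixed relative positions without sweep.
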(event Custom|OpenDoor
  ;[1 1 1] Blake Here
  (bind _opendoor (Timeline|Timeline_0 Play)
    (:Update
      (Utilities|FlowControl|Sequence
        (:then_0
          (Transformation|SetRelativeLocation (Variables|Default|GetLeft) (Math|Vector|Lerp(Vector) "-53.239209,0.000000,0.000003" "-274.539005,0.000000,0.000003" _opendoor) false false))
        (:then_1
          (Transformation|SetRelativeLocation (Variables|Default|GetRight) (Math|Vector|Lerp(Vector) "257.894937,0.000000,0.000001" "497.788224,0.000000,0.000001" _opendoor) false false))))))

(event EventBeginPlay
  (if (Utilities|IsValid (Variables|Default|GetCombatManager))
    ;[1 1 1] Blake Here
    (EventDispatchers|BindEventtoCombatComplete (Variables|Default|GetCombatManager) (delegate Custom|OpenDoor))
    (else
      (Development|PrintString "Warning[BP_CaveDoor]: CombatManager not assigned" true true "(R=1.000000,G=0.956983,B=0.085218,A=1.000000)" 1e+01))))

(fn ConstructionScript)