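; Beam acceptor that latches a signal on when hit by a beam of sufficient strength.
; On first activation, BeamHit sets its SignalSender, spawns a receptor-on Niagara effect, and lights every BP_pathLights actor matching its BeamLightNumber.
; ReflectLight line-traces onward with debug drawing, forwarding beam strength to the hit actor.
; GetSignal returns a separate AcceptorActivated flag, which the activation logic never sets.
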(event EventBeamHit
  (params (BeamStrength :type Integer))
  (bind _cube (Variables|Default|GetCube))
  (bind _beamlightnumber (Variables|Default|GetBeamLightNumber))
  (if (>= BeamStrength (Variables|Default|GetStrengthRequirement))
    ;[1 1 1] Activate
    (if (not (Default|GetSignal (Variables|Default|GetSignalSender)))
      (Utilities|FlowControl|Sequence
        (:then_0
          (Default|SetSignal (Variables|Default|GetSignalSender) true))
        (:then_1
          (Niagara|SpawnSystematLocation "/Game/VFX/Placeholder/NS_ReceptorOn.NS_ReceptorOn" (Transformation|GetWorldLocation _cube) (Transformation|GetWorldRotation _cube)))
        (:then_2
          (bind _outactors (Actor|GetAllActorsOfClass "/Game/Blueprints/BP_pathLights.BP_pathLights_C"))
          (bind _array_element (Utilities|Array|ForEachLoopwithBreak _outactors)
            (:LoopBody
              (if (== (Variables|/Game/Blueprints/BP_pathLights.BP_pathLights_C|GetLight%20Value _array_element) _beamlightnumber)
                (Default|BeamLighton _array_element _beamlightnumber)))))))))

(fn ConstructionScript)

(fn ReflectLight
  (params (BeamOrigin :type Vector) (BeamDirection :type Vector) (CastDistance :type Float%20%28double-precision%29) (BeamStrength :type Integer))
  (LocalVariables|SetL_BeamOrigin BeamOrigin)
  (LocalVariables|SetL_BeamDirection BeamDirection)
  (LocalVariables|SetL_CastDistance CastDistance)
  (bind _outhit (Collision|LineTraceByChannel (LocalVariables|GetL_BeamOrigin) (+ (LocalVariables|GetL_BeamOrigin) (* (LocalVariables|GetL_BeamDirection) (LocalVariables|GetL_CastDistance))) "TraceTypeQuery1" false 0 "ForDuration" true "(R=1.000000,G=0.000000,B=0.000000,A=1.000000)" "(R=0.000000,G=1.000000,B=0.000000,A=1.000000)" 0.1))
  (Class|BPIBeamHit|BeamHit(Message) (.HitActor (Collision|BreakHitResult _outhit)) BeamStrength))

(fn GetSignal
  (return (Variables|Default|GetAcceptorActivated)))