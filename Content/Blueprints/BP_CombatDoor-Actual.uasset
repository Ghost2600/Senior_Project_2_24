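; BP_CombatDoor-Actual is a door that slides upward when its OpenCombatDoor event is called.
; A timeline lerps the static mesh's relative location up along Z, then plays an unlock sound at the world origin on finish.
; BeginPlay stores closed and raised world positions, but the opening movement uses its own hardcoded offsets instead.
; The graph contains no closing logic.
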(event Custom|OpenCombatDoor
  (bind _opencombatdoor (Timeline|OpenDoor PlayFromStart)
    (:Update
      (Transformation|SetRelativeLocation (Variables|Default|GetStaticMesh) (Math|Vector|Lerp(Vector) "0, 0, 0" "0.000000,0.000000,400.000000" _opencombatdoor) false false))
    (:Finished
      (Audio|PlaySoundatLocation "/Game/Audio/Placeholders/Cues/SFX_SoundEffects/SFX_EnvironmentActors/Interactables/SFX_Door_Unlock_Head_Cue.SFX_Door_Unlock_Head_Cue" "0, 0, 0" "0, 0, 0" 1.0 1.0 0.0 0 0 0 0))))

(event EventBeginPlay
  (bind _output_get (Variables|Default|SetClosed (Transformation|GetWorldLocation (Variables|Default|GetStaticMesh))))
  (Variables|Default|SetOpen (Math|Vector|MakeVector (.x _output_get) (.y _output_get) (+ (.z _output_get) 6e+02))))

(event Collision|EventActorBeginOverlap
  (params (OtherActor :type Actor%20Object%20Reference)))

(event EventTick
  (params (DeltaSeconds :type Float%20%28single-precision%29)))

(fn ConstructionScript)