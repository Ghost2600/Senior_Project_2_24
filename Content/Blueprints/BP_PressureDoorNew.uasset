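; Pressure plate for door puzzles that responds to pushable blocks and the main character through separate trigger boxes.
; Overlaps swap the plate's green/red material, play a sound and run timelines that move it vertically.
; Each timeline update searches all BP_PuzzleDoor2 actors and opens or closes those whose DoorValue matches PlateValue.
; Only the player's exit calls CloseDoor; block removal reverses its timeline, whose update still calls OpenDoor.
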(event OnComponentBeginOverlap(Box)
  (params (OverlappedComponent :type Primitive%20Component%20Object%20Reference) (OtherActor :type Actor%20Object%20Reference) (OtherComp :type Primitive%20Component%20Object%20Reference) (OtherBodyIndex :type Integer) (bFromSweep :type Boolean) (SweepResult :type Hit%20Result%20Structure%20%28by%20ref%29))
  ;[1 1 1] Cube
  (Utilities|Casting|CastToBP_PushableBlock OtherActor)
  (Rendering|Material|SetMaterial (Variables|Default|GetPlate) 0 "/Game/Materials/M_Green.M_Green")
  (Audio|PlaySoundatLocation 0 (Transformation|GetActorLocation) "0, 0, 0" 1.0 1.0 0.0 0 0 0 0)
  (Variables|Default|SetPlateActive true)
  (bind _pressureplateheight (Timeline|Down Play)
    (:Update
      (Transformation|SetRelativeLocation (Variables|Default|GetPlate) (Math|Vector|MakeVector 0.0 0.0 (Math|Float|Lerp 13.0 6.0 _pressureplateheight)) false false)
      (Development|PrintString "Box on")
      (bind _outactors (Actor|GetAllActorsOfClass "/Game/Blueprints/BP_PuzzleDoor2.BP_PuzzleDoor2_C"))
      (bind _array_element (Utilities|Array|ForEachLoopwithBreak _outactors)
        (:LoopBody
          (if (== (Variables|/Game/Blueprints/BP_PuzzleDoor2.BP_PuzzleDoor2_C|GetDoorValue _array_element) (Variables|Default|GetPlateValue))
            (Default|OpenDoor _array_element)))))))

(event OnComponentEndOverlap(Box)
  (params (OverlappedComponent :type Primitive%20Component%20Object%20Reference) (OtherActor :type Actor%20Object%20Reference) (OtherComp :type Primitive%20Component%20Object%20Reference) (OtherBodyIndex :type Integer))
  ;[1 1 1] Cube
  (Utilities|Casting|CastToBP_PushableBlock OtherActor)
  (Rendering|Material|SetMaterial (Variables|Default|GetPlate) 0 "/Game/Materials/M_Red.M_Red")
  (Audio|PlaySoundatLocation 0 (Transformation|GetActorLocation) "0, 0, 0" 1.0 1.0 0.0 0 0 0 0)
  (Variables|Default|SetPlateActive false)
  (bind _pressureplateheight (Timeline|Down Reverse)
    (:Update
      (Transformation|SetRelativeLocation (Variables|Default|GetPlate) (Math|Vector|MakeVector 0.0 0.0 (Math|Float|Lerp 13.0 6.0 _pressureplateheight)) false false)
      (Development|PrintString "Box on")
      (bind _outactors (Actor|GetAllActorsOfClass "/Game/Blueprints/BP_PuzzleDoor2.BP_PuzzleDoor2_C"))
      (bind _array_element (Utilities|Array|ForEachLoopwithBreak _outactors)
        (:LoopBody
          (if (== (Variables|/Game/Blueprints/BP_PuzzleDoor2.BP_PuzzleDoor2_C|GetDoorValue _array_element) (Variables|Default|GetPlateValue))
            (Default|OpenDoor _array_element)))))))

(event OnComponentEndOverlap(PlayerBox)
  (params (OverlappedComponent :type Primitive%20Component%20Object%20Reference) (OtherActor :type Actor%20Object%20Reference) (OtherComp :type Primitive%20Component%20Object%20Reference) (OtherBodyIndex :type Integer))
  ;[1 1 1] Player
  (Utilities|Casting|CastToBP_MainCharacter OtherActor)
  (Rendering|Material|SetMaterial (Variables|Default|GetPlate) 0 "/Game/Materials/M_Red.M_Red")
  (Audio|PlaySoundatLocation 0 (Transformation|GetActorLocation) "0, 0, 0" 1.0 1.0 0.0 0 0 0 0)
  (bind _pressureplateheight (Timeline|Timeline Play)
    (:Update
      (Transformation|SetRelativeLocation (Variables|Default|GetPlate) (Math|Vector|MakeVector 0.0 0.0 (Math|Float|Lerp 6.0 13.0 _pressureplateheight)) false false)
      (bind _outactors (Actor|GetAllActorsOfClass "/Game/Blueprints/BP_PuzzleDoor2.BP_PuzzleDoor2_C"))
      (bind _array_element (Utilities|Array|ForEachLoopwithBreak _outactors)
        (:LoopBody
          (if (== (Variables|/Game/Blueprints/BP_PuzzleDoor2.BP_PuzzleDoor2_C|GetDoorValue _array_element) (Variables|Default|GetPlateValue))
            (Default|CloseDoor _array_element)))))))

(event OnComponentBeginOverlap(PlayerBox)
  (params (OverlappedComponent :type Primitive%20Component%20Object%20Reference) (OtherActor :type Actor%20Object%20Reference) (OtherComp :type Primitive%20Component%20Object%20Reference) (OtherBodyIndex :type Integer) (bFromSweep :type Boolean) (SweepResult :type Hit%20Result%20Structure%20%28by%20ref%29))
  ;[1 1 1] Player
  (Utilities|Casting|CastToBP_MainCharacter OtherActor)
  (Rendering|Material|SetMaterial (Variables|Default|GetPlate) 0 "/Game/Materials/M_Green.M_Green")
  (Audio|PlaySoundatLocation 0 (Transformation|GetActorLocation) "0, 0, 0" 1.0 1.0 0.0 0 0 0 0)
  (bind _pressureplateheight (Timeline|Timeline_0 Play)
    (:Update
      (Transformation|SetRelativeLocation (Variables|Default|GetPlate) (Math|Vector|MakeVector 0.0 0.0 (Math|Float|Lerp 13.0 6.0 _pressureplateheight)) false false)
      (bind _outactors (Actor|GetAllActorsOfClass "/Game/Blueprints/BP_PuzzleDoor2.BP_PuzzleDoor2_C"))
      (bind _array_element (Utilities|Array|ForEachLoopwithBreak _outactors)
        (:LoopBody
          (if (== (Variables|/Game/Blueprints/BP_PuzzleDoor2.BP_PuzzleDoor2_C|GetDoorValue _array_element) (Variables|Default|GetPlateValue))
            (Default|OpenDoor _array_element)))))))

(fn ConstructionScript)