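; Puzzle pressure plate that a pushable block or the main character activates, with sound and a green/red material change.
; Box overlaps set PlateActive and drive timelines that lower Plate for blocks or PlayerBox for the player.
; Timeline updates call PressureToRise or PressureToFall on BP_MovablePuzzleButton1 actors whose PressureValue matches PlateValue.
; Only player exit triggers red and fall; block exit reverses Down, repeating green and rise.
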(event OnComponentBeginOverlap(Box)
  (params (OverlappedComponent :type Primitive%20Component%20Object%20Reference) (OtherActor :type Actor%20Object%20Reference) (OtherComp :type Primitive%20Component%20Object%20Reference) (OtherBodyIndex :type Integer) (bFromSweep :type Boolean) (SweepResult :type Hit%20Result%20Structure%20%28by%20ref%29))
  (Utilities|FlowControl|Sequence
    (:then_0
      (Utilities|Casting|CastToBP_PushableBlock OtherActor)
      (Audio|PlaySoundatLocation 0 (Transformation|GetActorLocation) "0, 0, 0" 1.0 1.0 0.0 0 0 0 0)
      (Variables|Default|SetPlateActive true)
      (bind _pressureplateheight (Timeline|Down Play)
        (:Update
          (Transformation|SetRelativeLocation (Variables|Default|GetPlate) (Math|Vector|MakeVector 0.0 0.0 (Math|Float|Lerp 13.0 6.0 _pressureplateheight)) false false)
          (Rendering|Material|SetMaterial (Variables|Default|GetPlate) 0 "/Game/Materials/M_Green.M_Green")
          (Development|PrintString "Box on")
          (bind _outactors (Actor|GetAllActorsOfClass "/Game/PlaceHolderModels/BP_MovablePuzzleButton1.BP_MovablePuzzleButton1_C"))
          (bind _array_element (Utilities|Array|ForEachLoopwithBreak _outactors)
            (:LoopBody
              (if (== (Variables|/Game/PlaceHolderModels/BP_MovablePuzzleButton1.BP_MovablePuzzleButton1_C|GetPressureValue _array_element) (Variables|Default|GetPlateValue))
                (Default|PressuretoRise _array_element)))))))
    (:then_1
      (Utilities|Casting|CastToBP_MainCharacter OtherActor)
      (Audio|PlaySoundatLocation 0 (Transformation|GetActorLocation) "0, 0, 0" 1.0 1.0 0.0 0 0 0 0)
      (Variables|Default|SetPlateActive true)
      (bind _pressureplateheight_2 (Timeline|Timeline Play)
        (:Update
          (Transformation|SetRelativeLocation (Variables|Default|GetPlayerBox) (Math|Vector|MakeVector 0.0 0.0 (Math|Float|Lerp 13.0 6.0 _pressureplateheight_2)) false false)
          (Rendering|Material|SetMaterial (Variables|Default|GetPlate) 0 "/Game/Materials/M_Green.M_Green")
          (Development|PrintString "Player on")
          (bind _outactors_2 (Actor|GetAllActorsOfClass "/Game/PlaceHolderModels/BP_MovablePuzzleButton1.BP_MovablePuzzleButton1_C"))
          (bind _array_element_2 (Utilities|Array|ForEachLoopwithBreak _outactors_2)
            (:LoopBody
              (if (== (Variables|/Game/PlaceHolderModels/BP_MovablePuzzleButton1.BP_MovablePuzzleButton1_C|GetPressureValue _array_element_2) (Variables|Default|GetPlateValue))
                (Default|PressuretoRise _array_element_2)))))))))

(event OnComponentEndOverlap(Box)
  (params (OverlappedComponent :type Primitive%20Component%20Object%20Reference) (OtherActor :type Actor%20Object%20Reference) (OtherComp :type Primitive%20Component%20Object%20Reference) (OtherBodyIndex :type Integer))
  (Utilities|FlowControl|Sequence
    (:then_0
      (Utilities|Casting|CastToBP_PushableBlock OtherActor)
      (Audio|PlaySoundatLocation 0 (Transformation|GetActorLocation) "0, 0, 0" 1.0 1.0 0.0 0 0 0 0)
      (Variables|Default|SetPlateActive false)
      (bind _pressureplateheight (Timeline|Down Reverse)
        (:Update
          (Transformation|SetRelativeLocation (Variables|Default|GetPlate) (Math|Vector|MakeVector 0.0 0.0 (Math|Float|Lerp 13.0 6.0 _pressureplateheight)) false false)
          (Rendering|Material|SetMaterial (Variables|Default|GetPlate) 0 "/Game/Materials/M_Green.M_Green")
          (Development|PrintString "Box on")
          (bind _outactors (Actor|GetAllActorsOfClass "/Game/PlaceHolderModels/BP_MovablePuzzleButton1.BP_MovablePuzzleButton1_C"))
          (bind _array_element (Utilities|Array|ForEachLoopwithBreak _outactors)
            (:LoopBody
              (if (== (Variables|/Game/PlaceHolderModels/BP_MovablePuzzleButton1.BP_MovablePuzzleButton1_C|GetPressureValue _array_element) (Variables|Default|GetPlateValue))
                (Default|PressuretoRise _array_element)))))))
    (:then_1
      (Utilities|Casting|CastToBP_MainCharacter OtherActor)
      (Audio|PlaySoundatLocation 0 (Transformation|GetActorLocation) "0, 0, 0" 1.0 1.0 0.0 0 0 0 0)
      (Variables|Default|SetPlateActive false)
      (bind _pressureplateheight_2 (Timeline|Timeline_0 Play)
        (:Update
          (Transformation|SetRelativeLocation (Variables|Default|GetPlayerBox) (Math|Vector|MakeVector 0.0 0.0 (Math|Float|Lerp 13.0 6.0 _pressureplateheight_2)) false false)
          (Rendering|Material|SetMaterial (Variables|Default|GetPlate) 0 "/Game/Materials/M_Red.M_Red")
          (Development|PrintString "Player off")
          (bind _outactors_2 (Actor|GetAllActorsOfClass "/Game/PlaceHolderModels/BP_MovablePuzzleButton1.BP_MovablePuzzleButton1_C"))
          (bind _array_element_2 (Utilities|Array|ForEachLoopwithBreak _outactors_2)
            (:LoopBody
              (if (== (Variables|/Game/PlaceHolderModels/BP_MovablePuzzleButton1.BP_MovablePuzzleButton1_C|GetPressureValue _array_element_2) (Variables|Default|GetPlateValue))
                (Default|PressuretoFall _array_element_2)))))))))

(event EventBeginPlay)

(event Collision|EventActorBeginOverlap
  (params (OtherActor :type Actor%20Object%20Reference)))

(fn ConstructionScript)