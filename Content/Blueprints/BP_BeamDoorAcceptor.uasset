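; Beam puzzle receptor that opens doors and lights paths when hit by a beam of sufficient strength.
; BeamHit spawns Niagara receptor effects, then searches all BP_BeamDoor and BP_pathLights actors for matching puzzle numbers to trigger.
; Any match sets AcceptorActivated, blocking repeat activation.
; A ReflectLight function, not called in these graphs, line-traces with debug drawing and forwards beam strength to the hit actor.
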(event EventBeginPlay
  (Variables|Default|SetDoor%20Open false))

(event EventBeamHit
  (params (BeamStrength :type Integer))
  (bind _cube (Variables|Default|GetCube))
  (bind _cube_2 (Variables|Default|GetCube))
  (bind _beamlightnumber (Variables|Default|GetBeamLightNumber))
  ;[1 1 1] Activate
  (if (>= BeamStrength (Variables|Default|GetStrengthRequirement))
    (if (not (Variables|Default|GetAcceptorActivated))
      (Utilities|FlowControl|Sequence
        (:then_0
          (Niagara|SpawnSystematLocation "/Game/VFX/Placeholder/NS_ReceptorOn.NS_ReceptorOn" (Transformation|GetWorldLocation _cube_2) (Transformation|GetWorldRotation _cube_2))
          (bind _outactors (Actor|GetAllActorsOfClass "/Game/Blueprints/BP_BeamDoor.BP_BeamDoor_C"))
          (bind _array_element (Utilities|Array|ForEachLoopwithBreak _outactors)
            (:LoopBody
              (if (== (Variables|/Game/Blueprints/BP_BeamDoor.BP_BeamDoor_C|GetDoorValue _array_element) (Variables|Default|GetBeamPuzzleDoorNumber))
                (Default|OpenDoor _array_element)
                (Variables|Default|SetAcceptorActivated true)))))
        (:then_1
          (Niagara|SpawnSystematLocation "/Game/VFX/Placeholder/NS_ReceptorOn.NS_ReceptorOn" (Transformation|GetWorldLocation _cube) (Transformation|GetWorldRotation _cube))
          (bind _outactors_2 (Actor|GetAllActorsOfClass "/Game/Blueprints/BP_pathLights.BP_pathLights_C"))
          (bind _array_element_2 (Utilities|Array|ForEachLoopwithBreak _outactors_2)
            (:LoopBody
              (if (== (Variables|/Game/Blueprints/BP_pathLights.BP_pathLights_C|GetLight%20Value _array_element_2) _beamlightnumber)
                (Default|BeamLighton _array_element_2 _beamlightnumber)
                (Variables|Default|SetAcceptorActivated true)))))))))

(fn ConstructionScript)

(fn ReflectLight
  (params (BeamOrigin :type Vector) (BeamDirection :type Vector) (CastDistance :type Float%20%28double-precision%29) (BeamStrength :type Integer))
  (LocalVariables|SetL_BeamOrigin BeamOrigin)
  (LocalVariables|SetL_BeamDirection BeamDirection)
  (LocalVariables|SetL_CastDistance CastDistance)
  (bind _outhit (Collision|LineTraceByChannel (LocalVariables|GetL_BeamOrigin) (+ (LocalVariables|GetL_BeamOrigin) (* (LocalVariables|GetL_BeamDirection) (LocalVariables|GetL_CastDistance))) "TraceTypeQuery1" false 0 "ForDuration" true "(R=1.000000,G=0.000000,B=0.000000,A=1.000000)" "(R=0.000000,G=1.000000,B=0.000000,A=1.000000)" 0.1))
  (Class|BPIBeamHit|BeamHit(Message) (.HitActor (Collision|BreakHitResult _outhit)) BeamStrength))