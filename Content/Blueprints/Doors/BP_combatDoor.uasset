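; BP_combatDoor is a door that opens and closes in response to its signal receiver component, BPC_SignalReceiver.
; Activation swaps two material slots to M_Energy, plays an unlock sound and runs a timeline that lerps the Door mesh downward.
; Deactivation sets red-energy and daylight materials, plays a close sound and reverses a second, separate timeline from its end to raise the door back.
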(event ActivateReceiver(BPC_SignalReceiver)
  (Rendering|Material|SetMaterial (Variables|Default|GetDoor) 1 "/Game/Materials/M_Energy.M_Energy")
  (Rendering|Material|SetMaterial (Variables|Default|GetDoor) 3 "/Game/Materials/M_Energy.M_Energy")
  (Audio|PlaySound2D "/Game/Audio/Placeholders/Cues/SFX_SoundEffects/SFX_EnvironmentActors/Interactables/SFX_Door_Unlock_Head_Cue.SFX_Door_Unlock_Head_Cue" 1.0 1.0 0.0 0 0)
  (bind _openpuzzledoor (Timeline|Timeline Play)
    (:Update
      (Transformation|SetRelativeLocation (Variables|Default|GetDoor) (Math|Vector|Lerp(Vector) "0, 0, 0" "0.000000,0.000000,-600.000000" _openpuzzledoor) false false))))

(event DeactiveReceiver(BPC_SignalReceiver)
  (Rendering|Material|SetMaterial (Variables|Default|GetDoor) 1 "/Game/Materials/M_RedEnergy.M_RedEnergy")
  (Rendering|Material|SetMaterial (Variables|Default|GetDoor) 3 "/Game/Materials/M_Daylight.M_Daylight")
  (Audio|PlaySound2D "/Game/Audio/Placeholders/Cues/SFX_SoundEffects/SFX_EnvironmentActors/Interactables/SFX_Door_Close_Head_PH_Cue.SFX_Door_Close_Head_PH_Cue" 1.0 1.0 0.0 0 0)
  (bind _openpuzzledoor (Timeline|Timeline_0 ReverseFromEnd)
    (:Update
      (Transformation|SetRelativeLocation (Variables|Default|GetDoor) (Math|Vector|Lerp(Vector) "0, 0, 0" "0.000000,0.000000,-600.000000" _openpuzzledoor) false false))))

(fn ConstructionScript)