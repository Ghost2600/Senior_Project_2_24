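; BP_BeamDoor is a two-panel puzzle door that opens and closes in response to its SignalReceiver's activate and deactivate events.
; Activation switches both panels to the energy material, plays an unlock sound and runs a timeline that lerps the top panel up and the bottom panel down.
; Deactivation restores the red energy material, plays a close sound and reverses the same timeline.
; Both sounds play at the world origin.
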(event ActivateReceiver(SignalReceiver)
  (Rendering|Material|SetMaterial (Variables|Default|GetTopDoor) 1 "/Game/Materials/M_Energy.M_Energy")
  (Rendering|Material|SetMaterial (Variables|Default|GetBottomDoor) 1 "/Game/Materials/M_Energy.M_Energy")
  (Audio|PlaySoundatLocation (Variables|Default|GetAud_Door_Unlock_Head) "0, 0, 0" "0, 0, 0" 1.0 1.0 0.0 0 0 0 0)
  (bind _openpuzzledoor (Timeline|Timeline Play)
    (:Update
      (Utilities|FlowControl|Sequence
        (:then_0
          (Transformation|SetRelativeLocation (Variables|Default|GetTopDoor) (Math|Vector|Lerp(Vector) "0, 0, 0" "0.000000,0.000000,176.370912" _openpuzzledoor) false false))
        (:then_1
          (Transformation|SetRelativeLocation (Variables|Default|GetBottomDoor) (Math|Vector|Lerp(Vector) "0, 0, 0" "0.000000,0.000000,-271.372535" _openpuzzledoor) false false))))))

(event DeactiveReceiver(SignalReceiver)
  (Rendering|Material|SetMaterial (Variables|Default|GetBottomDoor) 1 "/Game/Materials/M_RedEnergy.M_RedEnergy")
  (Rendering|Material|SetMaterial (Variables|Default|GetTopDoor) 1 "/Game/Materials/M_RedEnergy.M_RedEnergy")
  (Audio|PlaySoundatLocation (Variables|Default|GetAud_Door_Close) "0, 0, 0" "0, 0, 0" 1.0 1.0 0.0 0 0 0 0)
  (bind _openpuzzledoor (Timeline|Timeline Reverse)
    (:Update
      (Utilities|FlowControl|Sequence
        (:then_0
          (Transformation|SetRelativeLocation (Variables|Default|GetTopDoor) (Math|Vector|Lerp(Vector) "0, 0, 0" "0.000000,0.000000,176.370912" _openpuzzledoor) false false))
        (:then_1
          (Transformation|SetRelativeLocation (Variables|Default|GetBottomDoor) (Math|Vector|Lerp(Vector) "0, 0, 0" "0.000000,0.000000,-271.372535" _openpuzzledoor) false false))))))

(fn ConstructionScript)