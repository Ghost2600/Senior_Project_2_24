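; BP_MonsterDoor is a two-panel sliding door driven by SignalReceiver activate and deactivate events.
; Activation plays a timeline that lerps the Left and Right relative locations in opposite directions along X, and deactivation reverses it.
; Each timeline update also activates the Box component once the OpenDoor value reaches a small threshold and deactivates it below that.
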(event ActivateReceiver(SignalReceiver)
  (bind _box (Variables|Default|GetBox))
  (bind _opendoor (Timeline|Timeline_0 Play)
    (:Update
      (Utilities|FlowControl|Sequence
        (:then_0
          (if (>= _opendoor 0.05)
            (Components|Activation|Activate _box false)
            (else
              (Components|Activation|Deactivate _box))))
        (:then_1
          (Transformation|SetRelativeLocation (Variables|Default|GetLeft) (Math|Vector|Lerp(Vector) "-53.239209,0.000000,0.000003" "-274.539005,0.000000,0.000003" _opendoor) false false))
        (:then_2
          (Transformation|SetRelativeLocation (Variables|Default|GetRight) (Math|Vector|Lerp(Vector) "257.894937,0.000000,0.000001" "497.788224,0.000000,0.000001" _opendoor) false false))))))

(event DeactiveReceiver(SignalReceiver)
  (bind _box (Variables|Default|GetBox))
  (bind _opendoor (Timeline|Timeline_0 Reverse)
    (:Update
      (Utilities|FlowControl|Sequence
        (:then_0
          (if (>= _opendoor 0.05)
            (Components|Activation|Activate _box false)
            (else
              (Components|Activation|Deactivate _box))))
        (:then_1
          (Transformation|SetRelativeLocation (Variables|Default|GetLeft) (Math|Vector|Lerp(Vector) "-53.239209,0.000000,0.000003" "-274.539005,0.000000,0.000003" _opendoor) false false))
        (:then_2
          (Transformation|SetRelativeLocation (Variables|Default|GetRight) (Math|Vector|Lerp(Vector) "257.894937,0.000000,0.000001" "497.788224,0.000000,0.000001" _opendoor) false false))))))

(fn ConstructionScript)