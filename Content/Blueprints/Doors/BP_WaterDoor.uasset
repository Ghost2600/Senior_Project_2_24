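; BP_WaterDoor is a puzzle door that slides open and shut through its OpenDoor and CloseDoor events.
; One timeline lerps the top door, bottom door and cube between fixed relative positions, and closing reverses it.
; Each event swaps the top door's energy material and plays a water sound.
; A player hitting the cube spawns an evil-water Niagara effect; a second timeline branch is left disconnected.
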(event OnComponentHit(Cube)
  (params (HitComponent :type Primitive%20Component%20Object%20Reference) (OtherActor :type Actor%20Object%20Reference) (OtherComp :type Primitive%20Component%20Object%20Reference) (NormalImpulse :type Vector :default "0, 0, 0") (Hit :type Hit%20Result%20Structure%20%28by%20ref%29))
  (if (Actor|ActorHasTag OtherActor "Player")
    (Niagara|SpawnSystematLocation "/Game/VFX/Placeholder/NS_EvilWater.NS_EvilWater" (Transformation|GetWorldLocation (Variables|Default|GetPartical%20Spawn)) (Transformation|GetActorRotation) (Math|Conversions|ToVector(Float) (Variables|Default|GetWaterBlock)))))

(event Custom|OpenDoor
  (params (Player :type Actor%20Object%20Reference))
  (Rendering|Material|SetMaterial (Variables|Default|GetTopDoor) 1 "/Game/Materials/M_Energy.M_Energy")
  (Audio|PlaySound2D "/Game/Audio/SmallSoundKit/SSKCue/MagicCue/Mgc_Water_Throw_01_Cue.Mgc_Water_Throw_01_Cue" 1.0 1.0 0.0 0 0)
  (bind _openpuzzledoor (Timeline|Timeline Play)
    (:Update
      (Utilities|FlowControl|Sequence
        (:then_0
          (Transformation|SetRelativeLocation (Variables|Default|GetTopDoor) (Math|Vector|Lerp(Vector) "-12.930139,405.208408,-111.298972" "-12.930139,405.208408,-228.385458" _openpuzzledoor) false false))
        (:then_1
          (Transformation|SetRelativeLocation (Variables|Default|GetBottomDoor) (Math|Vector|Lerp(Vector) "0, 0, 0" "0.000000,-498.710754,0.000000" _openpuzzledoor) false false))))))

(event Custom|CloseDoor
  (Rendering|Material|SetMaterial (Variables|Default|GetTopDoor) 1 "/Game/Materials/M_RedEnergy.M_RedEnergy")
  (Audio|PlaySound2D "/Game/Audio/SmallSoundKit/SSKCue/MagicCue/Mgc_Water_Throw_02_Cue.Mgc_Water_Throw_02_Cue" 1.0 1.0 0.0 0 0)
  (bind _openpuzzledoor (Timeline|Timeline Reverse)
    (:Update
      (Utilities|FlowControl|Sequence
        (:then_0
          (Transformation|SetRelativeLocation (Variables|Default|GetTopDoor) (Math|Vector|Lerp(Vector) "-12.930139,405.208408,-111.298972" "-12.930139,405.208408,-228.385458" _openpuzzledoor) false false))
        (:then_1
          (Transformation|SetRelativeLocation (Variables|Default|GetBottomDoor) (Math|Vector|Lerp(Vector) "0, 0, 0" "0.000000,-498.710754,0.000000" _openpuzzledoor) false false))))))

(fn ConstructionScript)